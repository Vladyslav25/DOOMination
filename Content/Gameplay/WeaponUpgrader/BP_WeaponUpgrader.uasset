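; BP_WeaponUpgrader is an actor that shows and hides the weapon upgrade menu.
; It creates a BP_WeaponUpgradeUI widget once on BeginPlay and keeps it for reuse.
; TriggerMenu toggles that widget through OpenUI and CloseUI, which add it to or remove it from the viewport and update IsUIActive.
; UIActive returns that flag; overlap and tick events are unused.
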(event EventBeginPlay
  (bind _returnvalue (UserInterface|CreateWidget "/Game/UI/UI_Blueprints/BP_WeaponUpgradeUI.BP_WeaponUpgradeUI_C"))
  (Variables|Default|SetUpgradeWidget _returnvalue))

(event Collision|EventActorBeginOverlap
  (params (OtherActor :type Actor%20Object%20Reference)))

(event EventTick
  (params (DeltaSeconds :type Float%20%28single-precision%29)))

(fn ConstructionScript)

(fn TriggerMenu
  (if (Variables|Default|GetIsUIActive)
    (CallFunction|CloseUI)
    (else
      (CallFunction|OpenUI))))

(fn UIActive
  (return (Variables|Default|GetIsUIActive)))

(fn OpenUI
  (UserInterface|Viewport|AddtoViewport (Variables|Default|GetUpgradeWidget) 0)
  (Variables|Default|SetIsUIActive true))

(fn CloseUI
  (Widget|RemovefromParent (Variables|Default|GetUpgradeWidget))
  (Variables|Default|SetIsUIActive false))