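; Round controller that runs endless enemy waves, queuing Tanks, Minions and Bombers on an EnemySpawner.
; Each wave's count per type is an exponentially growing HP pot, based on the round number, divided by that type's base HP.
; Tick drives a countdown that starts once the spawn queue empties; the next wave follows when it expires or all spawned enemies are gone.
; A debug print shows each wave's counts.
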(event Custom|New%20Wave
  (bind _pot_tank (HPPot|CalculateHPPotTank))
  (bind _pot_minion (HPPot|CalculateHPPotMinion))
  (bind _pot_bomber (HPPot|CalculateHPPotBomber))
  (bind _basehptank (Variables|BaseHP|GetBaseHPTank))
  (bind _basehpminion (Variables|BaseHP|GetBaseHPMinion))
  (bind _basehpbomber (Variables|BaseHP|GetBaseHPBomber))
  (bind _count (CallFunction|EnemySpawnCount _pot_tank _basehptank))
  (bind _count_2 (CallFunction|EnemySpawnCount _pot_bomber _basehpbomber))
  (bind _count_3 (CallFunction|EnemySpawnCount _pot_minion _basehpminion))
  (Math|Integer|IncrementInt (Variables|Default|GetEnemyRound)
    (:%20%20
      (Default|AddEnemytoQueue (Variables|Default|GetEnemySpawner) "/Game/Characters/NPC/Enemies/Blueprints/Tank/BP_Tank.BP_Tank_C" _count 0.5)
      (Default|AddEnemytoQueue (Variables|Default|GetEnemySpawner) "/Game/Characters/NPC/Enemies/Blueprints/Minion/BP_Minion.BP_Minion_C" _count_3 0.5)
      (Default|AddEnemytoQueue (Variables|Default|GetEnemySpawner) "/Game/Characters/NPC/Enemies/Blueprints/Bomber/BP_Bomber.BP_Bomber_C" _count_2 0.5)
      ;[1 1 1] DEBUG
      (Development|PrintString (Utilities|String|Append "Wave: " (Utilities|String|ToString(Integer) (Variables|Default|GetEnemyRound)) " 
" "Tank:" (Utilities|String|ToString(Integer) _count) " 
" "Minion: " (Utilities|String|ToString(Integer) _count_3) " 
" "Bomber: " (Utilities|String|ToString(Integer) _count_2)) true true "(R=1.000000,G=0.000000,B=0.594255,A=1.000000)" (* (+ _count _count_3 _count_2 5) 0.5)))))

(event EventBeginPlay)

(event Collision|EventActorBeginOverlap
  (params (OtherActor :type Actor%20Object%20Reference)))

(event EventTick
  (params (DeltaSeconds :type Float%20%28single-precision%29))
  (CallFunction|CounterUpdate DeltaSeconds)
  ;[1 1 1] True when no enemies needs to spawn
  (if (== (Default|EnemiestoSpawnCount (Variables|Default|GetEnemySpawner)) 0)
    (if (Variables|Counter|GetInCounter)
      (if (== (Utilities|Array|Length (Variables|/Game/Gameplay/RoundController/BP_EnemySpawner.BP_EnemySpawner_C|GetAllSpawnedEnemies (Variables|Default|GetEnemySpawner))) 0)
        _))))

(fn ConstructionScript)

(fn CalculateHPTank
  (return (* (Math|Float|Power (LocalVariables|Getb) (* (- (Variables|Default|GetEnemyRound) 1) (LocalVariables|Getd))) (Variables|BaseHP|GetBaseHPTank))))

(fn CalculateHPMinion
  (return (* (Math|Float|Power (LocalVariables|Getb) (* (- (Variables|Default|GetEnemyRound) 1) (LocalVariables|Getd))) (Variables|BaseHP|GetBaseHPMinion))))

(fn CalculateHPBomber
  (return (* (Math|Float|Power (LocalVariables|Getb) (* (- (Variables|Default|GetEnemyRound) 1) (LocalVariables|Getd))) (Variables|BaseHP|GetBaseHPBomber))))

(fn CalculateHPPotTank
  (bind _newhp (CallFunction|HPPot (LocalVariables|Geta) (LocalVariables|Getb) (LocalVariables|Getd) (LocalVariables|Getk)))
  (return _newhp))

(fn HPPot
  (params (a :type Float%20%28single-precision%29) (b :type Float%20%28single-precision%29) (d :type Float%20%28single-precision%29) (k :type Float%20%28single-precision%29))
  ;[1 1 1] BasewertHP * b^[(Rundenanzahl-1)*d] + k
  (return (+ (* a (Math|Float|Power b (* (- (Variables|Default|GetEnemyRound) 1) d))) k)))

(fn CalculateHPPotMinion
  (bind _newhp (CallFunction|HPPot (LocalVariables|Geta) (LocalVariables|Getb) (LocalVariables|Getd) (LocalVariables|Getk)))
  (return _newhp))

(fn CalculateHPPotBomber
  (bind _newhp (CallFunction|HPPot (LocalVariables|Geta) (LocalVariables|Getb) (LocalVariables|Getd) (LocalVariables|Getk)))
  (return _newhp))

(fn EnemySpawnCount
  (params (Pot :type Float%20%28single-precision%29) (BaseHP :type Float%20%28single-precision%29))
  (return (Math|Integer|Max(Integer) (Math|Float|Truncate (/ Pot BaseHP)))))

(fn CounterUpdate
  (params (DeltaSeconds :type Float%20%28single-precision%29))
  ;[1 1 1] New wave starts if "InCounter" is false.
  (if (Variables|Counter|GetInCounter)
    ;[1 1 1] Check if enemies need to be spawn. Counter starts only if all enemies are spawned
    (if (== (Default|EnemiestoSpawnCount (Variables|Default|GetEnemySpawner)) 0)
      (Variables|Counter|SetCounterTimeTemp (- (Variables|Counter|GetCounterTimeTemp) DeltaSeconds))
      ;[1 1 1] Check if Enemies are on map. If no enemies are on the map, set timer to 0 and set "InCounter" to false so next frame the next wave spawns
      (if (== (Utilities|Array|Length (Variables|/Game/Gameplay/RoundController/BP_EnemySpawner.BP_EnemySpawner_C|GetAllSpawnedEnemies (Variables|Default|GetEnemySpawner))) 0)
        ;[1 1 1] No Enemies on Map, set Timer to 0
        (Variables|Counter|SetCounterTimeTemp 0.0)
        (Variables|Counter|SetInCounter false)
        (else
          ;[1 1 1] Check Timer. If timer is at 0, Set "InCounter" to false.
          (if (<= (Variables|Counter|GetCounterTimeTemp) 0.0)
            (Variables|Counter|SetInCounter false))))
      (else
        (return)))
    (else
      ;[1 1 1] If not in counter, spawn new wave. "InCounter" Variable is only false when counter is at 0. "InCounter" is set to true, else it would spawn the next wave next frame
      (CallFunction|NewWave)
      (Variables|Counter|SetCounterTimeTemp (Variables|Counter|GetCounterTime))
      (Variables|Counter|SetInCounter true))))