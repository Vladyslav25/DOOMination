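; Gameplay statistics collector for a wave-based tower game that writes a summary of the run through SaveXML on OnGameOver.
; Public functions accumulate per-tower builds, losses, shots, upgrades, kills and Argent spend, sorted by a cast-based Switch On BaseTower macro, with hardcoded build costs.
; Damage, hit and crit totals can also be swept from living BP_BaseEnemy actors.
; Wave and player stats are read from BP_RoundController and BP_Player at save time.
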(event Custom|OnGameOver
  (bind _player (CallFunction|GetPlayer))
  (bind (_playtimepistol _playtimeminigun _playtimeharpune _playtimesniper _playtimelmg _playtimeshotgun) (CallFunction|GetWeaponPlayTime _player))
  (Class|BDataCollector|SaveXML (.WavesCleared (CallFunction|GetWave)) (Variables|Player|AmountOfDamagebyPlayer|GetAmountOfDamageByPlayer) (TotalTowerAmount|TotalAmountOfDamagebyTurret) (TotalTowerAmount|TotalShotTowerShots) (Variables|/Game/Characters/PC/Blueprints/BP_Player.BP_Player_C|GetCompleteShootFired _player) (Variables|Player|AmountofPlayerShotsHit|GetAmountOfPlayerShotsHit) (Variables|Player|TotalAmountCrit|GetPlayerCrit) (Variables|/Game/Characters/PC/Blueprints/BP_Player.BP_Player_C|GetCollecedArgent _player) (Variables|/Game/Characters/PC/Blueprints/BP_Player.BP_Player_C|GetSpendedArgent _player) (+ (TotalTowerAmount|TotalSpendedAmountOfArgentforTowerBuilded) (TotalTowerAmount|TotalSpendedAmountOfArgentforTowerUpgrades)) (Variables|/Game/Characters/PC/Blueprints/BP_Player.BP_Player_C|GetAmountOfWepaonUpgrades _player) (TotalTowerAmount|TotalTowerBuilds) (TotalTowerAmount|TotalAmountOfUpgrades) _playtimepistol _playtimeminigun _playtimeharpune _playtimesniper _playtimelmg _playtimeshotgun (Variables|/Game/Characters/PC/Blueprints/BP_Player.BP_Player_C|GetDistance _player)))

(event EventBeginPlay)

(event Collision|EventActorBeginOverlap
  (params (OtherActor :type Actor%20Object%20Reference)))

(event EventTick
  (params (DeltaSeconds :type Float%20%28single-precision%29)))

(fn ConstructionScript)

(fn TowerSpawned
  (params (TowerReference :type BP%20Base%20Tower%20Object%20Reference) (Tower :type BP%20Base%20Tower%20Class%20Reference))
  (Utilities|SwitchonBaseTower TowerReference Tower
    (:Cannon
      (Math|Integer|IncrementInt (Variables|Tower|TurretsBuild|GetCannonsBuild)
        (:%20%20
          (Variables|SpendedAmountOfArgentForTurretBuilded|SetSpendedAmountOfArgentForCannonBuilded (+ 100 (Variables|SpendedAmountOfArgentForTurretBuilded|GetSpendedAmountOfArgentForCannonBuilded))))))
    (:Laser
      (Math|Integer|IncrementInt (Variables|Tower|TurretsBuild|GetLasersBuild)
        (:%20%20
          (Variables|SpendedAmountOfArgentForTurretBuilded|SetSpendedAmountOfArgentForLaserBuilded (+ 140 (Variables|SpendedAmountOfArgentForTurretBuilded|GetSpendedAmountOfArgentForLaserBuilded))))))
    (:Rifle
      (Math|Integer|IncrementInt (Variables|Tower|TurretsBuild|GetRiflesBuild)
        (:%20%20
          (Variables|SpendedAmountOfArgentForTurretBuilded|SetSpendedAmountOfArgentForRifleBuilded (+ 114 (Variables|SpendedAmountOfArgentForTurretBuilded|GetSpendedAmountOfArgentForRifleBuilded))))))
    (:RocketLauncher
      (Math|Integer|IncrementInt (Variables|Tower|TurretsBuild|GetRocketLaunchersBuild)
        (:%20%20
          (Variables|SpendedAmountOfArgentForTurretBuilded|SetSpendedAmountOfArgentForRocketLauncherBuilded (+ 124 (Variables|SpendedAmountOfArgentForTurretBuilded|GetSpendedAmountOfArgentForRocketLauncherBuilded))))))))

(fn TowerDestroyed
  (params (TowerRef :type BP%20Base%20Tower%20Object%20Reference) (TowerClass :type BP%20Base%20Tower%20Class%20Reference))
  (Utilities|SwitchonBaseTower TowerRef TowerClass
    (:Cannon
      (Math|Integer|IncrementInt (Variables|Tower|TurretsDestroyed|GetCannonsDestroyed)))
    (:Laser
      (Math|Integer|IncrementInt (Variables|Tower|TurretsDestroyed|GetLasersDestroyed)))
    (:Rifle
      (Math|Integer|IncrementInt (Variables|Tower|TurretsDestroyed|GetRiflesDestroyed)))
    (:RocketLauncher
      (Math|Integer|IncrementInt (Variables|Tower|TurretsDestroyed|GetRocketLaunchersDestroyed)))))

(fn AddSpendedAmountOfArgentforTurretUpgrades
  (params (TowerRef :type BP%20Base%20Tower%20Object%20Reference) (TowerClass :type BP%20Base%20Tower%20Class%20Reference) (ArgentSpended :type Integer))
  (Utilities|SwitchonBaseTower TowerRef TowerClass
    (:Cannon
      (Variables|Tower|SpendedAmountOfArgentForTurretUpgrades|SetSpendedAmountOfArgentForCannonUpgrades (+ (Variables|Tower|SpendedAmountOfArgentForTurretUpgrades|GetSpendedAmountOfArgentForCannonUpgrades) ArgentSpended)))
    (:Laser
      (Variables|Tower|SpendedAmountOfArgentForTurretUpgrades|SetSpendedAmountOfArgentForLaserUpgrades (+ ArgentSpended (Variables|Tower|SpendedAmountOfArgentForTurretUpgrades|GetSpendedAmountOfArgentForLaserUpgrades))))
    (:Rifle
      (Variables|Tower|SpendedAmountOfArgentForTurretUpgrades|SetSpendedAmountOfArgentForRifleUpgrades (+ ArgentSpended (Variables|Tower|SpendedAmountOfArgentForTurretUpgrades|GetSpendedAmountOfArgentForRifleUpgrades))))
    (:RocketLauncher
      (Variables|Tower|SpendedAmountOfArgentForTurretUpgrades|SetSpendedAmountOfArgentForRocketLauncherUpgrades (+ ArgentSpended (Variables|Tower|SpendedAmountOfArgentForTurretUpgrades|GetSpendedAmountOfArgentForRocketLauncherUpgrades))))))

(fn TotalSpendedAmountOfArgentforTowerBuilded
  (return (+ (Variables|SpendedAmountOfArgentForTurretBuilded|GetSpendedAmountOfArgentForCannonBuilded) (Variables|SpendedAmountOfArgentForTurretBuilded|GetSpendedAmountOfArgentForLaserBuilded) (Variables|SpendedAmountOfArgentForTurretBuilded|GetSpendedAmountOfArgentForRifleBuilded) (Variables|SpendedAmountOfArgentForTurretBuilded|GetSpendedAmountOfArgentForRocketLauncherBuilded))))

(fn TotalSpendedAmountOfArgentforTowerUpgrades
  (return (+ (Variables|Tower|SpendedAmountOfArgentForTurretUpgrades|GetSpendedAmountOfArgentForCannonUpgrades) (Variables|Tower|SpendedAmountOfArgentForTurretUpgrades|GetSpendedAmountOfArgentForLaserUpgrades) (Variables|Tower|SpendedAmountOfArgentForTurretUpgrades|GetSpendedAmountOfArgentForRifleUpgrades) (Variables|Tower|SpendedAmountOfArgentForTurretUpgrades|GetSpendedAmountOfArgentForRocketLauncherUpgrades))))

(fn TotalAmountOfDamagebyTurret
  (return (Variables|Tower|AmountOfDamagebyTurret|GetAmountOfDamageByTurret)))

(fn DeathbyTower
  (params (TowerRef :type BP%20Base%20Tower%20Object%20Reference) (TowerClass :type BP%20Base%20Tower%20Class%20Reference))
  (Utilities|SwitchonBaseTower TowerRef TowerClass
    (:Cannon
      (Math|Integer|IncrementInt (Variables|Tower|EnemiesKilledByTower|GetEnemiesKilledByCannon)))
    (:Laser
      (Math|Integer|IncrementInt (Variables|Tower|EnemiesKilledByTower|GetEnemiesKilledByLaser)))
    (:Rifle
      (Math|Integer|IncrementInt (Variables|Tower|EnemiesKilledByTower|GetEnemiesKilledByRifle)))
    (:RocketLauncher
      (Math|Integer|IncrementInt (Variables|Tower|EnemiesKilledByTower|GetEnemiesKilledByRocketLauncher)))
    (:Default
      (Development|PrintString "No Tower given!" true false "(R=1.000000,G=0.132595,B=0.092793,A=1.000000)"))))

(fn TotalShotTowerShots
  (return (+ (Variables|Tower|ShotTowerShots|GetShotCannonShots) (Variables|Tower|ShotTowerShots|GetShotLaserShots) (Variables|Tower|ShotTowerShots|GetShotRifleShots) (Variables|Tower|ShotTowerShots|GetShotRocketLauncherShots))))

(fn TotalTowerBuilds
  (return (+ (Variables|Tower|TurretsBuild|GetCannonsBuild) (Variables|Tower|TurretsBuild|GetLasersBuild) (Variables|Tower|TurretsBuild|GetRiflesBuild) (Variables|Tower|TurretsBuild|GetRocketLaunchersBuild))))

(fn TotalTowerDestroyed
  (return (+ (Variables|Tower|TurretsDestroyed|GetCannonsDestroyed) (Variables|Tower|TurretsDestroyed|GetLasersDestroyed) (Variables|Tower|TurretsDestroyed|GetRiflesDestroyed) (Variables|Tower|TurretsDestroyed|GetRocketLaunchersDestroyed))))

(fn TotalEnemieKilledbyTower
  (return (+ (Variables|Tower|EnemiesKilledByTower|GetEnemiesKilledByCannon) (Variables|Tower|EnemiesKilledByTower|GetEnemiesKilledByLaser) (Variables|Tower|EnemiesKilledByTower|GetEnemiesKilledByRifle) (Variables|Tower|EnemiesKilledByTower|GetEnemiesKilledByRocketLauncher))))

(fn AddCannonShots
  (params (CannonShots :type Integer))
  (bind _output_get (Variables|Tower|ShotTowerShots|SetShotCannonShots (+ CannonShots (Variables|Tower|ShotTowerShots|GetShotCannonShots))))
  (return _output_get))

(fn AddLaserShots
  (params (LaserShots :type Integer))
  (bind _output_get (Variables|Tower|ShotTowerShots|SetShotLaserShots (+ LaserShots (Variables|Tower|ShotTowerShots|GetShotLaserShots))))
  (return _output_get))

(fn AddRifleShots
  (params (RifleShots :type Integer))
  (bind _output_get (Variables|Tower|ShotTowerShots|SetShotRifleShots (+ RifleShots (Variables|Tower|ShotTowerShots|GetShotRifleShots))))
  (return _output_get))

(fn AddRocketLauncherShots
  (params (RocketLauncherShots :type Integer))
  (bind _output_get (Variables|Tower|ShotTowerShots|SetShotRocketLauncherShots (+ RocketLauncherShots (Variables|Tower|ShotTowerShots|GetShotRocketLauncherShots))))
  (return _output_get))

(fn AddCannonUpgrade
  (params (CannonUpgrades :type Integer))
  (bind _output_get (Variables|Tower|AmountTurretUpgraded|SetAmountCannonUpgraded (+ CannonUpgrades (Variables|Tower|AmountTurretUpgraded|GetAmountCannonUpgraded))))
  (return _output_get))

(fn AddLaserUpgrade
  (params (LaserUpgrades :type Integer))
  (bind _output_get (Variables|Tower|AmountTurretUpgraded|SetAmountLaserUpgraded (+ LaserUpgrades (Variables|Tower|AmountTurretUpgraded|GetAmountLaserUpgraded))))
  (return _output_get))

(fn AddRifleUpgrade
  (params (RifleUpgrades :type Integer))
  (bind _output_get (Variables|Tower|AmountTurretUpgraded|SetAmountRifleUpgraded (+ RifleUpgrades (Variables|Tower|AmountTurretUpgraded|GetAmountRifleUpgraded))))
  (return _output_get))

(fn AddRocketLauncherUpgrade
  (params (RocketLauncherUpgrades :type Integer))
  (bind _output_get (Variables|Tower|AmountTurretUpgraded|SetAmountRocketLauncherUpgraded (+ RocketLauncherUpgrades (Variables|Tower|AmountTurretUpgraded|GetAmountRocketLauncherUpgraded))))
  (return _output_get))

(fn TotalAmountOfUpgrades
  (return (+ (Variables|Tower|AmountTurretUpgraded|GetAmountCannonUpgraded) (Variables|Tower|AmountTurretUpgraded|GetAmountLaserUpgraded) (Variables|Tower|AmountTurretUpgraded|GetAmountRifleUpgraded) (Variables|Tower|AmountTurretUpgraded|GetAmountRocketLauncherUpgraded))))

(fn AddAmountOfDamage
  (params (TowerDamage :type Float%20%28single-precision%29) (PlayerDamage :type Float%20%28single-precision%29))
  (bind _output_get (Variables|Tower|AmountOfDamagebyTurret|SetAmountOfDamageByTurret (+ TowerDamage (Variables|Tower|AmountOfDamagebyTurret|GetAmountOfDamageByTurret))))
  (bind _output_get_2 (Variables|Player|AmountOfDamagebyPlayer|SetAmountOfDamageByPlayer (+ PlayerDamage (Variables|Player|AmountOfDamagebyPlayer|GetAmountOfDamageByPlayer))))
  (return _output_get _output_get_2))

(fn GetWave
  (bind _returnvalue (Actor|GetActorOfClass "/Game/Gameplay/RoundController/BP_RoundController.BP_RoundController_C"))
  (return (- (Variables|/Game/Gameplay/RoundController/BP_RoundController.BP_RoundController_C|GetEnemyRound _returnvalue) 1) (Variables|/Game/Gameplay/RoundController/BP_RoundController.BP_RoundController_C|GetEnemyRound _returnvalue) _returnvalue))

(fn GetPlayer
  (bind _asbp_player (Utilities|Casting|CastToBP_Player (Pawn|GetControlledPawn (Game|GetPlayerController 0)))
    (:then
      (return _asbp_player))
    (:CastFailed
      (return 0))))

(fn GetWeaponPlayTime
  (params (Player :type BP%20Player%20Object%20Reference))
  (bind _weapontimer (Variables|/Game/Characters/PC/Blueprints/BP_Player.BP_Player_C|GetWeaponTimer Player))
  (return (Utilities|Array|Get(acopy) _weapontimer) (Utilities|Array|Get(acopy) _weapontimer 1) (Utilities|Array|Get(acopy) _weapontimer 2) (Utilities|Array|Get(acopy) _weapontimer 3) (Utilities|Array|Get(acopy) _weapontimer 4) (Utilities|Array|Get(acopy) _weapontimer 5)))

(fn AddCrit
  (params (Crit :type Integer))
  (bind _output_get (Variables|Player|TotalAmountCrit|SetPlayerCrit (+ Crit (Variables|Player|TotalAmountCrit|GetPlayerCrit))))
  (return _output_get))

(fn AddShotsHitPlayer
  (params (ShotsHit :type Integer))
  (Variables|Player|AmountofPlayerShotsHit|SetAmountOfPlayerShotsHit (+ ShotsHit (Variables|Player|AmountofPlayerShotsHit|GetAmountOfPlayerShotsHit))))

(fn AddDatafromEnemiesinScene
  (bind _outactors (Actor|GetAllActorsOfClass "/Game/Characters/NPC/Enemies/Blueprints/BP_BaseEnemy.BP_BaseEnemy_C"))
  (for _array_element _outactors
    (CallFunction|AddShotsHitPlayer (Variables|/Game/Characters/NPC/Enemies/Blueprints/BP_BaseEnemy.BP_BaseEnemy_C|GetPlayerShotHit _array_element))
    (CallFunction|AddCrit (Variables|/Game/Characters/NPC/Enemies/Blueprints/BP_BaseEnemy.BP_BaseEnemy_C|GetCritAmountByPlayer _array_element))
    (AddDamage|AddAmountOfDamage (Variables|/Game/Characters/NPC/Enemies/Blueprints/BP_BaseEnemy.BP_BaseEnemy_C|GetTotalDamageByTower _array_element) (Variables|/Game/Characters/NPC/Enemies/Blueprints/BP_BaseEnemy.BP_BaseEnemy_C|GetTotalDamageByPlayer _array_element)))
  (return))