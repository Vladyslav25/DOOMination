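; Static mesh component that hovers by bobbing vertically above the world location it has at BeginPlay.
; Each tick advances a timer by hover speed and feeds its degree-based sine into a lerp between raised and spawn positions.
; The unclamped -1 to 1 alpha makes it swing from spawn up to twice HoverHeight.
; A random offset is added every tick, so it varies bob speed per instance and depends on frame rate.
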(event EventTick
  (params (DeltaSeconds :type Float%20%28single-precision%29))
  (bind _spawnpos (Variables|Default|GetSpawnPos))
  (bind _output_get (Variables|Default|SetSin%20Timer (+ (* DeltaSeconds (Variables|HowerSettings|GetHoverSpeed)) (Variables|Default|GetSin%20Timer) (Variables|Default|GetRandomOffset))))
  (Transformation|SetWorldLocation (Math|Vector|Lerp(Vector) (Math|Vector|MakeVector (.x _spawnpos) (.y _spawnpos) (+ (.z _spawnpos) (Variables|HowerSettings|GetHoverHeight))) (Math|Vector|MakeVector (.x _spawnpos) (.y _spawnpos) (.z _spawnpos)) (Math|Trig|Sin(Degrees) _output_get)) false false))

(event EventBeginPlay
  (Variables|Default|SetSpawnPos (Transformation|GetWorldLocation))
  (Variables|Default|SetRandomOffset (Math|Random|RandomFloatinRange 0.0 1.0)))