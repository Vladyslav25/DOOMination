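; BP_Argent is an Argent pickup actor, scaled by its amount within clamped limits, that hovers on a sine wave around its spawn point.
; A PlayerOverlap macro distinguishes the player's magnet, which triggers flight toward the player with a timeline-driven Niagara mesh scale, from the collector, which adds Argent and destroys the pickup.
; SpawnNewArgent can split excess amount into another nearby pickup, but nothing here calls it.
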(event OnComponentBeginOverlap(Sphere)
  (params (OverlappedComponent :type Primitive%20Component%20Object%20Reference) (OtherActor :type Actor%20Object%20Reference) (OtherComp :type Primitive%20Component%20Object%20Reference) (OtherBodyIndex :type Integer) (bFromSweep :type Boolean) (SweepResult :type Hit%20Result%20Structure%20%28by%20ref%29))
  (bind _asbp_player (Utilities|Casting|CastToBP_Player OtherActor))
  (bind _output_get (Variables|Member|SetPlayerRef _asbp_player))
  (Utilities|PlayerOverlap _output_get OtherComp
    (:IsPlayerMagnet
      (Variables|Settings|SetFlyToPlayer true))
    (:IsPlayerCollector
      (Default|AddArgent _asbp_player (Variables|Settings|GetArgentAmount))
      (Actor|DestroyActor))))

(event EventTick
  (params (DeltaSeconds :type Float%20%28single-precision%29))
  (bind _playerref (Variables|Member|GetPlayerRef))
  (bind _hoverheight (Variables|HowerSettings|GetHoverHeight))
  (bind _spawnpos (Variables|Member|GetSpawnPos))
  (if (Variables|Settings|GetFlyToPlayer)
    (Utilities|FlowControl|Sequence
      (:then_0
        (bind _scale (Timeline|ParticelMeshSclae Play)
          (:Update
            (Effects|Components|ParticleSystem|SetFloatParameter (Variables|Default|GetNiagara) "MeshScale" _scale))))
      (:then_1
        (Utilities|IsValid _playerref
          (:Is%20Valid
            (Components|MoveComponentTo (Variables|Default|GetRoot) (Transformation|GetActorLocation _playerref) "0, 0, 0" false false 0.3 true)))))
    (else
      (bind _output_get (Variables|Member|SetSin%20Timer (+ (* DeltaSeconds (Variables|HowerSettings|GetHoverSpeed)) (Variables|Member|GetSin%20Timer))))
      (Transformation|SetWorldLocation (Variables|Default|GetRoot) (Math|Vector|Lerp(Vector) (Math|Vector|MakeVector (.x _spawnpos) (.y _spawnpos) (+ (.z _spawnpos) _hoverheight)) (Math|Vector|MakeVector (.x _spawnpos) (.y _spawnpos) (- (.z _spawnpos) _hoverheight)) (Math|Trig|Sin(Degrees) _output_get)) false false))))

(event EventBeginPlay
  (bind _amountscaleweight (Variables|Settings|GetAmountScaleWeight))
  (bind _argentamount (Variables|Settings|GetArgentAmount))
  (bind _returnvalue (* _argentamount _amountscaleweight))
  (bind _returnvalue_2 (Math|Float|Clamp(Float) _returnvalue 0.3 1.3))
  (Transformation|SetWorldScale3D (Variables|Default|GetRoot) (Math|Vector|MakeVector _returnvalue_2 _returnvalue_2 _returnvalue_2))
  (Variables|Member|SetSpawnPos (Transformation|GetActorLocation))
  (if (Variables|Settings|GetFlyToPlayer)
    (bind _asbp_player (Utilities|Casting|CastToBP_Player (Game|Player|GetPlayerPawn 0)))
    (Variables|Member|SetPlayerRef _asbp_player)
    (Effects|Components|ParticleSystem|SetFloatParameter (Variables|Default|GetNiagara) "MeshScale" 1.0)))

(fn ConstructionScript)

(fn SpawnNewArgent
  (Game|SpawnActorfromClass "BP_Argent_C" (Math|Transform|MakeTransform (CallFunction|GetRandomLocationAround (.location (Transformation|GetActorTransform)) 1e+02 1.5e+02) "0, 0, 0" "1,1,1") "Undefined" 0 (- (Variables|Settings|GetArgentAmount) (Variables|Settings|GetMaxArgentAmount)) false 0)
  (Variables|Settings|SetArgentAmount (Variables|Settings|GetMaxArgentAmount)))

(fn GetRandomLocationAround
  (params (Origion :type Vector) (MinRadius :type Float%20%28single-precision%29) (Max%20Radius :type Float%20%28single-precision%29))
  (return (+ Origion (Math|Vector|RotateVector (Math|Vector|MakeVector 0.0 (Math|Random|RandomFloatinRange MinRadius Max%20Radius) 0.0) (Math|Rotator|MakeRotator 0.0 0.0 (Math|Random|RandomFloatinRange 0.0 359.0))))))