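; BP_Argent is an Argent pickup that scales with its amount and adds it to BP_BPlayer when collected.
; On BeginPlay it destroys itself if empty, or caps its amount and spawns the excess as another pickup nearby.
; Tick bobs it on a sine, faster for smaller amounts, until the player's magnet component triggers a MoveComponentTo flight toward the player.
; Overlapping the player's collector component awards the Argent and destroys the pickup.
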(event OnComponentBeginOverlap(StaticMesh)
  (params (OverlappedComponent :type Primitive%20Component%20Object%20Reference) (OtherActor :type Actor%20Object%20Reference) (OtherComp :type Primitive%20Component%20Object%20Reference) (OtherBodyIndex :type Integer) (bFromSweep :type Boolean) (SweepResult :type Hit%20Result%20Structure%20%28by%20ref%29))
  (bind _asbp_bplayer (Utilities|Casting|CastToBP_BPlayer OtherActor))
  (bind _output_get (Variables|Member|SetPlayerRef _asbp_bplayer))
  (Utilities|PlayerOverlap _output_get OtherComp
    (:IsPlayerMagnet
      (Variables|Settings|SetFlyToPlayer true))
    (:IsPlayerCollector
      (Default|AddArgent _asbp_bplayer (Variables|Settings|GetArgentAmount))
      (Actor|DestroyActor))))

(event EventTick
  (params (DeltaSeconds :type Float%20%28single-precision%29))
  (bind _hoverheight (Variables|HowerSettings|GetHoverHeight))
  (bind _spawnpos (Variables|Member|GetSpawnPos))
  (if (Variables|Settings|GetFlyToPlayer)
    (Components|MoveComponentTo (Variables|Default|GetRoot) (Transformation|GetActorLocation (Variables|Member|GetPlayerRef)) "0, 0, 0" false false 0.3 true)
    (else
      (bind _output_get (Variables|Member|SetSin%20Timer (+ (* DeltaSeconds (Variables|HowerSettings|GetHoverSpeed)) (Variables|Member|GetSin%20Timer) (* (- 1.0 (/ (Math|Conversions|ToFloat(Integer) (Variables|Settings|GetArgentAmount)) (Math|Conversions|ToFloat(Integer) (Variables|Settings|GetMaxArgentAmount)))) (Variables|HowerSettings|GetAmountWeight)))))
      (Transformation|SetWorldLocation (Variables|Default|GetRoot) (Math|Vector|Lerp(Vector) (Math|Vector|MakeVector (.x _spawnpos) (.y _spawnpos) (+ (.z _spawnpos) _hoverheight)) (Math|Vector|MakeVector (.x _spawnpos) (.y _spawnpos) (- (.z _spawnpos) _hoverheight)) (Math|Trig|Sin(Degrees) _output_get)) false false))))

(event EventBeginPlay
  (bind _argentamount (Variables|Settings|GetArgentAmount))
  (bind _argentamount_2 (Variables|Settings|GetArgentAmount))
  (bind _returnvalue (* _argentamount 0.02))
  (if (<= _argentamount_2 0)
    (Actor|DestroyActor)
    (else
      (if (> _argentamount_2 (Variables|Settings|GetMaxArgentAmount))
        (CallFunction|SpawnNewArgent))
      (Transformation|SetWorldScale3D (Variables|Default|GetStaticMesh) (Math|Vector|MakeVector _returnvalue _returnvalue _returnvalue))
      (Variables|Member|SetSpawnPos (Transformation|GetActorLocation))
      (if (Variables|Settings|GetFlyToPlayer)
        (bind _asbp_bplayer (Utilities|Casting|CastToBP_BPlayer (Game|Player|GetPlayerPawn 0)))
        (Variables|Member|SetPlayerRef _asbp_bplayer)))))

(fn ConstructionScript)

(fn SpawnNewArgent
  (Game|SpawnActorfromClass "BP_Argent_C" (Math|Transform|MakeTransform (CallFunction|GetRandomLocationAround (.location (Transformation|GetActorTransform)) 1e+02 1.5e+02) "0, 0, 0" "1,1,1") "Undefined" 0 (- (Variables|Settings|GetArgentAmount) (Variables|Settings|GetMaxArgentAmount)) false 0)
  (Variables|Settings|SetArgentAmount (Variables|Settings|GetMaxArgentAmount)))

(fn GetRandomLocationAround
  (params (Origion :type Vector) (MinRadius :type Float%20%28single-precision%29) (Max%20Radius :type Float%20%28single-precision%29))
  (return (+ Origion (Math|Vector|RotateVector (Math|Vector|MakeVector 0.0 (Math|Random|RandomFloatinRange MinRadius Max%20Radius) 0.0) (Math|Rotator|MakeRotator 0.0 0.0 (Math|Random|RandomFloatinRange 0.0 359.0))))))