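; BP_Shield is a shield object that animates the M_Shield material on its Sphere component.
; BeginPlay creates a dynamic material instance, zeroes its SpeedX and SpeedY parameters and seeds two matching variables with random values.
; Each Tick advances both variables by randomly jittered delta time scaled by RotSpeed, then feeds their sines, scaled by RotMulti, into the material for irregular oscillating motion.
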(event EventBeginPlay
  (bind _returnvalue (Rendering|Material|CreateDynamicMaterialInstance (Variables|Default|GetSphere) 0 "/Game/Effects/Mastermatrial/M_Shield.M_Shield" "None" :!class /Script/Engine.PrimitiveComponent))
  (bind _output_get (Variables|Default|SetMaterialInstanceRef _returnvalue))
  (Utilities|FlowControl|Sequence
    (:then_0
      (Rendering|Material|SetScalarParameterValue _output_get "SpeedX" 0.0 :!class /Script/Engine.MaterialInstanceDynamic)
      (Variables|Default|SetSpeedX (Math|Random|RandomFloatinRange -1.0 1.0)))
    (:then_1
      (Rendering|Material|SetScalarParameterValue _output_get "SpeedY" 0.0 :!class /Script/Engine.MaterialInstanceDynamic)
      (Variables|Default|SetSpeedY (Math|Random|RandomFloatinRange -1.0 1.0)))))

(event EventTick
  (params (DeltaSeconds :type Float%20%28single-precision%29))
  (bind _materialinstanceref (Variables|Default|GetMaterialInstanceRef))
  (Variables|Default|SetSpeedX (+ (* (+ DeltaSeconds (Math|Random|RandomFloatinRange 0.0 DeltaSeconds)) (Variables|Default|GetRotSpeed)) (Variables|Default|GetSpeedX)))
  (Variables|Default|SetSpeedY (+ (* (+ DeltaSeconds (Math|Random|RandomFloatinRange 0.0 DeltaSeconds)) (Variables|Default|GetRotSpeed)) (Variables|Default|GetSpeedY)))
  (Rendering|Material|SetScalarParameterValue _materialinstanceref "SpeedX" (* (Variables|Default|GetRotMulti) (Math|Trig|Sin(Radians) (Variables|Default|GetSpeedX))) :!class /Script/Engine.MaterialInstanceDynamic)
  (Rendering|Material|SetScalarParameterValue _materialinstanceref "SpeedY" (* (Variables|Default|GetRotMulti) (Math|Trig|Sin(Radians) (Variables|Default|GetSpeedY))) :!class /Script/Engine.MaterialInstanceDynamic))

(fn ConstructionScript)