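; Base weapon actor that auto-fires projectiles while fire is held, with growing spray and vertical recoil.
; Tick re-fires whenever the ShotTimer timeline re-arms CanShot; each shot spawns at Hole along Arrow, then randomly rotates Arrow within CurrSpray-scaled bounds for the next.
; The RecoilRot timeline drives recoil, which Tick passes to BP_BPlayer.
; The SprayDecrese timeline delays spray decay, which eases Arrow back toward center.
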(event Custom|Recoile
  (Variables|Members|SetTmpWeaponRotY (.pitch (Variables|/Script/Engine.SceneComponent|GetRelativeRotation (Variables|Components|GetRoot))))
  ;[1 1 1] The Delta Recoil Rotation. Set the Recoile Rotation. (Delta: Start with 0 and end with 0)
  (bind _recoilamount (Timeline|Recoil%20Rot PlayFromStart)
    (:Update
      (Variables|Members|SetRecoileRot (* _recoilamount (Variables|WeaponSettingsValues|GetRecoilMulti)))
      ;[1 1 1] When the timer finished the currSpray can decrese. After the Recoil the Timer start. And after finish its reset
      (Timeline|SprayDecrese PlayFromStart
        (:Finished
          (Variables|Members|SetCanSprayDecrease true)
          (Timeline|SprayDecrese SetNewTime))))))

(event Custom|Fire_Pressed
  (Variables|Members|SetIsFirering true)
  (Variables|Members|SetCanSprayDecrease false)
  (Variables|Members|SetIsPressed true)
  (if (and (Variables|Members|GetCanShot) (Variables|Members|GetIsPressed))
    (CallFunction|Shoot)
    (Variables|Members|SetCanShot false)
    (Utilities|FlowControl|Sequence
      (:then_0
        ;[1 1 1] Whe the timer finish the "Can Shot" sets to true
        (Timeline|ShotTimer Play
          (:Finished
            (Utilities|FlowControl|Sequence
              (:then_0
                (Variables|Members|SetCanShot true))
              (:then_1
                (Timeline|ShotTimer SetNewTime))))))
      (:then_1
        ;[1 1 1] When the timer finished the currSpray can decrese. After the Recoil the Timer start. And after finish its reset
        (Timeline|SprayDecrese Stop
          (:Finished
            (Variables|Members|SetCanSprayDecrease true)
            (Timeline|SprayDecrese SetNewTime)))))))

(event Custom|Fire_Relesed
  (Variables|Members|SetIsFirering false)
  (Variables|Members|SetIsPressed false))

(event EventBeginPlay
  (Input|EnableInput (Game|GetPlayerController 0))
  (Components|Timeline|SetPlayRate (Variables|Default|GetSprayDecrese) (/ 1.0 (Variables|WeaponSettingsValues|GetSprayResetTime)))
  (Components|Timeline|SetPlayRate (Variables|Default|GetRecoil%20Rot) (/ 1.0 (Variables|Members|GetRecoileRotSpeed)))
  (Components|Timeline|SetPlayRate (Variables|Default|GetShotTimer) (/ 1.0 (Variables|WeaponSettingsValues|GetMaxFireTimer)))
  (bind _asbp_bplayer (Utilities|Casting|CastToBP_BPlayer (Game|Player|GetPlayerPawn 0)))
  (Variables|Members|SetPlayerRef _asbp_bplayer))

(event EventTick
  (params (DeltaSeconds :type Float%20%28single-precision%29))
  (bind _arrow (Variables|Components|GetArrow))
  (Utilities|FlowControl|Sequence
    (:then_0
      (Default|SetVerticalWeaponRecoile (Variables|Members|GetPlayerRef) (Variables|Members|GetRecoileRot))
      (if (Variables|Members|GetCanSprayDecrease)
        (bind _output_get (Variables|Members|SetCurrSpray (Math|Float|Clamp(Float) (- (Variables|Members|GetCurrSpray) (* (Variables|WeaponSettingsValues|GetSprayDecreaseSpeed) DeltaSeconds)))))
        (Transformation|SetRelativeRotation _arrow (Math|Rotator|Lerp(Rotator) "0, 0, 0" (Variables|/Script/Engine.SceneComponent|GetRelativeRotation _arrow) _output_get) false false)))
    (:then_1
      (if (and (Variables|Members|GetCanShot) (Variables|Members|GetIsPressed))
        (CallFunction|Shoot)
        (Variables|Members|SetCanShot false)
        (Utilities|FlowControl|Sequence
          (:then_0
            ;[1 1 1] Whe the timer finish the "Can Shot" sets to true
            (Timeline|ShotTimer Play
              (:Finished
                (Utilities|FlowControl|Sequence
                  (:then_0
                    (Variables|Members|SetCanShot true))
                  (:then_1
                    (Timeline|ShotTimer SetNewTime))))))
          (:then_1
            ;[1 1 1] When the timer finished the currSpray can decrese. After the Recoil the Timer start. And after finish its reset
            (Timeline|SprayDecrese Stop
              (:Finished
                (Variables|Members|SetCanSprayDecrease true)
                (Timeline|SprayDecrese SetNewTime)))))))))

(fn ConstructionScript)

(fn Shoot
  (bind _minspraystep (Variables|WeaponSettingsValues|GetMinSprayStep))
  (bind _maxspraystep (Variables|WeaponSettingsValues|GetMaxSprayStep))
  (bind _returnvalue (Game|SpawnActorfromClass "/Game/Gameplay/Weapon/BP_BaseProjectile.BP_BaseProjectile_C" (Math|Transform|MakeTransform (Transformation|GetWorldLocation (Variables|Components|GetHole)) "0, 0, 0" "1,1,1") "AdjustIfPossibleButAlwaysSpawn" 0 0))
  (Variables|/Script/Engine.MovementComponent|SetVelocity (Variables|/Game/Gameplay/Weapon/BP_BaseProjectile.BP_BaseProjectile_C|GetProjectileMovement _returnvalue) (* (Math|Vector|GetForwardVector (Variables|Components|GetArrow)) 999.0))
  (bind _rotation (CallFunction|GetRandomRotation _minspraystep (Math|Float|Clamp(Float) (* (Variables|Members|GetCurrSpray) _maxspraystep) _minspraystep _maxspraystep)))
  (Variables|Members|SetCurrSpray (Math|Float|Clamp(Float) (+ (Variables|Members|GetCurrSpray) (Variables|WeaponSettingsValues|GetAddCurrSpray))))
  (Transformation|SetRelativeRotation (Variables|Components|GetArrow) _rotation false false)
  (CallFunction|Recoile))

(fn GetRandomRotation
  (params (Min :type Float%20%28single-precision%29) (Max :type Float%20%28single-precision%29))
  (LocalVariables|SetRotZ (Math|Random|RandomFloatinRange Min Max))
  (LocalVariables|SetRotY (Math|Random|RandomFloatinRange Min Max))
  (if (Math|Random|RandomBool)
    (LocalVariables|SetRotZ (* (LocalVariables|GetRotZ) -1.0)))
  (if (Math|Random|RandomBool)
    (LocalVariables|SetRotY (* (LocalVariables|GetRotY) -1.0)))
  (return (Math|Rotator|MakeRotator 0.0 (LocalVariables|GetRotY) (LocalVariables|GetRotZ))))