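; Shotgun projectile Blueprint that loses damage the longer it is in flight, limiting its effective range.
; BeginPlay gives it a lifespan of a fraction of a second.
; Each Tick lowers DamageAmount at a fixed rate scaled by delta time and destroys the actor once it reaches zero.
; The construction script only calls the parent's.
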(event EventBeginPlay
  (Actor|SetLifeSpan 0.1))

(event EventTick
  (params (DeltaSeconds :type Float%20%28single-precision%29))
  (bind _output_get (Variables|Default|SetDamageAmount (- (Variables|Default|GetDamageAmount) (* DeltaSeconds 1.5e+03))))
  (if (<= _output_get 0.0)
    (Actor|DestroyActor)))

(fn ConstructionScript
  (|CallParentFunction))