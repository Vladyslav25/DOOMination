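; Harpoon projectile that stays inactive until Fire launches it along an arrow's forward vector with gravity.
; While airborne, a short forward line trace each tick, ignoring tower points, detects hits instead of collision events.
; On a hit it sticks to the actor with a limited lifespan, damaging enemies with a hitmarker sound and double damage on Head-tagged components.
; Hits on projectile despawners destroy it.
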(event Custom|Fire
  (params (Arrow :type Arrow%20Component%20Object%20Reference))
  (bind _projectilemovement (Variables|Default|GetProjectileMovement))
  (Variables|Default|SetInAir true)
  (Components|Activation|SetActive _projectilemovement true false)
  (Variables|/Script/Engine.MovementComponent|SetVelocity _projectilemovement (* (Math|Vector|GetForwardVector Arrow) (Variables|Default|GetSpeedMulti)))
  (Variables|/Script/Engine.ProjectileMovementComponent|SetbRotationFollowsVelocity _projectilemovement true)
  (Variables|/Script/Engine.ProjectileMovementComponent|SetProjectileGravityScale _projectilemovement 0.8))

(event EventBeginPlay
  (Components|Activation|Deactivate (Variables|Default|GetProjectileMovement))
  (bind _outactors (Actor|GetAllActorsOfClass "/Game/Characters/NPC/Turrets/Blueprints/BlueprintTower/BP_TowerPoint.BP_TowerPoint_C"))
  (Variables|Default|SetActorsToIgnore _outactors))

(event EventTick
  (params (DeltaSeconds :type Float%20%28single-precision%29))
  (bind _returnvalue (Transformation|GetActorLocation))
  (if (Variables|Default|GetInAir)
    (bind (_outhit _returnvalue_2) (Collision|LineTraceByChannel _returnvalue (+ _returnvalue (* (Transformation|GetActorForwardVector) 8e+01)) "TraceTypeQuery1" true (Variables|Default|GetActorsToIgnore) "None"))
    (if _returnvalue_2
      (Utilities|FlowControl|Sequence
        (:then_0
          (Transformation|SetActorLocation (.location _outhit) false true)
          (Transformation|AttachActorToActor (.hitactor _outhit) "None" "KeepWorld" "KeepWorld" "KeepWorld" false)
          (Components|Activation|Deactivate (Variables|Default|GetProjectileMovement))
          (Collision|SetCollisionEnabled (Variables|Default|GetCollider) "NoCollision")
          (Variables|Default|SetInAir false)
          (Actor|SetLifeSpan 6e+01)
          (bind _asbp_base_enemy (Utilities|Casting|CastToBP_BaseEnemy (.hitactor _outhit)))
          (Utilities|IsValid _asbp_base_enemy
            (:Is%20Valid
              (if (Components|ComponentHasTag (.hitcomponent _outhit) "Head")
                (Game|Damage|ApplyDamage _asbp_base_enemy (* (Variables|Default|GetDamageAmount) 2.0) 0 self "/Game/Characters/NPC/Turrets/Blueprints/BT_PlayerDamagaType.BT_PlayerDamagaType_C")
                (Development|PrintString "Crit")
                (else
                  (Game|Damage|ApplyDamage _asbp_base_enemy (Variables|Default|GetDamageAmount) 0 self "/Game/Characters/NPC/Turrets/Blueprints/BT_PlayerDamagaType.BT_PlayerDamagaType_C")))
              (Class|FMODBlueprintStatics|PlayEvent2D "/Game/FMOD/Events/Gunshots/hitmarker.hitmarker"))))
        (:then_1
          (Utilities|Casting|CastToBP_ProjectileDespawner (.hitactor _outhit))
          (Actor|DestroyActor))))))

(fn ConstructionScript
  (|CallParentFunction))