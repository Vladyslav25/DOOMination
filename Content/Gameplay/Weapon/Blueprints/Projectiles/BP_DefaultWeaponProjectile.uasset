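; Default weapon projectile that spawns a Niagara impact effect on hit and reacts to what it struck.
; A CastActor macro sorts the hit actor by exact class into enemy, shield, despawner or other.
; Enemies take player-type damage with a 2D hitmarker event, then the projectile is destroyed, as it is on despawners and other actors.
; Shields instead receive the impact location through a dynamic material parameter, without destroying the projectile.
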(event EventBeginPlay
  (|CallParentFunction) ; This node is disabled and will not be called.\nDrag off pins to build functionality.
)

(event Collision|EventHit
  (params (MyComp :type Primitive%20Component%20Object%20Reference) (Other :type Actor%20Object%20Reference) (OtherComp :type Primitive%20Component%20Object%20Reference) (bSelfMoved :type Boolean) (HitLocation :type Vector :default "0, 0, 0") (HitNormal :type Vector :default "0, 0, 0") (NormalImpulse :type Vector :default "0, 0, 0") (Hit :type Hit%20Result%20Structure%20%28by%20ref%29))
  (bind _returnvalue (Niagara|SpawnSystematLocation "/Game/Effects/Weapons/OnHit/NS_OnHit.NS_OnHit" HitLocation (Math|Rotator|MakeRotfromX HitNormal)))
  (bind (_baseenemy_actor _shield_actor) (Utilities|CastActor Other)
    (:BaseEnemy
      (Utilities|IsValid _baseenemy_actor
        (:Is%20Valid
          (Game|Damage|ApplyDamage 0 (Variables|Default|GetDamageAmount) 0 self "/Game/Characters/NPC/Turrets/Blueprints/BT_PlayerDamagaType.BT_PlayerDamagaType_C")
          (Class|FMODBlueprintStatics|PlayEvent2D "/Game/FMOD/Events/Gunshots/hitmarker.hitmarker")
          (Actor|DestroyActor :!label _label))))
    (:Shield
      (bind _returnvalue_2 (Rendering|Material|CreateDynamicMaterialInstance (Variables|/Game/Gameplay/Shield/BP_Shield.BP_Shield_C|GetSphere _shield_actor) 0 0 "None" :!class /Script/Engine.PrimitiveComponent))
      (Rendering|Material|SetVectorParameterValue _returnvalue_2 "Location" (Math|Conversions|ToLinearColor(Vector) (Transformation|GetWorldLocation _returnvalue)) :!class /Script/Engine.MaterialInstanceDynamic))
    (:Despawner
      (goto _label))
    (:Other
      (goto _label))))

(event EventTick
  (params (DeltaSeconds :type Float%20%28single-precision%29))
  (|CallParentFunction DeltaSeconds) ; This node is disabled and will not be called.\nDrag off pins to build functionality.
)

(fn ConstructionScript
  (|CallParentFunction))