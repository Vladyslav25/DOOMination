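; BP_SniperProjectile is a piercing sniper shot that damages enemies it passes through.
; Its sphere's begin-overlap applies player-typed damage to BP_BaseEnemy actors, halves the remaining damage after each hit and plays a 2D hitmarker event.
; Overlapping a BP_ProjectileDespawner or any other non-enemy actor destroys the projectile.
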(event OnComponentBeginOverlap(Sphere)
  (params (OverlappedComponent :type Primitive%20Component%20Object%20Reference) (OtherActor :type Actor%20Object%20Reference) (OtherComp :type Primitive%20Component%20Object%20Reference) (OtherBodyIndex :type Integer) (bFromSweep :type Boolean) (SweepResult :type Hit%20Result%20Structure%20%28by%20ref%29))
  (Utilities|Casting|CastToBP_ProjectileDespawner OtherActor
    (:then
      (Actor|DestroyActor :!label _label))
    (:CastFailed
      (bind _asbp_base_enemy (Utilities|Casting|CastToBP_BaseEnemy OtherActor)
        (:then
          (Utilities|IsValid _asbp_base_enemy
            (:Is%20Valid
              (Game|Damage|ApplyDamage _asbp_base_enemy (Variables|Default|GetDamageAmount) 0 self "/Game/Characters/NPC/Turrets/Blueprints/BT_PlayerDamagaType.BT_PlayerDamagaType_C")
              (Variables|Default|SetDamageAmount (* (Variables|Default|GetDamageAmount) 0.5))
              (Class|FMODBlueprintStatics|PlayEvent2D "/Game/FMOD/Events/Gunshots/hitmarker.hitmarker"))))
        (:CastFailed
          (goto _label))))))

(event EventBeginPlay
  (|CallParentFunction) ; This node is disabled and will not be called.\nDrag off pins to build functionality.
)

(event EventTick
  (params (DeltaSeconds :type Float%20%28single-precision%29))
  (|CallParentFunction DeltaSeconds) ; This node is disabled and will not be called.\nDrag off pins to build functionality.
)

(fn ConstructionScript
  (|CallParentFunction))