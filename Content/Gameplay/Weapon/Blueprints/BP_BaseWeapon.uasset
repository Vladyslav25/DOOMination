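; Base weapon actor that fires damage-carrying projectiles for the player, with fire-rate timer, magazine and delayed reload.
; Tick traces from the player camera, ignoring tower points, to aim an Arrow component that sets projectile direction.
; Each shot adds spray, randomly offsets the next direction and plays a recoil timeline passed to the player.
; Timelines scaled by tunable durations gate firing and delay spray decay, which eases the Arrow back toward the target.
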(event Custom|Recoile
  (Variables|Members|SetTmpWeaponRotY (.pitch (Variables|/Script/Engine.SceneComponent|GetRelativeRotation (Variables|Components|GetRoot))))
  ;[1 1 1] The Delta Recoil Rotation. Set the Recoile Rotation. (Delta: Start with 0 and end with 0)
  (bind _recoilamount (Timeline|Recoil%20Rot PlayFromStart)
    (:Update
      (Variables|Members|SetRecoileRot (* _recoilamount (Variables|WeaponSettingsValues|GetRecoilMulti)))
      ;[1 1 1] When the timer finished the currSpray can decrese. After the Recoil the Timer start. And after finish its reset
      (Timeline|SprayDecrese PlayFromStart
        (:Finished
          (Variables|Members|SetCanSprayDecrease true)
          (Timeline|SprayDecrese SetNewTime))))))

(event Custom|Fire_Pressed
  (Variables|Members|SetIsFirering true)
  (Variables|Members|SetCanSprayDecrease false)
  (Variables|Members|SetIsPressed true)
  (if (Math|Boolean|ANDBoolean (Variables|Members|GetCanShot) (Variables|Members|GetIsPressed) (> (Variables|Members|GetInMagazin) 0))
    (CallFunction|Shoot)
    (Variables|Members|SetCanShot false)
    (Utilities|FlowControl|Sequence
      (:then_0
        ;[1 1 1] Whe the timer finish the "Can Shot" sets to true
        (Timeline|ShotTimer Play
          (:Finished
            (Utilities|FlowControl|Sequence
              (:then_0
                (Variables|Members|SetCanShot true))
              (:then_1
                (Timeline|ShotTimer SetNewTime))))))
      (:then_1
        ;[1 1 1] When the timer finished the currSpray can decrese. After the Recoil the Timer start. And after finish its reset
        (Timeline|SprayDecrese Stop
          (:Finished
            (Variables|Members|SetCanSprayDecrease true)
            (Timeline|SprayDecrese SetNewTime)))))))

(event Custom|Fire_Relesed
  (Variables|Members|SetIsFirering false)
  (Variables|Members|SetIsPressed false))

(event Custom|Relode
  (Variables|Members|SetCanShot false)
  (Development|PrintString "StartRelode")
  (Utilities|FlowControl|Delay (Variables|WeaponSettingsValues|GetRelodeTime))
  (Variables|Members|SetInMagazin (Variables|WeaponSettingsValues|GetMaxMagazin))
  (Variables|Members|SetCanShot true)
  (Development|PrintString "FinRelode"))

(event EventBeginPlay
  (Input|EnableInput (Game|GetPlayerController 0))
  ;[1 1 1] Set Playrates of the Timelines
  (Components|Timeline|SetPlayRate (Variables|Default|GetSprayDecrese) (/ 1.0 (Variables|WeaponSettingsValues|GetSprayResetTime)))
  (Components|Timeline|SetPlayRate (Variables|Default|GetRecoil%20Rot) (/ 1.0 (Variables|Members|GetRecoileRotSpeed)))
  (Components|Timeline|SetPlayRate (Variables|Default|GetShotTimer) (/ 1.0 (Variables|WeaponSettingsValues|GetMaxFireTimer)))
  (bind _asbp_bplayer (Utilities|Casting|CastToBP_BPlayer (Game|Player|GetPlayerPawn 0)))
  (Variables|Members|SetPlayerRef _asbp_bplayer)
  (Variables|Members|SetInMagazin (Variables|WeaponSettingsValues|GetMaxMagazin))
  (bind _outactors (Actor|GetAllActorsOfClass "/Game/Characters/NPC/Turrets/Blueprints/BlueprintTower/BP_TowerPoint.BP_TowerPoint_C"))
  (Variables|Members|SetAllTowerPoints _outactors))

(event EventTick
  (params (DeltaSeconds :type Float%20%28single-precision%29))
  (bind _arrow (Variables|Components|GetArrow))
  (if (== (Variables|/Game/Characters/PC/Blueprints/BP_BPlayer.BP_BPlayer_C|GetCurrendWeapon (Variables|Members|GetPlayerRef)) self)
    (Utilities|FlowControl|Sequence
      (:then_0
        (Default|SetVerticalWeaponRecoile (Variables|Members|GetPlayerRef) (Variables|Members|GetRecoileRot))
        (if (Variables|Members|GetCanSprayDecrease)
          (bind _output_get (Variables|Members|SetCurrSpray (Math|Float|Clamp(Float) (- (Variables|Members|GetCurrSpray) (* (Variables|WeaponSettingsValues|GetSprayDecreaseSpeed) DeltaSeconds)))))
          (Transformation|SetWorldRotation _arrow (Math|Rotator|Lerp(Rotator) (Math|Conversions|RotationFromXVector (Variables|Members|GetTargetDirection)) (Transformation|GetWorldRotation _arrow) _output_get true) false false)))
      (:then_1
        (if (Math|Boolean|ANDBoolean (Variables|Members|GetCanShot) (Variables|Members|GetIsPressed) (> (Variables|Members|GetInMagazin) 0))
          (CallFunction|Shoot)
          (Variables|Members|SetCanShot false)
          (Utilities|FlowControl|Sequence
            (:then_0
              ;[1 1 1] Whe the timer finish the "Can Shot" sets to true
              (Timeline|ShotTimer Play
                (:Finished
                  (Utilities|FlowControl|Sequence
                    (:then_0
                      (Variables|Members|SetCanShot true))
                    (:then_1
                      (Timeline|ShotTimer SetNewTime))))))
            (:then_1
              ;[1 1 1] When the timer finished the currSpray can decrese. After the Recoil the Timer start. And after finish its reset
              (Timeline|SprayDecrese Stop
                (:Finished
                  (Variables|Members|SetCanSprayDecrease true)
                  (Timeline|SprayDecrese SetNewTime)))))))
      (:then_2
        (CallFunction|SetTargetDirection)
        (if (== (Variables|Members|GetCurrSpray) 0.0)
          (Transformation|SetWorldRotation (Variables|Components|GetArrow) (Math|Conversions|RotationFromXVector (Variables|Members|GetTargetDirection)) false false))))))

(fn ConstructionScript)

(fn Shoot
  (bind _minspraystep (Variables|WeaponSettingsValues|GetMinSprayStep))
  (bind _maxspraystep (Variables|WeaponSettingsValues|GetMaxSprayStep))
  (bind _returnvalue (Game|SpawnActorfromClass "/Game/Gameplay/Weapon/Blueprints/BP_BaseWeaponProjectile.BP_BaseWeaponProjectile_C" (Math|Transform|MakeTransform (Transformation|GetWorldLocation (Variables|Components|GetHole)) (Math|Rotator|MakeRotfromX (Math|Vector|GetForwardVector (Variables|Components|GetArrow))) "1,1,1") "AdjustIfPossibleButAlwaysSpawn" 0 0))
  (Utilities|IsValid _returnvalue
    (:Is%20Valid
      (Variables|/Game/Gameplay/Weapon/Blueprints/BP_BaseWeaponProjectile.BP_BaseWeaponProjectile_C|SetDamageAmount _returnvalue (Variables|WeaponSettingsValues|GetDamage))
      (bind _newdirection (CallFunction|GetRandomDirection _minspraystep (Math|Float|Clamp(Float) (* _maxspraystep (Variables|Members|GetCurrSpray)) _minspraystep _maxspraystep)))
      (Variables|Members|SetCurrSpray (Math|Float|Clamp(Float) (+ (Variables|Members|GetCurrSpray) (Variables|WeaponSettingsValues|GetAddCurrSpray))))
      (Transformation|SetWorldRotation (Variables|Components|GetArrow) (Math|Conversions|RotationFromXVector _newdirection) false false)
      (CallFunction|Recoile)
      (Math|Integer|DecrementInt (Variables|Members|GetInMagazin)))))

(fn GetRandomDirection
  (params (Min :type Float%20%28single-precision%29) (Max :type Float%20%28single-precision%29))
  (bind _returnvalue (Math|Random|RandomFloatinRange Min Max))
  (LocalVariables|SetRotZ _returnvalue)
  (LocalVariables|SetRotY _returnvalue)
  (if (Math|Random|RandomBool)
    (bind _output_get (LocalVariables|SetRotZ (* (LocalVariables|GetRotZ) -1.0))))
  (if (Math|Random|RandomBool)
    (bind _output_get_2 (LocalVariables|SetRotY (* (LocalVariables|GetRotY) -1.0))))
  (return (Math|Vector|RotateVector (Variables|Members|GetTargetDirection) (Math|Rotator|MakeRotator 0.0 _output_get_2 _output_get))))

(fn SetTargetDirection
  (bind _returnvalue (Transformation|GetActorLocation))
  (bind _playerref (Variables|Members|GetPlayerRef))
  (bind _camera (Variables|/Script/DOOMination.BPlayer|GetCamera _playerref))
  (bind _returnvalue_2 (Transformation|GetWorldLocation _camera))
  (bind (_outhit _returnvalue_3) (Collision|LineTraceByChannel _returnvalue_2 (+ _returnvalue_2 (* (Math|Vector|GetForwardVector _camera) 1e+09)) "TraceTypeQuery1" false (Variables|Members|GetAllTowerPoints) "None"))
  (if _returnvalue_3
    (Variables|Members|SetTargetDirection (Math|Vector|GetForwardVector (Math|Rotator|FindLookatRotation _returnvalue (.ImpactPoint (Collision|BreakHitResult _outhit)))))
    (else
      (Variables|Members|SetTargetDirection (Math|Vector|GetForwardVector (Math|Rotator|FindLookatRotation _returnvalue (+ (* (Math|Vector|GetForwardVector (Variables|/Script/DOOMination.BPlayer|GetCamera (Variables|Members|GetPlayerRef))) 99.0) _returnvalue)))))))