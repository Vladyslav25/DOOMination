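; BP_Sniper is a sniper weapon Blueprint with a live picture-in-picture scope.
; When no render target is set, its construction script creates one for the scene capture, applies the scope FOV and hides the weapon from the capture.
; A dynamic M_Scope material on the mesh displays that texture with adjustable brightness.
; BeginPlay and Tick only call the parent class.
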(event EventBeginPlay
  (|CallParentFunction))

(event EventTick
  (params (DeltaSeconds :type Float%20%28single-precision%29))
  (|CallParentFunction DeltaSeconds))

(fn ConstructionScript
  (bind _scenecapturecomponent2d (Variables|Default|GetSceneCaptureComponent2D))
  (|CallParentFunction)
  (Utilities|IsValid (Variables|/Script/Engine.SceneCaptureComponent2D|GetTextureTarget (Variables|Default|GetSceneCaptureComponent2D))
    (:Is%20Not%20Valid
      (Class|SceneCaptureComponent|HideActorComponents _scenecapturecomponent2d self false)
      (Variables|/Script/Engine.SceneCaptureComponent2D|SetFOVAngle _scenecapturecomponent2d (Variables|Default|GetFOV))
      (bind _returnvalue (Rendering|CreateRenderTarget2D 512 512 "RTF_RGBA16f"))
      (bind _output_get (Variables|/Script/Engine.SceneCaptureComponent2D|SetTextureTarget _scenecapturecomponent2d _returnvalue))
      (bind _returnvalue_2 (Rendering|Material|CreateDynamicMaterialInstance (Variables|Default|GetStaticMesh) 2 "/Game/Gameplay/Weapon/Material/Sniper/M_Scope.M_Scope" "None" :!class /Script/Engine.PrimitiveComponent))
      (Rendering|Material|SetTextureParameterValue _returnvalue_2 "Render" _output_get)
      (Rendering|Material|SetScalarParameterValue _returnvalue_2 "Brightness" (Variables|Default|GetBrightness) :!class /Script/Engine.MaterialInstanceDynamic))))