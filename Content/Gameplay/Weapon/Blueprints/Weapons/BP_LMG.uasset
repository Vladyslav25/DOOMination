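; Placeable, mountable LMG weapon that the player possesses to aim, fire and reload.
; It starts as a wireframe preview, tinted green or red by a box-trace placement check, and gets its real materials when placed.
; An overlap box flags the player in range; interacting hides and attaches the player and transfers controller possession, or reverses it.
; Aim input is angle-clamped, Tick adds recoil to pitch, and a muzzle line trace sets target direction.
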(event OnComponentBeginOverlap(Box)
  (params (OverlappedComponent :type Primitive%20Component%20Object%20Reference) (OtherActor :type Actor%20Object%20Reference) (OtherComp :type Primitive%20Component%20Object%20Reference) (OtherBodyIndex :type Integer) (bFromSweep :type Boolean) (SweepResult :type Hit%20Result%20Structure%20%28by%20ref%29))
  (bind _asbp_player (Utilities|Casting|CastToBP_Player OtherActor))
  (Variables|/Game/Characters/PC/Blueprints/BP_Player.BP_Player_C|SetLMGInRange _asbp_player true))

(event OnComponentEndOverlap(Box)
  (params (OverlappedComponent :type Primitive%20Component%20Object%20Reference) (OtherActor :type Actor%20Object%20Reference) (OtherComp :type Primitive%20Component%20Object%20Reference) (OtherBodyIndex :type Integer))
  (bind _asbp_player (Utilities|Casting|CastToBP_Player OtherActor))
  (Variables|/Game/Characters/PC/Blueprints/BP_Player.BP_Player_C|SetLMGInRange _asbp_player false))

(event EventBeginPlay
  (|CallParentFunction)
  (CallFunction|CreateMaterials)
  (CallFunction|SetColor "(R=0.000000,G=1.000000,B=0.000000,A=1.000000)"))

(event EventTick
  (params (DeltaSeconds :type Float%20%28single-precision%29))
  (|CallParentFunction DeltaSeconds)
  (Transformation|AddLocalRotation (Variables|Default|GetStaticMesh) (Math|Rotator|MakeRotator 0.0 (* 1 (+ (Variables|Default|GetRecoileRot) (Variables|Memeber|Private|GetCurrVerticalRot))) 0.0) false false))

(event Input|ActionEvents|InputActionFire_Weapon
  (params (Key :type Key%20Structure))
  (bind _ispossesed (Variables|Memeber|Private|GetIsPossesed))
  (:Pressed
    (if _ispossesed
      (CallFunction|FirePressed)))
  (:Released
    (if _ispossesed
      (CallFunction|FireRelesed))))

(event Input|ActionEvents|InputActionRelode
  (params (Key :type Key%20Structure))
  (:Pressed
    (if (Variables|Memeber|Private|GetIsPossesed)
      (CallFunction|Relode))))

(event Input|ActionEvents|InputActionInteract
  (params (Key :type Key%20Structure))
  (:Pressed
    (if (Variables|Memeber|Private|GetIsPossesed)
      (CallFunction|LeavePossesion)
      (else
        (CallFunction|TakePossesion)))))

(event Input|AxisEvents|InputAxisVerticalRotation
  (params (AxisValue :type Float%20%28single-precision%29))
  (bind _staticmesh (Variables|Default|GetStaticMesh))
  (bind _relativerotation (Variables|/Script/Engine.SceneComponent|GetRelativeRotation _staticmesh))
  (bind _returnvalue (+ AxisValue (.pitch _relativerotation)))
  (if (and (< _returnvalue 2e+01) (>= _returnvalue -2e+01))
    (Variables|Memeber|Private|SetCurrVerticalRot AxisValue)
    (else
      (Variables|Memeber|Private|SetCurrVerticalRot 0.0))))

(event Input|AxisEvents|InputAxisHorizontalRotation
  (params (AxisValue :type Float%20%28single-precision%29))
  (bind _staticmesh (Variables|Default|GetStaticMesh))
  (bind _relativerotation (Variables|/Script/Engine.SceneComponent|GetRelativeRotation _staticmesh))
  (bind _returnvalue (+ AxisValue (.yaw _relativerotation)))
  (if (and (< _returnvalue 45.0) (>= _returnvalue -45.0))
    (Transformation|AddRelativeRotation _staticmesh (Math|Rotator|MakeRotator 0.0 0.0 AxisValue) false false)))

(fn ConstructionScript
  (|CallParentFunction))

(fn TakePossesion
  (bind _self self)
  (bind _playerref (Variables|Default|GetPlayerRef))
  (Variables|Memeber|Private|SetIsPossesed true)
  (Rendering|SetVisibility (Variables|/Script/Engine.Character|GetMesh _playerref) false true)
  (Collision|SetCollisionEnabled (Variables|/Script/Engine.Character|GetCapsuleComponent _playerref) "NoCollision")
  (Transformation|AttachActorToActor _playerref _self "None" "KeepRelative" "KeepRelative" "KeepRelative" true)
  (Rendering|SetCastShadow (Variables|/Script/Engine.Character|GetMesh _playerref) false)
  (Variables|/Game/Characters/PC/Blueprints/BP_Player.BP_Player_C|SetCurrendWeapon _playerref _self)
  (Pawn|Possess (Pawn|GetController _playerref) _self))

(fn LeavePossesion
  (bind _playerref (Variables|Default|GetPlayerRef))
  (Variables|Memeber|Private|SetIsPossesed false)
  (Rendering|SetVisibility (Variables|/Script/Engine.Character|GetMesh _playerref) true true)
  (Collision|SetCollisionEnabled (Variables|/Script/Engine.Character|GetCapsuleComponent _playerref) "QueryAndPhysics")
  (Transformation|DetachFromActor _playerref "KeepRelative" "KeepRelative" "KeepRelative")
  (Rendering|SetCastShadow (Variables|/Script/Engine.Character|GetMesh _playerref) true)
  (Pawn|Possess (Pawn|GetController) _playerref)
  (Default|SwitchWeaponto _playerref))

(fn SetTargetDirection
  (bind _hole (Variables|Default|GetHole))
  (bind _returnvalue (Transformation|GetWorldLocation _hole))
  (bind _returnvalue_2 (Transformation|GetWorldLocation _hole))
  (bind (_outhit _returnvalue_3) (Collision|LineTraceByChannel _returnvalue (+ _returnvalue (* (Math|Vector|GetForwardVector _hole) 1e+09)) "TraceTypeQuery1" false 0 "None"))
  (if _returnvalue_3
    (Variables|Default|SetTargetDirection (Math|Vector|GetForwardVector (Math|Rotator|FindLookatRotation _returnvalue_2 (.ImpactPoint (Collision|BreakHitResult _outhit)))))
    (else
      (Variables|Default|SetTargetDirection (Math|Vector|GetForwardVector (Math|Rotator|FindLookatRotation _returnvalue_2 (+ (* (Math|Vector|GetForwardVector _hole) 99) _returnvalue_2)))))))

(fn CreateMaterials
  (bind _returnvalue (Rendering|Material|CreateDynamicMaterialInstance "/Game/Effects/Mastermatrial/M_Wireframe.M_Wireframe" "None" :!class /Script/Engine.KismetMaterialLibrary))
  (CallFunction|SetMaterials _returnvalue _returnvalue _returnvalue))

(fn PlaceatCurrendLocation
  (if (Variables|Memeber|Public|GetValidPos)
    (CallFunction|SetMaterials "/Game/Gameplay/Weapon/Material/LMG/MI_LMG_Ammopack.MI_LMG_Ammopack" "/Game/Gameplay/Weapon/Material/LMG/MI_LMG02.MI_LMG02" "/Game/Gameplay/Weapon/Material/LMG/MI_LMG01.MI_LMG01")
    (Variables|/Game/Characters/PC/Blueprints/BP_Player.BP_Player_C|SetLMGPlaced (Variables|Default|GetPlayerRef) true)))

(fn SetColor
  (params (Color :type Linear%20Color%20Structure))
  (for _array_element (Variables|Memeber|Private|GetMaterialLMG)
    (Rendering|Material|SetVectorParameterValue _array_element "Color" Color :!class /Script/Engine.MaterialInstanceDynamic))
  (for _array_element_2 (Variables|Memeber|Private|GetMaterialFuss)
    (Rendering|Material|SetVectorParameterValue _array_element_2 "Color" Color :!class /Script/Engine.MaterialInstanceDynamic)))

(fn SetMaterials
  (params (Mat01 :type Material%20Instance%20Object%20Reference) (Mat02 :type Material%20Instance%20Object%20Reference) (Mat03 :type Material%20Instance%20Object%20Reference))
  (bind _materiallmg (Variables|Memeber|Private|GetMaterialLMG))
  (bind _materialfuss (Variables|Memeber|Private|GetMaterialFuss))
  (bind _staticmesh (Variables|Default|GetStaticMesh))
  (bind _fuss (Variables|Default|GetFuss))
  (Utilities|FlowControl|Sequence
    (:then_0
      (bind _returnvalue (Rendering|Material|CreateDynamicMaterialInstance _staticmesh 0 Mat01 "None" :!class /Script/Engine.PrimitiveComponent))
      (Utilities|Array|SetArrayElem _materiallmg 0 _returnvalue))
    (:then_1
      (bind _returnvalue_2 (Rendering|Material|CreateDynamicMaterialInstance _staticmesh 1 Mat02 "None" :!class /Script/Engine.PrimitiveComponent))
      (Utilities|Array|SetArrayElem _materiallmg 1 _returnvalue_2))
    (:then_2
      (bind _returnvalue_3 (Rendering|Material|CreateDynamicMaterialInstance _staticmesh 2 Mat03 "None" :!class /Script/Engine.PrimitiveComponent))
      (Utilities|Array|SetArrayElem _materiallmg 2 _returnvalue_3))
    (:then_3
      (bind _returnvalue_4 (Rendering|Material|CreateDynamicMaterialInstance _fuss 0 Mat01 "None" :!class /Script/Engine.PrimitiveComponent))
      (Utilities|Array|SetArrayElem _materialfuss 0 _returnvalue_4))
    (:then_4
      (bind _returnvalue_5 (Rendering|Material|CreateDynamicMaterialInstance _fuss 1 Mat02 "None" :!class /Script/Engine.PrimitiveComponent))
      (Utilities|Array|SetArrayElem _materialfuss 1 _returnvalue_5))))

(fn CheckforPosition
  (params (NewTransform :type Transform))
  (bind _returnvalue (+ (.location NewTransform) "0, 0,128.000000"))
  (bind _returnvalue_2 (Class|KismetSystemLibrary|BoxTraceSingleforObjects _returnvalue _returnvalue "180.000000,180.000000,32.000000" (.rotation NewTransform) (Variables|Setting|GetCollEnum) false 0 "None" true))
  (if _returnvalue_2
    (CallFunction|SetColor "(R=1.000000,G=0.000000,B=0.000000,A=1.000000)")
    (else
      (CallFunction|SetColor "(R=0.000000,G=1.000000,B=0.000000,A=1.000000)")))
  (bind _output_get (Variables|Memeber|Public|SetValidPos (not _returnvalue_2)))
  (return _output_get))