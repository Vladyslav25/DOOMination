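; BP_Harpune is a harpoon weapon that keeps a loaded BP_HarpuneProjectile actor attached to its mesh socket.
; On BeginPlay it spawns the first spear, and Shoot plays a sound, detaches the spear, fires it using Arrow and clears the reference.
; With no spear loaded, Relode spawns one in the player's left hand, waits RelodeTime, then attaches it to the weapon, refills the magazine and re-enables shooting.
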(event EventBeginPlay
  (|CallParentFunction)
  (bind _returnvalue (Game|SpawnActorfromClass "/Game/Gameplay/Weapon/Blueprints/Projectiles/BP_HarpuneProjectile.BP_HarpuneProjectile_C" (Transformation|GetActorTransform (Game|Player|GetPlayerPawn 0)) "Undefined" 0 0))
  (Transformation|AttachComponentToComponent _returnvalue (Variables|Default|GetStaticMesh) "WurfspeerSocket" "SnapToTarget" "SnapToTarget" "SnapToTarget" true)
  (Variables|Default|SetWurfspeer _returnvalue))

(event Collision|EventActorBeginOverlap
  (params (OtherActor :type Actor%20Object%20Reference)))

(event EventTick
  (params (DeltaSeconds :type Float%20%28single-precision%29))
  (|CallParentFunction DeltaSeconds) ; This node is disabled and will not be called.\nDrag off pins to build functionality.
)

(event EventRelode
  (bind _returnvalue (Game|Player|GetPlayerPawn 0))
  (Utilities|IsValid (Variables|Default|GetWurfspeer)
    (:Is%20Not%20Valid
      (Variables|Default|SetCanShot false)
      (Development|PrintString "StartRelode")
      (bind _returnvalue_2 (Game|SpawnActorfromClass "/Game/Gameplay/Weapon/Blueprints/Projectiles/BP_HarpuneProjectile.BP_HarpuneProjectile_C" (Transformation|GetActorTransform _returnvalue) "AlwaysSpawn" 0 0))
      (bind _asbp_player (Utilities|Casting|CastToBP_Player _returnvalue))
      (Transformation|AttachComponentToComponent _returnvalue_2 (Variables|/Script/Engine.Character|GetMesh _asbp_player) "LeftHandSocket" "SnapToTarget" "SnapToTarget" "KeepWorld" true)
      ;[1 1 1] animation
      (Utilities|FlowControl|Delay (Variables|Default|GetRelodeTime))
      (Transformation|AttachComponentToComponent _returnvalue_2 (Variables|Default|GetStaticMesh) "WurfspeerSocket" "SnapToTarget" "SnapToTarget" "KeepWorld" true)
      (Variables|Default|SetWurfspeer _returnvalue_2)
      (Variables|Default|SetInMagazin (Variables|Default|GetMaxMagazin))
      (Variables|Default|SetCanShot true)
      (Development|PrintString "FinRelode"))))

(fn ConstructionScript
  (|CallParentFunction))

(fn Shoot
  (Class|FMODBlueprintStatics|PlayEventatLocation (Variables|Default|GetShootSound) (Transformation|GetActorTransform))
  (Utilities|IsValid (Variables|Default|GetWurfspeer)
    (:Is%20Valid
      (Transformation|DetachFromActor (Variables|Default|GetWurfspeer) "KeepWorld" "KeepWorld" "KeepWorld")
      (Default|Fire (Variables|Default|GetWurfspeer) (Variables|Default|GetArrow))
      (Variables|Default|SetWurfspeer 0))
    (:Is%20Not%20Valid
      (Development|PrintString "Wurfspeer is NULL" true false "(R=1.000000,G=0.000000,B=0.000000,A=1.000000)"))))