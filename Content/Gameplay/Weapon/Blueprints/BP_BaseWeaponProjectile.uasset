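; Base weapon projectile actor that deals player damage to enemies it touches.
; The construction script sets the projectile movement component's initial and max speed to the same fixed value.
; On sphere overlap, a valid BP_BaseEnemy receives DamageAmount with the player damage type, then the projectile destroys itself.
; Other overlaps also destroy it, except BP_ProjectileDespawner, which this blueprint ignores.
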(event OnComponentBeginOverlap(Sphere)
  (params (OverlappedComponent :type Primitive%20Component%20Object%20Reference) (OtherActor :type Actor%20Object%20Reference) (OtherComp :type Primitive%20Component%20Object%20Reference) (OtherBodyIndex :type Integer) (bFromSweep :type Boolean) (SweepResult :type Hit%20Result%20Structure%20%28by%20ref%29))
  (bind _asbp_base_enemy (Utilities|Casting|CastToBP_BaseEnemy OtherActor)
    (:then
      (Utilities|IsValid _asbp_base_enemy
        (:Is%20Valid
          (Game|Damage|ApplyDamage _asbp_base_enemy (Variables|Default|GetDamageAmount) 0 self "/Game/Characters/NPC/Turrets/Blueprints/BT_PlayerDamagaType.BT_PlayerDamagaType_C"))))
    (:CastFailed
      (Utilities|Casting|CastToBP_ProjectileDespawner OtherActor
        (:CastFailed
          _))))
  (Actor|DestroyActor))

(event EventBeginPlay)

(event Collision|EventActorBeginOverlap
  (params (OtherActor :type Actor%20Object%20Reference)))

(event EventTick
  (params (DeltaSeconds :type Float%20%28single-precision%29)))

(fn ConstructionScript
  (bind _projectilemovement (Variables|Default|GetProjectileMovement))
  (bind _output_get (Variables|/Script/Engine.ProjectileMovementComponent|SetInitialSpeed _projectilemovement 2e+03))
  (Variables|/Script/Engine.ProjectileMovementComponent|SetMaxSpeed _projectilemovement _output_get))