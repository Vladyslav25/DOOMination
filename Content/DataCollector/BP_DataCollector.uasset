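; BP_DataCollector is a statistics actor that tallies tower performance and Argent spending for Cannon, Laser, Rifle and Rocket Launcher towers.
; Functions called from outside increment per-type counters for builds, destructions, kills, damage, shots and upgrades, with build costs hard-coded.
; The Switch On BaseTower macro routes many calls by casting a tower reference, falling back to its class.
; Total functions sum the per-type values.
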(event EventBeginPlay)

(event Collision|EventActorBeginOverlap
  (params (OtherActor :type Actor%20Object%20Reference)))

(event EventTick
  (params (DeltaSeconds :type Float%20%28single-precision%29)))

(fn ConstructionScript)

(fn TowerSpawned
  (params (TowerReference :type BP%20Base%20Tower%20Object%20Reference) (Tower :type BP%20Base%20Tower%20Class%20Reference))
  (Utilities|SwitchonBaseTower TowerReference Tower
    (:Cannon
      (Math|Integer|IncrementInt (Variables|Tower|TurretsBuild|GetCannonsBuild)
        (:%20%20
          (Variables|Tower|SpendedAmountOfArgentForTurretBuilded|SetSpendedAmountOfArgentForCannonBuilded (+ 100 (Variables|Tower|SpendedAmountOfArgentForTurretBuilded|GetSpendedAmountOfArgentForCannonBuilded))))))
    (:Laser
      (Math|Integer|IncrementInt (Variables|Tower|TurretsBuild|GetLasersBuild)
        (:%20%20
          (Variables|Tower|SpendedAmountOfArgentForTurretBuilded|SetSpendedAmountOfArgentForLaserBuilded (+ 140 (Variables|Tower|SpendedAmountOfArgentForTurretBuilded|GetSpendedAmountOfArgentForLaserBuilded))))))
    (:Rifle
      (Math|Integer|IncrementInt (Variables|Tower|TurretsBuild|GetRiflesBuild)
        (:%20%20
          (Variables|Tower|SpendedAmountOfArgentForTurretBuilded|SetSpendedAmountOfArgentForRifleBuilded (+ 114 (Variables|Tower|SpendedAmountOfArgentForTurretBuilded|GetSpendedAmountOfArgentForRifleBuilded))))))
    (:RocketLauncher
      (Math|Integer|IncrementInt (Variables|Tower|TurretsBuild|GetRocketLaunchersBuild)
        (:%20%20
          (Variables|Tower|SpendedAmountOfArgentForTurretBuilded|SetSpendedAmountOfArgentForRocketLauncherBuilded (+ 124 (Variables|Tower|SpendedAmountOfArgentForTurretBuilded|GetSpendedAmountOfArgentForRocketLauncherBuilded))))))))

(fn TowerDestroyed
  (params (TowerRef :type BP%20Base%20Tower%20Object%20Reference) (TowerClass :type BP%20Base%20Tower%20Class%20Reference))
  (Utilities|SwitchonBaseTower TowerRef TowerClass
    (:Cannon
      (Math|Integer|IncrementInt (Variables|Tower|TurretsDestroyed|GetCannonsDestroyed)))
    (:Laser
      (Math|Integer|IncrementInt (Variables|Tower|TurretsDestroyed|GetLasersDestroyed)))
    (:Rifle
      (Math|Integer|IncrementInt (Variables|Tower|TurretsDestroyed|GetRiflesDestroyed)))
    (:RocketLauncher
      (Math|Integer|IncrementInt (Variables|Tower|TurretsDestroyed|GetRocketLaunchersDestroyed)))))

(fn AddSpendedAmountOfArgentforTurretUpgrades
  (params (TowerRef :type BP%20Base%20Tower%20Object%20Reference) (TowerClass :type BP%20Base%20Tower%20Class%20Reference) (ArgentSpended :type Integer))
  (Utilities|SwitchonBaseTower TowerRef TowerClass
    (:Cannon
      (Variables|Tower|SpendedAmountOfArgentForTurretUpgrades|SetSpendedAmountOfArgentForCannonUpgrades (+ (Variables|Tower|SpendedAmountOfArgentForTurretUpgrades|GetSpendedAmountOfArgentForCannonUpgrades) ArgentSpended)))
    (:Laser
      (Variables|Tower|SpendedAmountOfArgentForTurretUpgrades|SetSpendedAmountOfArgentForLaserUpgrades (+ ArgentSpended (Variables|Tower|SpendedAmountOfArgentForTurretUpgrades|GetSpendedAmountOfArgentForLaserUpgrades))))
    (:Rifle
      (Variables|Tower|SpendedAmountOfArgentForTurretUpgrades|SetSpendedAmountOfArgentForRifleUpgrades (+ ArgentSpended (Variables|Tower|SpendedAmountOfArgentForTurretUpgrades|GetSpendedAmountOfArgentForRifleUpgrades))))
    (:RocketLauncher
      (Variables|Tower|SpendedAmountOfArgentForTurretUpgrades|SetSpendedAmountOfArgentForRocketLauncherUpgrades (+ ArgentSpended (Variables|Tower|SpendedAmountOfArgentForTurretUpgrades|GetSpendedAmountOfArgentForRocketLauncherUpgrades))))))

(fn AddTowerDamage
  (params (NewParam :type BP%20Base%20Tower%20Class%20Reference) (Damage :type Float%20%28single-precision%29))
  (Utilities|SwitchonBaseTower 0 NewParam
    (:Cannon
      (bind _totaldamage (AddAmountOfDamageByTurret|AddCannonDamage Damage))
      (return _totaldamage))
    (:Laser
      (bind _totaldamage_2 (AddAmountOfDamageByTurret|AddLaserDamage Damage))
      (return _totaldamage_2))
    (:Rifle
      (bind _totaldamage_3 (AddAmountOfDamageByTurret|AddRifleDamage Damage))
      (return _totaldamage_3))
    (:RocketLauncher
      (bind _totaldamage_4 (AddAmountOfDamageByTurret|AddRocketLauncherDamage Damage))
      (return _totaldamage_4))
    (:Default
      (Development|PrintString "Wrong Tower given in BP_DataCollector.AddTowerDamage" true true "(R=1.000000,G=0.000000,B=0.014919,A=1.000000)" 3.0)
      (return -1.0))))

(fn AddCannonDamage
  (params (Damage :type Float%20%28single-precision%29))
  (bind _output_get (Variables|Tower|AmountOfDamageByTurret|SetAmountOfDamageByCannon (+ Damage (Variables|Tower|AmountOfDamageByTurret|GetAmountOfDamageByCannon))))
  (return _output_get))

(fn AddLaserDamage
  (params (Damage :type Float%20%28single-precision%29))
  (bind _output_get (Variables|Tower|AmountOfDamageByTurret|SetAmountOfDamageByLaser (+ Damage (Variables|Tower|AmountOfDamageByTurret|GetAmountOfDamageByLaser))))
  (return _output_get))

(fn AddRifleDamage
  (params (Damage :type Float%20%28single-precision%29))
  (bind _output_get (Variables|Tower|AmountOfDamageByTurret|SetAmountOfDamageByRifle (+ Damage (Variables|Tower|AmountOfDamageByTurret|GetAmountOfDamageByRifle))))
  (return _output_get))

(fn AddRocketLauncherDamage
  (params (Damage :type Float%20%28single-precision%29))
  (bind _output_get (Variables|Tower|AmountOfDamageByTurret|SetAmountOfDamageByRocketLauncher (+ Damage (Variables|Tower|AmountOfDamageByTurret|GetAmountOfDamageByRocketLauncher))))
  (return _output_get))

(fn TotalSpendedAmountOfArgentforTowerBuilded
  (return (+ (Variables|Tower|SpendedAmountOfArgentForTurretBuilded|GetSpendedAmountOfArgentForCannonBuilded) (Variables|Tower|SpendedAmountOfArgentForTurretBuilded|GetSpendedAmountOfArgentForLaserBuilded) (Variables|Tower|SpendedAmountOfArgentForTurretBuilded|GetSpendedAmountOfArgentForRifleBuilded) (Variables|Tower|SpendedAmountOfArgentForTurretBuilded|GetSpendedAmountOfArgentForRocketLauncherBuilded))))

(fn TotalSpendedAmountOfArgentforTowerUpgrades
  (return (+ (Variables|Tower|SpendedAmountOfArgentForTurretUpgrades|GetSpendedAmountOfArgentForCannonUpgrades) (Variables|Tower|SpendedAmountOfArgentForTurretUpgrades|GetSpendedAmountOfArgentForLaserUpgrades) (Variables|Tower|SpendedAmountOfArgentForTurretUpgrades|GetSpendedAmountOfArgentForRifleUpgrades) (Variables|Tower|SpendedAmountOfArgentForTurretUpgrades|GetSpendedAmountOfArgentForRocketLauncherUpgrades))))

(fn TotalAmountOfDamagebyTurret
  (return (+ (Variables|Tower|AmountOfDamageByTurret|GetAmountOfDamageByCannon) (Variables|Tower|AmountOfDamageByTurret|GetAmountOfDamageByLaser) (Variables|Tower|AmountOfDamageByTurret|GetAmountOfDamageByRifle) (Variables|Tower|AmountOfDamageByTurret|GetAmountOfDamageByRocketLauncher))))

(fn DeathbyTower
  (params (TowerRef :type BP%20Base%20Tower%20Object%20Reference) (TowerClass :type BP%20Base%20Tower%20Class%20Reference))
  (Utilities|SwitchonBaseTower TowerRef TowerClass
    (:Cannon
      (Math|Integer|IncrementInt (Variables|Tower|EnemiesKilledByTower|GetEnemiesKilledByCannon)))
    (:Laser
      (Math|Integer|IncrementInt (Variables|Tower|EnemiesKilledByTower|GetEnemiesKilledByLaser)))
    (:Rifle
      (Math|Integer|IncrementInt (Variables|Tower|EnemiesKilledByTower|GetEnemiesKilledByRifle)))
    (:RocketLauncher
      (Math|Integer|IncrementInt (Variables|Tower|EnemiesKilledByTower|GetEnemiesKilledByRocketLauncher)))
    (:Default
      (Development|PrintString "No Tower given!" true false "(R=1.000000,G=0.132595,B=0.092793,A=1.000000)"))))

(fn TotalShotTowerShots
  (return (+ (Variables|Tower|ShotTowerShots|GetShotCannonShots) (Variables|Tower|ShotTowerShots|GetShotLaserShots) (Variables|Tower|ShotTowerShots|GetShotRifleShots) (Variables|Tower|ShotTowerShots|GetShotRocketLauncherShots))))

(fn TotalTowerBuilds
  (return (+ (Variables|Tower|TurretsBuild|GetCannonsBuild) (Variables|Tower|TurretsBuild|GetLasersBuild) (Variables|Tower|TurretsBuild|GetRiflesBuild) (Variables|Tower|TurretsBuild|GetRocketLaunchersBuild))))

(fn TotalTowerDestroyed
  (return (+ (Variables|Tower|TurretsDestroyed|GetCannonsDestroyed) (Variables|Tower|TurretsDestroyed|GetLasersDestroyed) (Variables|Tower|TurretsDestroyed|GetRiflesDestroyed) (Variables|Tower|TurretsDestroyed|GetRocketLaunchersDestroyed))))

(fn TotalEnemieKilledbyTower
  (return (+ (Variables|Tower|EnemiesKilledByTower|GetEnemiesKilledByCannon) (Variables|Tower|EnemiesKilledByTower|GetEnemiesKilledByLaser) (Variables|Tower|EnemiesKilledByTower|GetEnemiesKilledByRifle) (Variables|Tower|EnemiesKilledByTower|GetEnemiesKilledByRocketLauncher))))

(fn AddCannonShots
  (params (CannonShots :type Integer))
  (bind _output_get (Variables|Tower|ShotTowerShots|SetShotCannonShots (+ CannonShots (Variables|Tower|ShotTowerShots|GetShotCannonShots))))
  (return _output_get))

(fn AddLaserShots
  (params (LaserShots :type Integer))
  (bind _output_get (Variables|Tower|ShotTowerShots|SetShotLaserShots (+ LaserShots (Variables|Tower|ShotTowerShots|GetShotLaserShots))))
  (return _output_get))

(fn AddRifleShots
  (params (RifleShots :type Integer))
  (bind _output_get (Variables|Tower|ShotTowerShots|SetShotRifleShots (+ RifleShots (Variables|Tower|ShotTowerShots|GetShotRifleShots))))
  (return _output_get))

(fn AddRocketLauncherShots
  (params (RocketLauncherShots :type Integer))
  (bind _output_get (Variables|Tower|ShotTowerShots|SetShotRocketLauncherShots (+ RocketLauncherShots (Variables|Tower|ShotTowerShots|GetShotRocketLauncherShots))))
  (return _output_get))

(fn AddCannonUpgrade
  (params (CannonUpgrades :type Integer))
  (bind _output_get (Variables|Tower|AmountTurretUpgraded|SetAmountCannonUpgraded (+ CannonUpgrades (Variables|Tower|AmountTurretUpgraded|GetAmountCannonUpgraded))))
  (return _output_get))

(fn AddLaserUpgrade
  (params (LaserUpgrades :type Integer))
  (bind _output_get (Variables|Tower|AmountTurretUpgraded|SetAmountLaserUpgraded (+ LaserUpgrades (Variables|Tower|AmountTurretUpgraded|GetAmountLaserUpgraded))))
  (return _output_get))

(fn AddRifleUpgrade
  (params (RifleUpgrades :type Integer))
  (bind _output_get (Variables|Tower|AmountTurretUpgraded|SetAmountRifleUpgraded (+ RifleUpgrades (Variables|Tower|AmountTurretUpgraded|GetAmountRifleUpgraded))))
  (return _output_get))

(fn AddRocketLauncherUpgrade
  (params (RocketLauncherUpgrades :type Integer))
  (bind _output_get (Variables|Tower|AmountTurretUpgraded|SetAmountRocketLauncherUpgraded (+ RocketLauncherUpgrades (Variables|Tower|AmountTurretUpgraded|GetAmountRocketLauncherUpgraded))))
  (return _output_get))

(fn TotalAmountOfUpgrades
  (return (+ (Variables|Tower|AmountTurretUpgraded|GetAmountCannonUpgraded) (Variables|Tower|AmountTurretUpgraded|GetAmountLaserUpgraded) (Variables|Tower|AmountTurretUpgraded|GetAmountRifleUpgraded) (Variables|Tower|AmountTurretUpgraded|GetAmountRocketLauncherUpgraded))))