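; BP_BPlayerClassic is a player character with a weapon, handling movement, camera rotation, jumping, zoom and firing.
; BeginPlay spawns a BP_BaseWeapon on the mesh's WeaponSocket, and fire input forwards to it.
; Input events call movement and zoom helpers or store state, while Tick polls jump, lerps camera arm length for aim zoom and rotates to camera forward.
; Weapon recoil is added to vertical look input every frame.
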(event EventBeginPlay
  (bind _mesh (Variables|Character|GetMesh))
  (bind _returnvalue (Game|SpawnActorfromClass "/Game/Gameplay/Weapon/BP_BaseWeapon.BP_BaseWeapon_C" (Transformation|GetSocketTransform _mesh "WeaponSocket" "RTS_Actor") "AlwaysSpawn" 0 0))
  (bind _output_get (Variables|Default|SetCurrendWeapon _returnvalue))
  (Transformation|AttachComponentToComponent _output_get _mesh "WeaponSocket" "KeepRelative" "KeepRelative" "KeepRelative" true)
  (Development|PrintString (Utilities|String|ToString(Vector) (Transformation|GetActorLocation _output_get))))

(event EventTick
  (params (DeltaSeconds :type Float%20%28single-precision%29))
  (Utilities|FlowControl|Sequence
    (:then_0
      (CallFunction|CheckforJump))
    (:then_1
      (CallFunction|CheckforZoom))
    (:then_2
      (Class|BPlayer|VerticalRot (+ (Variables|Default|GetWeaponVerticalcRecoil) (Variables|Default|GetVerticalRotationInput))))
    (:then_3
      (Class|BPlayer|RotatetoCameraForward))))

(event Input|ActionEvents|InputActionFire_Weapon
  (params (Key :type Key%20Structure :default "None"))
  (bind _currendweapon (Variables|Default|GetCurrendWeapon))
  (:Pressed
    (Default|FirePressed _currendweapon))
  (:Released
    (Default|FireRelesed _currendweapon)))

(event Input|ActionEvents|InputActionJump
  (params (Key :type Key%20Structure :default "None"))
  (:Pressed
    (Class|BPlayer|CheckJump :!label _label))
  (:Released
    (goto _label)))

(event Input|ActionEvents|InputActionAim
  (params (Key :type Key%20Structure :default "None"))
  (:Pressed
    (Class|BPlayer|ToggelZoomin))
  (:Released
    (Class|BPlayer|ToggelZoomOut)))

(event Input|AxisEvents|InputAxisHorizontalMovement
  (params (AxisValue :type Float%20%28single-precision%29))
  (Class|BPlayer|Move AxisValue (stale Input|AxisEvents|InputAxisVerticalMovement AxisValue)))

(event Input|AxisEvents|InputAxisVerticalMovement
  (params (AxisValue :type Float%20%28single-precision%29))
  (Class|BPlayer|Move (stale Input|AxisEvents|InputAxisHorizontalMovement AxisValue) AxisValue))

(event Input|AxisEvents|InputAxisHorizontalRotation
  (params (AxisValue :type Float%20%28single-precision%29))
  (Class|BPlayer|HorizontalRot AxisValue))

(event Input|AxisEvents|InputAxisVerticalRotation
  (params (AxisValue :type Float%20%28single-precision%29))
  (Variables|Default|SetVerticalRotationInput AxisValue))

(event Input|AxisEvents|InputAxisZoom
  (params (AxisValue :type Float%20%28single-precision%29))
  (Class|BPlayer|Zoom AxisValue))

(fn ConstructionScript)

(fn CheckforZoom
  (if (not (Variables|Default|GetreachedTargetArmLenght))
    (Utilities|FlowControl|Sequence
      (:then_0
        (if (Variables|Default|GetisZoomingIn)
          (Class|BPlayer|Zoomin)
          (else
            (Class|BPlayer|ZoomOut))))
      (:then_1
        (Variables|/Script/Engine.SpringArmComponent|SetTargetArmLength (Variables|Default|GetArm) (Math|Float|Lerp (Variables|Default|GetcurrArmLenght) (Variables|Default|GetWeaponZoomScale) (Variables|Default|GetzoomRatio)))
        (return)))
    (else
      (return))))

(fn CheckforJump
  (if (Variables|Default|Getjumping)
    (Character|Jump)))

(fn SetVerticalWeaponRecoile
  (params (Value :type Float%20%28single-precision%29))
  (Variables|Default|SetWeaponVerticalcRecoil Value))