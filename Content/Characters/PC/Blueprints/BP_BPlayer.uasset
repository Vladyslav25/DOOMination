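; Player character for a shooter with tower building, handling movement, aim zoom, jump, pause and an Argent currency.
; Spawns three weapons at start, switches them on a hand socket, and can replace each with a V2 class.
; Tick drives jump, camera-arm zoom and vertical rotation combined with weapon recoil.
; A camera trace opens tower-point UI and disables firing; Tick closes it when the player moves too far away.
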(event EventBeginPlay
  (bind _asbp_player_anim (Utilities|Casting|CastToBP_PlayerAnim (Components|SkeletalMesh|GetAnimInstance (Variables|Character|GetMesh))))
  (Variables|References|SetAnimationInstanceRef _asbp_player_anim)
  (Weapon|SpawnAllWeapons)
  (Weapon|SwitchWeaponto))

(event EventTick
  (params (DeltaSeconds :type Float%20%28single-precision%29))
  (Utilities|FlowControl|Sequence
    (:then_0
      (CallFunction|CheckforJump))
    (:then_1
      (CallFunction|CheckforZoom))
    (:then_2
      (Class|BPlayer|VerticalRot (+ (Variables|Member|GetWeaponVerticalcRecoil) (Variables|Member|GetVerticalRotationInput))))
    (:then_3
      ;[1 1 1] If Variable is valid, UI has to be open
      (Utilities|IsValid (Variables|UIInputs|GetCurrentTowerPoint)
        (:Is%20Valid
          ;[1 1 1] Check distance between Player and tower point. If distance is too high close tower UI
          (if (> (Class|KismetMathLibrary|VectorDistanceSquared (Transformation|GetWorldLocation (Variables|Default|GetCapsuleComponent)) (Transformation|GetWorldLocation (Variables|/Game/Characters/NPC/Turrets/Blueprints/BlueprintTower/BP_TowerPoint.BP_TowerPoint_C|GetDefaultSceneRoot (Variables|UIInputs|GetCurrentTowerPoint)))) 5e+05)
            (UI|CloseTurretOptionsUI)))))))

(event Input|ActionEvents|InputActionFire_Weapon
  (params (Key :type Key%20Structure :default "None"))
  (bind _currendweapon (Variables|Member|GetCurrendWeapon))
  (:Pressed
    (Default|FirePressed _currendweapon))
  (:Released
    (Default|FireRelesed _currendweapon)))

(event Input|ActionEvents|InputActionJump
  (params (Key :type Key%20Structure :default "None"))
  (:Pressed
    (Class|BPlayer|CheckJump :!label _label))
  (:Released
    (goto _label)))

(event Input|ActionEvents|InputActionPause
  (params (Key :type Key%20Structure :default "None"))
  ;[1 1 1] Pause Game
  (:Pressed
    (UI|PauseGame)))

(event Input|ActionEvents|InputActionTestUpgradeWeapon
  (params (Key :type Key%20Structure :default "None"))
  (:Pressed
    (Weapon|UpgradeWeapon 0 2)))

(event Input|ActionEvents|InputActionAim
  (params (Key :type Key%20Structure :default "None"))
  (bind _animationinstanceref (Variables|References|GetAnimationInstanceRef))
  (:Pressed
    (Class|BPlayer|ToggelZoomin)
    (Variables|/Game/Characters/PC/Anim/Blueprints/BP_PlayerAnim.BP_PlayerAnim_C|SetIsAiming _animationinstanceref true))
  (:Released
    (Class|BPlayer|ToggelZoomOut)
    (Variables|/Game/Characters/PC/Anim/Blueprints/BP_PlayerAnim.BP_PlayerAnim_C|SetIsAiming _animationinstanceref false)))

(event Input|ActionEvents|InputActionSprint
  (params (Key :type Key%20Structure :default "None"))
  (:Pressed
    (Variables|Member|SetIsSprinting true))
  (:Released
    (Variables|Member|SetIsSprinting false)))

(event Input|ActionEvents|InputActionRelode
  (params (Key :type Key%20Structure :default "None"))
  (:Pressed
    (Default|Relode (Variables|Member|GetCurrendWeapon))))

(event Input|ActionEvents|InputActionWeapon1
  (params (Key :type Key%20Structure :default "None"))
  (:Pressed
    (Weapon|SwitchWeaponto)))

(event Input|ActionEvents|InputActionWeapon2
  (params (Key :type Key%20Structure :default "None"))
  (:Pressed
    (Weapon|SwitchWeaponto 1)))

(event Input|ActionEvents|InputActionWeapon3
  (params (Key :type Key%20Structure :default "None"))
  (:Pressed
    (Weapon|SwitchWeaponto 2)))

(event Input|ActionEvents|InputActionSwitchWeaponDown
  (params (Key :type Key%20Structure :default "None"))
  (:Released
    (bind _result (Math|Integer|DecrementInt (Variables|Member|GetCurrendWeaopnIndex))
      (:%20%20
        (if (< _result 0)
          (Variables|Member|SetCurrendWeaopnIndex (Variables|Member|GetMaxWeaponIndex)))
        (Weapon|SwitchWeaponto (Variables|Member|GetCurrendWeaopnIndex))))))

(event Input|ActionEvents|InputActionSwitchWeaponUp
  (params (Key :type Key%20Structure :default "None"))
  (:Released
    (bind _result (Math|Integer|IncrementInt (Variables|Member|GetCurrendWeaopnIndex))
      (:%20%20
        (if (> _result (Variables|Member|GetMaxWeaponIndex))
          (Variables|Member|SetCurrendWeaopnIndex 0))
        (Weapon|SwitchWeaponto (Variables|Member|GetCurrendWeaopnIndex))))))

(event Input|AxisEvents|InputAxisHorizontalMovement
  (params (AxisValue :type Float%20%28single-precision%29))
  (bind _output_get (Variables|Member|SetLeftRightMovementInput AxisValue))
  (if (Variables|Member|GetIsSprinting)
    (bind _output_get_2 (Variables|Member|SetLeftRightMovementInput (* _output_get 2.0))))
  (Variables|/Game/Characters/PC/Anim/Blueprints/BP_PlayerAnim.BP_PlayerAnim_C|SetLeftRightMovement (Variables|References|GetAnimationInstanceRef) _output_get_2))

(event Input|AxisEvents|InputAxisVerticalMovement
  (params (AxisValue :type Float%20%28single-precision%29))
  (bind _output_get (Variables|Member|SetForwardBackwardMovementInput AxisValue))
  (if (Variables|Member|GetIsSprinting)
    (bind _output_get_2 (Variables|Member|SetForwardBackwardMovementInput (* _output_get 2.0))))
  (Variables|/Game/Characters/PC/Anim/Blueprints/BP_PlayerAnim.BP_PlayerAnim_C|SetForwardBackwardMovement (Variables|References|GetAnimationInstanceRef) _output_get_2))

(event Input|AxisEvents|InputAxisHorizontalRotation
  (params (AxisValue :type Float%20%28single-precision%29))
  (Class|BPlayer|HorizontalRot AxisValue))

(event Input|AxisEvents|InputAxisVerticalRotation
  (params (AxisValue :type Float%20%28single-precision%29))
  (Variables|Member|SetVerticalRotationInput AxisValue))

(event Input|AxisEvents|InputAxisZoom
  (params (AxisValue :type Float%20%28single-precision%29))
  (Class|BPlayer|Zoom AxisValue))

(event Input|KeyboardEvents|F
  (params (Key :type Key%20Structure))
  (:Pressed
    (Utilities|IsValid (Variables|UIInputs|GetCurrentTowerPoint)
      (:Is%20Valid
        (UI|CloseTurretOptionsUI))
      (:Is%20Not%20Valid
        (UI|OpenTurretOptionsUI)))))

(fn ConstructionScript)

(fn CheckforZoom
  (if (not (Variables|Default|GetreachedTargetArmLenght))
    (Utilities|FlowControl|Sequence
      (:then_0
        (if (Variables|Default|GetisZoomingIn)
          (Class|BPlayer|Zoomin)
          (else
            (Class|BPlayer|ZoomOut))))
      (:then_1
        (Variables|/Script/Engine.SpringArmComponent|SetTargetArmLength (Variables|Default|GetArm) (Math|Float|Lerp (Variables|Default|GetcurrArmLenght) (Variables|Default|GetWeaponZoomScale) (Variables|Default|GetzoomRatio)))
        (return)))
    (else
      (return))))

(fn CheckforJump
  (if (Variables|Default|Getjumping)
    (Character|Jump)))

(fn SetVerticalWeaponRecoile
  (params (Value :type Float%20%28single-precision%29))
  (Variables|Member|SetWeaponVerticalcRecoil Value))

(fn SpawnAllWeapons
  (bind _returnvalue (Math|Vector|MakeVector 0.1 0.1 0.1))
  (bind _returnvalue_2 (Game|SpawnActorfromClass "/Game/Gameplay/Weapon/Blueprints/BP_Handgun.BP_Handgun_C" (Math|Transform|MakeTransform "0, 0, 0" "0, 0, 0" _returnvalue) "AlwaysSpawn" 0 0))
  (Utilities|Array|AddUnique (Variables|References|GetWeapons) _returnvalue_2)
  (bind _returnvalue_3 (Game|SpawnActorfromClass "/Game/Gameplay/Weapon/Blueprints/BP_Minigun.BP_Minigun_C" (Math|Transform|MakeTransform "0, 0, 0" "0, 0, 0" _returnvalue) "AlwaysSpawn" 0 0))
  (Utilities|Array|AddUnique (Variables|References|GetWeapons) _returnvalue_3)
  (bind _returnvalue_4 (Game|SpawnActorfromClass "/Game/Gameplay/Weapon/Blueprints/BP_Harpune.BP_Harpune_C" (Math|Transform|MakeTransform "0, 0, 0" "0, 0, 0" _returnvalue) "AlwaysSpawn" 0 0))
  (Utilities|Array|AddUnique (Variables|References|GetWeapons) _returnvalue_4))

(fn SwitchWeaponto
  (params (WeaponIndex :type Integer))
  (Utilities|IsValid (Variables|Member|GetCurrendWeapon)
    (:Is%20Valid
      (Transformation|DetachFromActor (Variables|Member|GetCurrendWeapon) "KeepRelative" "KeepRelative" "KeepRelative")
      (Rendering|SetVisibility (Variables|/Game/Gameplay/Weapon/Blueprints/BP_BaseWeapon.BP_BaseWeapon_C|GetRoot (Variables|Member|GetCurrendWeapon)) false true))
    (:Is%20Not%20Valid
      _))
  (bind _output_get (Variables|Member|SetCurrendWeaopnIndex WeaponIndex))
  (bind _output_get_2 (Variables|Member|SetCurrendWeapon (Utilities|Array|Get(acopy) (Variables|References|GetWeapons) _output_get)))
  (Rendering|SetVisibility (Variables|/Game/Gameplay/Weapon/Blueprints/BP_BaseWeapon.BP_BaseWeapon_C|GetRoot _output_get_2) true true)
  (Transformation|AttachComponentToComponent _output_get_2 (Variables|Character|GetMesh) "RightHandSocket" "KeepRelative" "KeepRelative" "KeepRelative" true)
  (return _output_get_2))

(fn OpenTurretOptionsUI
  (bind _camera (Variables|Default|GetCamera))
  (bind _returnvalue (Transformation|GetWorldLocation _camera))
  ;[1 1 1] Shoot a Ray from Camera to forward direction
  (bind _outhit (Collision|LineTraceByChannel _returnvalue (+ _returnvalue (* (Math|Vector|GetForwardVector _camera) 1.5e+03)) "TraceTypeQuery1" false 0 "None"))
  (bind _asbp_tower_point (Utilities|Casting|CastToBP_TowerPoint (.hitactor _outhit)))
  ;[1 1 1] Open tower UI and set correct input mode
  (Default|OpenUI _asbp_tower_point)
  (Input|SetInputModeGameandUI (Game|GetPlayerController 0) 0 "DoNotLock" true)
  (Variables|UIInputs|SetCurrentTowerPoint _asbp_tower_point)
  (Variables|/Script/Engine.PlayerController|SetbShowMouseCursor (Game|GetPlayerController 0) true)
  (Variables|/Game/Gameplay/Weapon/Blueprints/BP_BaseWeapon.BP_BaseWeapon_C|SetCanShot (Variables|Member|GetCurrendWeapon) false))

(fn CloseTurretOptionsUI
  (bind _returnvalue (Game|GetPlayerController 0))
  ;[1 1 1] Close tower UI and open main UI
  (Default|CloseUI (Variables|UIInputs|GetCurrentTowerPoint))
  (bind _returnvalue_2 (UserInterface|CreateWidget "/Game/UI/UI_Blueprints/MainGameBlueprint.MainGameBlueprint_C" _returnvalue))
  (UserInterface|Viewport|AddtoViewport _returnvalue_2 0)
  (Input|SetInputModeGameOnly _returnvalue)
  (Variables|/Script/Engine.PlayerController|SetbShowMouseCursor _returnvalue false)
  (Variables|UIInputs|SetCurrentTowerPoint 0)
  (Variables|/Game/Gameplay/Weapon/Blueprints/BP_BaseWeapon.BP_BaseWeapon_C|SetCanShot (Variables|Member|GetCurrendWeapon) true))

(fn HasAmountOfArgent
  (params (Needed%20Amount :type Integer))
  (return (<= Needed%20Amount (Variables|Member|GetArgentAmount))))

(fn AddArgent
  (params (Amount :type Integer))
  (Variables|Member|SetArgentAmount (+ Amount (Variables|Member|GetArgentAmount))))

(fn RemoveArgent
  (params (Amount :type Integer))
  (if (ArgentManagment|HasAmountOfArgent Amount)
    (Variables|Member|SetArgentAmount (- (Variables|Member|GetArgentAmount) Amount))
    (return true)
    (else
      (return false))))

(fn PauseGame
  (bind _returnvalue (Game|GetPlayerController 0))
  (Game|SetGamePaused true)
  (Utilities|IsValid (Variables|Default|GetPause%20Menu)
    (:Is%20Valid
      _)
    (:Is%20Not%20Valid
      (bind _returnvalue_2 (UserInterface|CreateWidget "/Game/UI/UI_Blueprints/PauseBlueprint.PauseBlueprint_C" _returnvalue))
      (Variables|Default|SetPause%20Menu _returnvalue_2)))
  (UserInterface|Viewport|AddtoViewport (Variables|Default|GetPause%20Menu) 0)
  (Input|SetInputModeUIOnly _returnvalue (Variables|Default|GetPause%20Menu) "DoNotLock")
  (Variables|/Script/Engine.PlayerController|SetbShowMouseCursor _returnvalue true))

(fn ResumeGame
  (bind _returnvalue (Game|GetPlayerController 0))
  (Game|SetGamePaused false)
  (Viewport|RemoveAllWidgets)
  ;[1 1 1] Main Ui Blueprint
  (bind _returnvalue_2 (UserInterface|CreateWidget "/Game/UI/UI_Blueprints/MainGameBlueprint.MainGameBlueprint_C" _returnvalue))
  (UserInterface|Viewport|AddtoViewport _returnvalue_2 0)
  (Variables|/Script/Engine.PlayerController|SetbShowMouseCursor _returnvalue false)
  (Input|SetInputModeGameOnly _returnvalue)
  (bind _returnvalue_3 (Actor|GetActorOfClass "BP_BPlayer_C"))
  (Variables|Default|SetPlayer _returnvalue_3))

(fn UpgradeWeapon
  (params (ArgentCost :type Integer) (WeaponIndex :type Integer))
  (if (and (ArgentManagment|HasAmountOfArgent ArgentCost) (not (Utilities|Array|Get(acopy) (Variables|Member|GetUpgradedWeaponIndex) WeaponIndex)))
    ;[1 1 1] Destroy old Weapon
    (Actor|DestroyActor (Utilities|Array|Get(acopy) (Variables|References|GetWeapons) WeaponIndex))
    ;[1 1 1] Spawn New Weapon and set it in the Array Index
    (bind _returnvalue (Game|SpawnActorfromClass (Utilities|Array|Get(acopy) (Variables|Member|GetWeaponsV2) WeaponIndex) (Math|Transform|MakeTransform "0, 0, 0" "0, 0, 0" "0.100000,0.100000,0.100000") "Undefined" 0 0))
    (Utilities|Array|SetArrayElem (Variables|References|GetWeapons) WeaponIndex _returnvalue)
    (Weapon|SwitchWeaponto WeaponIndex)
    (return true)
    (else
      (return false))))