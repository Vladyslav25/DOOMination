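; Player character Blueprint handling movement, weapons, Argent currency, upgrader interaction, pausing and defeat.
; Movement input feeds the anim instance for root motion, switched off while launched, while Tick drives jumping, spring-arm zoom and recoil-adjusted pitch.
; Three weapon slots support tier-two upgrades, the middle becoming an LMG previewed by ground trace, then placed, possessed or collected.
; A timer rising while enemies overlap DeathRange opens the Defeat level at its limit.
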(event OnComponentBeginOverlap(DeathRange)
  (params (OverlappedComponent :type Primitive%20Component%20Object%20Reference) (OtherActor :type Actor%20Object%20Reference) (OtherComp :type Primitive%20Component%20Object%20Reference) (OtherBodyIndex :type Integer) (bFromSweep :type Boolean) (SweepResult :type Hit%20Result%20Structure%20%28by%20ref%29))
  (Utilities|Casting|CastToBP_BaseEnemy OtherActor)
  (Math|Integer|IncrementInt (Variables|Member|Private|GetEnemyAmountInDeathRange)))

(event OnComponentEndOverlap(DeathRange)
  (params (OverlappedComponent :type Primitive%20Component%20Object%20Reference) (OtherActor :type Actor%20Object%20Reference) (OtherComp :type Primitive%20Component%20Object%20Reference) (OtherBodyIndex :type Integer))
  (Utilities|Casting|CastToBP_BaseEnemy OtherActor)
  (Math|Integer|DecrementInt (Variables|Member|Private|GetEnemyAmountInDeathRange)))

(event EventBeginPlay
  (bind _asbp_player_anim (Utilities|Casting|CastToBP_PlayerAnim (Components|SkeletalMesh|GetAnimInstance (Variables|Character|GetMesh))))
  (Variables|References|SetAnimationInstanceRef _asbp_player_anim)
  (Weapon|SpawnAllWeapons)
  (Weapon|SwitchWeaponto)
  (Variables|Member|Private|Controller|SetMovementMultiplikator (Variables|Setting|Private|Controller|Movement|GetWalkingMultiplier)))

(event EventTick
  (params (DeltaSeconds :type Float%20%28single-precision%29))
  (Utilities|FlowControl|Sequence
    (:then_0
      (Controller|ProcessJumping))
    (:then_1
      (Controller|UpdateZoom DeltaSeconds))
    (:then_2
      (Controller|VerticalRotation (+ (Variables|Member|Private|Controller|GetVerticalRotationInput) (Variables|Member|Private|Weapopn|GetWeaponVerticalRecoil))))
    (:then_3
      (if (> (Variables|Member|Private|GetEnemyAmountInDeathRange) 0)
        (bind _output_get (Variables|Member|Public|SetDeathTimer (+ DeltaSeconds (Variables|Member|Public|GetDeathTimer))))
        (else
          (Variables|Member|Public|SetDeathTimer (Math|Float|Clamp(Float) (- (Variables|Member|Public|GetDeathTimer) DeltaSeconds)))))
      (Development|PrintString (Utilities|String|ToString(Float) _output_get) true true "(R=1.000000,G=0.000000,B=0.000000,A=1.000000)" 0.0)
      (if (>= (Variables|Member|Public|GetDeathTimer) (Variables|Setting|Private|GetMaxDeathTimer))
        (Game|OpenLevel(byName) "Defeat")))
    (:then_4
      (if (Weapon|IsLMGSelected)
        (if (not (Variables|Member|Public|GetLMGPlaced))
          (bind _asbp_lmg (Utilities|Casting|CastToBP_LMG (Variables|Member|Public|GetCurrendWeapon)))
          (bind _output (Weapon|GetLMGTransform))
          (bind _isvalid (Default|CheckforPosition _asbp_lmg _output))
          (if _isvalid
            _
            (else
              _))
          (Transformation|SetActorTransform _asbp_lmg _output))))
    (:then_5
      (Utilities|IsValid (Variables|References|UI|GetCurrentInteractedPoint)
        (:Is%20Valid
          (if (> (Class|KismetMathLibrary|VectorDistanceSquared (Transformation|GetWorldLocation (Variables|Collision|GetCapsuleComponent)) (Transformation|GetWorldLocation (Variables|/Game/Characters/NPC/Turrets/Blueprints/BlueprintTower/BP_TowerPoint.BP_TowerPoint_C|GetDefaultSceneRoot (Variables|References|UI|GetCurrentInteractedPoint)))) 5e+05)
            (UI|CloseInteractedUI)))))))

(event EventOnLaunched
  (params (LaunchVelocity :type Vector :default "0, 0, 0") (bXYOverride :type Boolean) (bZOverride :type Boolean))
  (Class|AnimInstance|SetRootMotionMode (Variables|References|GetAnimationInstanceRef) "NoRootMotionExtraction"))

(event EventOnLanded
  (params (Hit :type Hit%20Result%20Structure%20%28by%20ref%29))
  (Class|AnimInstance|SetRootMotionMode (Variables|References|GetAnimationInstanceRef) "RootMotionFromEverything"))

(event Input|ActionEvents|InputActionInteract
  (params (Key :type Key%20Structure :default "None"))
  (bind _weapons (Variables|References|GetWeapons))
  (bind _output (Utilities|Array|Get(acopy) _weapons 1))
  ;[1 1 1] Interaction
  (:Pressed
    (if (Variables|Member|Public|GetLMGInRange)
      (Utilities|IsValid _output
        (:Is%20Valid
          (bind _asbp_lmg (Utilities|Casting|CastToBP_LMG _output))
          (Default|TakePossesion _asbp_lmg))
        (:Is%20Not%20Valid
          (Utilities|IsValid (Variables|References|UI|GetCurrentInteractedPoint) :!label _label
            (:Is%20Valid
              (UI|CloseInteractedUI))
            (:Is%20Not%20Valid
              (bind (_hitupgrader _upgrader) (Controller|ShootRayinFrontOfPlayer))
              (if _hitupgrader
                (UI|OpenInteractedUI _upgrader)
                (else
                  (UI|CloseInteractedUI)))))))
      (elif (not (Weapon|IsLMGSelected))
        (goto _label)
        (else
          (bind _asbp_lmg_2 (Utilities|Casting|CastToBP_LMG _output))
          (Default|PlaceatCurrendLocation _asbp_lmg_2))))))

(event Input|ActionEvents|InputActionJump
  (params (Key :type Key%20Structure :default "None"))
  ;[1 1 1] Player Controller
  ;;[1 1 1] Input Jump
  (:Pressed
    (Controller|CheckJump :!label _label))
  (:Released
    (goto _label)))

(event Input|ActionEvents|InputActionFire_Weapon
  (params (Key :type Key%20Structure :default "None"))
  (bind _output (Weapon|IsLMGSelected))
  (bind _currendweapon (Variables|Member|Public|GetCurrendWeapon))
  (bind _returnvalue (not _output))
  ;[1 1 1] WeaponHandeling
  ;;[0.2999 0.496 1] Fire Weapon
  (:Pressed
    (if _returnvalue
      (Default|FirePressed _currendweapon)
      (else
        (bind _asbp_lmg (Utilities|Casting|CastToBP_LMG _currendweapon))
        (Default|PlaceatCurrendLocation _asbp_lmg))))
  (:Released
    (if _returnvalue
      (Default|FireRelesed _currendweapon))))

(event Input|ActionEvents|InputActionRelode
  (params (Key :type Key%20Structure :default "None"))
  ;[1 1 1] WeaponHandeling
  ;;[1 0.2705 0.2904] Relode
  (:Pressed
    (if (not (Weapon|IsLMGSelected))
      (Variables|/Game/Characters/PC/Anim/Blueprints/BP_PlayerAnim.BP_PlayerAnim_C|SetIsReloding (Variables|References|GetAnimationInstanceRef) true)
      (Default|Relode (Variables|Member|Public|GetCurrendWeapon))
      ;[1 1 1] TODO: Entfernen, wenn Animations Notify Relode Beendet
      (Variables|/Game/Characters/PC/Anim/Blueprints/BP_PlayerAnim.BP_PlayerAnim_C|SetIsReloding (Variables|References|GetAnimationInstanceRef) false))))

(event Input|ActionEvents|InputActionPause
  (params (Key :type Key%20Structure :default "None"))
  ;[1 1 1] Pause Game
  (:Pressed
    (UI|PauseGame)))

(event Input|ActionEvents|InputActionCollect
  (params (Key :type Key%20Structure :default "None"))
  (bind _charactermovement (Variables|Character|GetCharacterMovement))
  ;[1 1 1] Collect LMG
  (:Pressed
    (if (Variables|Member|Public|GetLMGInRange)
      (Pawn|Components|CharacterMovement|DisableMovement _charactermovement)
      (bind _asbp_lmg (Utilities|Casting|CastToBP_LMG (Utilities|Array|Get(acopy) (Variables|References|GetWeapons) 1)))
      (Utilities|FlowControl|Delay (Variables|/Game/Gameplay/Weapon/Blueprints/Weapons/BP_LMG.BP_LMG_C|GetCollectTime _asbp_lmg))
      (Actor|DestroyActor _asbp_lmg)
      (Pawn|Components|CharacterMovement|SetMovementMode _charactermovement "MOVE_Walking" 0)
      (Variables|Member|Public|SetLMGPlaced false))))

(event Input|ActionEvents|InputActionAim
  (params (Key :type Key%20Structure :default "None"))
  (bind _animationinstanceref (Variables|References|GetAnimationInstanceRef))
  ;[1 1 1] WeaponHandeling
  ;;[0.3149 1 0.2686] Aim
  (:Pressed
    (Controller|ToggelZoomin)
    (Variables|/Game/Characters/PC/Anim/Blueprints/BP_PlayerAnim.BP_PlayerAnim_C|SetIsAiming _animationinstanceref true)
    (Variables|Member|Private|Controller|SetMovementMultiplikator (Variables|Setting|Private|Controller|Movement|GetAimingMovementMultiplier)))
  (:Released
    (Controller|ToggelZoomOut)
    (Variables|/Game/Characters/PC/Anim/Blueprints/BP_PlayerAnim.BP_PlayerAnim_C|SetIsAiming _animationinstanceref false)
    (Variables|Member|Private|Controller|SetMovementMultiplikator (Variables|Setting|Private|Controller|Movement|GetWalkingMultiplier))))

(event Input|ActionEvents|InputActionSprint
  (params (Key :type Key%20Structure :default "None"))
  ;[1 1 1] Player Controller
  ;;[1 1 1] Sprint
  (:Pressed
    (Variables|Member|Private|Controller|SetIsSprinting true)
    (Variables|Member|Private|Controller|SetMovementMultiplikator (Variables|Setting|Private|Controller|Movement|GetSprintMultiplier)))
  (:Released
    (Variables|Member|Private|Controller|SetIsSprinting false)
    (Variables|Member|Private|Controller|SetMovementMultiplikator (Variables|Setting|Private|Controller|Movement|GetWalkingMultiplier))))

(event Input|ActionEvents|InputActionTestUpgradeWeapon
  (params (Key :type Key%20Structure :default "None"))
  ;[1 1 1] Test Upgrade Weapon
  (:Pressed
    (Weapon|UpgradeWeapon 0 1)))

(event Input|ActionEvents|InputActionWeapon1
  (params (Key :type Key%20Structure :default "None"))
  ;[1 1 1] WeaponHandeling
  ;;[1 0.9348 0.3437] Switch Weapon Number
  (:Pressed
    (Weapon|SwitchWeaponto)))

(event Input|ActionEvents|InputActionWeapon2
  (params (Key :type Key%20Structure :default "None"))
  ;[1 1 1] WeaponHandeling
  ;;[1 0.9348 0.3437] Switch Weapon Number
  (:Pressed
    (Weapon|SwitchWeaponto 1)))

(event Input|ActionEvents|InputActionWeapon3
  (params (Key :type Key%20Structure :default "None"))
  ;[1 1 1] WeaponHandeling
  ;;[1 0.9348 0.3437] Switch Weapon Number
  (:Pressed
    (Weapon|SwitchWeaponto 2)))

(event Input|ActionEvents|InputActionSwitchWeaponDown
  (params (Key :type Key%20Structure :default "None"))
  ;[1 1 1] WeaponHandeling
  ;;[1 0.9315 0.2456] Switch Weapon MouseWheel
  (:Released
    (bind _result (Math|Integer|DecrementInt (Variables|Member|Public|GetCurrendWeaponIndex))
      (:%20%20
        (if (< _result 0)
          (Variables|Member|Public|SetCurrendWeaponIndex (Variables|Setting|Private|GetMaxWeaponIndex)))
        (Weapon|SwitchWeaponto (Variables|Member|Public|GetCurrendWeaponIndex))))))

(event Input|ActionEvents|InputActionSwitchWeaponUp
  (params (Key :type Key%20Structure :default "None"))
  ;[1 1 1] WeaponHandeling
  ;;[1 0.9315 0.2456] Switch Weapon MouseWheel
  (:Released
    (bind _result (Math|Integer|IncrementInt (Variables|Member|Public|GetCurrendWeaponIndex))
      (:%20%20
        (if (> _result (Variables|Setting|Private|GetMaxWeaponIndex))
          (Variables|Member|Public|SetCurrendWeaponIndex 0))
        (Weapon|SwitchWeaponto (Variables|Member|Public|GetCurrendWeaponIndex))))))

(event Input|AxisEvents|InputAxisHorizontalMovement
  (params (AxisValue :type Float%20%28single-precision%29))
  ;[1 1 1] Player Controller
  ;;[1 1 1] Input Movement
  (Variables|/Game/Characters/PC/Anim/Blueprints/BP_PlayerAnim.BP_PlayerAnim_C|SetLeftRightMovement (Variables|References|GetAnimationInstanceRef) (* AxisValue (Variables|Member|Private|Controller|GetMovementMultiplikator))))

(event Input|AxisEvents|InputAxisVerticalMovement
  (params (AxisValue :type Float%20%28single-precision%29))
  ;[1 1 1] Player Controller
  ;;[1 1 1] Input Movement
  (Variables|/Game/Characters/PC/Anim/Blueprints/BP_PlayerAnim.BP_PlayerAnim_C|SetForwardBackwardMovement (Variables|References|GetAnimationInstanceRef) (* (Variables|Member|Private|Controller|GetMovementMultiplikator) AxisValue)))

(event Input|AxisEvents|InputAxisHorizontalRotation
  (params (AxisValue :type Float%20%28single-precision%29))
  ;[1 1 1] Player Controller
  ;;[1 1 1] Rotation
  (Controller|HorizontalRotation AxisValue))

(event Input|AxisEvents|InputAxisVerticalRotation
  (params (AxisValue :type Float%20%28single-precision%29))
  ;[1 1 1] Player Controller
  ;;[1 1 1] Rotation
  (Variables|Member|Private|Controller|SetVerticalRotationInput AxisValue))

(fn ConstructionScript)

(fn CloseInteractedUI
  (bind _returnvalue (Game|GetPlayerController 0))
  ;[1 1 1] Close tower UI and open main UI
  (Default|CloseUI (Variables|References|UI|GetCurrentInteractedPoint))
  (bind _returnvalue_2 (UserInterface|CreateWidget "/Game/UI/UI_Blueprints/MainGameBlueprint.MainGameBlueprint_C" _returnvalue))
  (UserInterface|Viewport|AddtoViewport _returnvalue_2 0)
  (Input|SetInputModeGameOnly _returnvalue)
  (Variables|/Script/Engine.PlayerController|SetbShowMouseCursor _returnvalue false)
  (Variables|References|UI|SetCurrentInteractedPoint 0)
  (Variables|/Game/Gameplay/Weapon/Blueprints/Weapons/BP_BaseWeapon.BP_BaseWeapon_C|SetCanShot (Variables|Member|Public|GetCurrendWeapon) true))

(fn OpenInteractedUI
  (params (InteractedPoint :type BP%20Base%20Upgrader%20Object%20Reference))
  ;[1 1 1] Open tower UI and set correct input mode
  (Default|OpenUI InteractedPoint)
  (Input|SetInputModeGameandUI (Game|GetPlayerController 0) 0 "DoNotLock" true)
  (Variables|References|UI|SetCurrentInteractedPoint InteractedPoint)
  (Variables|/Script/Engine.PlayerController|SetbShowMouseCursor (Game|GetPlayerController 0) true)
  (Variables|/Game/Gameplay/Weapon/Blueprints/Weapons/BP_BaseWeapon.BP_BaseWeapon_C|SetCanShot (Variables|Member|Public|GetCurrendWeapon) false))

(fn HorizontalRotation
  (params (Input :type Float%20%28single-precision%29))
  (Transformation|AddWorldRotation (Variables|Collision|GetCapsuleComponent) (Math|Rotator|MakeRotator 0.0 0.0 (* Input (Variables|Member|Private|Controller|GetRotationSpeed) (Utilities|Time|GetWorldDeltaSeconds))) false false))

(fn Move
  (params (ForwardBackward_Input :type Float%20%28single-precision%29) (LeftRight_Input :type Float%20%28single-precision%29) (Multiplier :type Float%20%28single-precision%29))
  (Pawn|Input|AddMovementInput (Math|Vector|MakeVector ForwardBackward_Input 0.0 LeftRight_Input) Multiplier false))

(fn ToggelZoomin
  (Variables|Member|Private|Controller|SetIsZoomingIn true)
  (Variables|Member|Private|Controller|SetRotationSpeed (Variables|Setting|Private|Controller|Rotation|GetAimingRotationSpeed))
  (Variables|Member|Private|Controller|SetMovementMultiplikator (Variables|Setting|Private|Controller|Movement|GetAimingMovementMultiplier))
  (Variables|Member|Private|Controller|SetIsPressingAim true))

(fn CheckJump
  (if (Variables|Member|Private|Controller|GetJumping)
    (Variables|Member|Private|Controller|SetJumping false)
    (else
      (Variables|Member|Private|Controller|SetJumping true))))

(fn ToggelZoomOut
  (Variables|Member|Private|Controller|SetIsZoomingIn false)
  (Variables|Member|Private|Controller|SetRotationSpeed (Variables|Setting|Private|Controller|Rotation|GetWalkingRotaionSpeed))
  (Variables|Member|Private|Controller|SetMovementMultiplikator (Variables|Setting|Private|Controller|Movement|GetWalkingMultiplier))
  (Variables|Member|Private|Controller|SetIsPressingAim false))

(fn VerticalRotation
  (params (Value :type Float%20%28single-precision%29))
  (bind _arm (Variables|Default|GetArm))
  (bind _relativerotation (Variables|/Script/Engine.SceneComponent|GetRelativeRotation _arm))
  (bind _returnvalue (+ (.pitch _relativerotation) Value))
  (if (and (< _returnvalue 45.0) (> _returnvalue -65.0))
    (Transformation|AddLocalRotation _arm (Math|Rotator|MakeRotator 0.0 Value 0.0) false false)))

(fn UpdateZoom
  (params (DeltaTime :type Float%20%28single-precision%29))
  (bind _aimingspeed (Variables|Setting|Private|GetAimingSpeed))
  (bind _returnvalue (* _aimingspeed DeltaTime))
  (Utilities|FlowControl|Sequence
    (:then_0
      (if (Variables|Member|Private|Controller|GetIsZoomingIn)
        (Variables|Member|Private|Controller|SetZoomRatio (Math|Float|Clamp(Float) (+ (Variables|Member|Private|Controller|GetZoomRatio) _returnvalue)))
        (else
          (Variables|Member|Private|Controller|SetZoomRatio (Math|Float|Clamp(Float) (- (Variables|Member|Private|Controller|GetZoomRatio) _returnvalue))))))
    (:then_1
      (Variables|/Script/Engine.SpringArmComponent|SetTargetArmLength (Variables|Default|GetArm) (Math|Float|Lerp (Variables|Setting|Private|GetIdleArmLength) (Variables|Setting|Private|GetAimingArmLength) (Variables|Member|Private|Controller|GetZoomRatio))))))

(fn SetVerticalWeaponRecoile
  (params (Value :type Float%20%28single-precision%29))
  (Variables|Member|Private|Weapopn|SetWeaponVerticalRecoil Value))

(fn SpawnAllWeapons
  (bind _returnvalue (Game|SpawnActorfromClass "/Game/Gameplay/Weapon/Blueprints/Weapons/BP_Handgun.BP_Handgun_C" (Math|Transform|MakeTransform "0, 0,-500.000000" "0, 0, 0" "1,1,1") "AlwaysSpawn" 0 0))
  (Utilities|Array|AddUnique (Variables|References|GetWeapons) _returnvalue)
  (bind _returnvalue_2 (Game|SpawnActorfromClass "/Game/Gameplay/Weapon/Blueprints/Weapons/BP_Minigun.BP_Minigun_C" (Math|Transform|MakeTransform "0, 0,-500.000000" "0, 0, 0" "1,1,1") "AlwaysSpawn" 0 0))
  (Utilities|Array|AddUnique (Variables|References|GetWeapons) _returnvalue_2)
  (bind _returnvalue_3 (Game|SpawnActorfromClass "/Game/Gameplay/Weapon/Blueprints/Weapons/BP_Harpune.BP_Harpune_C" (Math|Transform|MakeTransform "0, 0,-500.000000" "0, 0, 0" "1,1,1") "AlwaysSpawn" 0 0))
  (Utilities|Array|AddUnique (Variables|References|GetWeapons) _returnvalue_3))

(fn SwitchWeaponto
  (params (Index :type Integer))
  (Utilities|IsValid (Variables|Member|Public|GetCurrendWeapon)
    (:Is%20Valid
      (bind _asbp_lmg (Utilities|Casting|CastToBP_LMG (Variables|Member|Public|GetCurrendWeapon))
        (:then
          (if (Variables|Member|Public|GetLMGPlaced)
            _
            (else
              (Actor|DestroyActor _asbp_lmg))))
        (:CastFailed
          (Transformation|DetachFromActor (Variables|Member|Public|GetCurrendWeapon) "KeepRelative" "KeepRelative" "KeepRelative")
          (Rendering|SetVisibility (Variables|/Game/Gameplay/Weapon/Blueprints/Weapons/BP_BaseWeapon.BP_BaseWeapon_C|GetRoot (Variables|Member|Public|GetCurrendWeapon)) false true))))
    (:Is%20Not%20Valid
      _))
  (bind _output_get (Variables|Member|Public|SetCurrendWeaponIndex Index))
  (Weapon|ChangeWepaonEnuminAnim)
  (bind _output_get_2 (Variables|Member|Public|SetCurrendWeapon (Utilities|Array|Get(acopy) (Variables|References|GetWeapons) _output_get)))
  (if (and (Utilities|Array|Get(acopy) (Variables|Member|Public|GetUpgradedWeaponIndex) 1) (== _output_get 1))
    (if (Variables|Member|Public|GetLMGPlaced)
      _
      (else
        (bind _newlmg (Weapon|SpawnLMG))
        (Rendering|SetVisibility (Variables|/Script/Engine.Actor|GetRootComponent _newlmg) true true)
        (return _output_get_2)))
    (else
      (Rendering|SetVisibility (Variables|/Game/Gameplay/Weapon/Blueprints/Weapons/BP_BaseWeapon.BP_BaseWeapon_C|GetRoot _output_get_2) true true)
      (Transformation|AttachComponentToComponent _output_get_2 (Variables|Character|GetMesh) "RightHandSocket" "SnapToTarget" "KeepRelative" "KeepRelative" true)))
  (return _output_get_2))

(fn UpgradeWeapon
  (params (ArgentCost :type Integer) (WeaponIndex :type Integer))
  (bind _weapons_tier2 (Variables|Setting|Private|GetWeapons_Tier2))
  (bind _output (Utilities|Array|Get(acopy) _weapons_tier2 WeaponIndex))
  (if (and (ArgentManagment|HasAmountOfArgent ArgentCost) (not (Utilities|Array|Get(acopy) (Variables|Member|Public|GetUpgradedWeaponIndex) WeaponIndex)))
    ;[1 1 1] Destroy old Weapon
    (Actor|DestroyActor (Utilities|Array|Get(acopy) (Variables|References|GetWeapons) WeaponIndex))
    (if (!= _output "/Game/Gameplay/Weapon/Blueprints/Weapons/BP_LMG.BP_LMG_C")
      ;[1 1 1] Spawn New Weapon and set it in the Array Index
      (bind _returnvalue (Game|SpawnActorfromClass _output (Math|Transform|MakeTransform "0, 0, 0" "0, 0, 0" "1,1,1") "Undefined" 0 0))
      (Utilities|Array|SetArrayElem (Variables|References|GetWeapons) WeaponIndex _returnvalue)
      (Class|FMODBlueprintStatics|PlayEvent2D (Variables|/Game/Gameplay/Weapon/Blueprints/Weapons/BP_BaseWeapon.BP_BaseWeapon_C|GetUpgradeSound _returnvalue))
      (else
        (Class|FMODBlueprintStatics|PlayEvent2D "/Game/FMOD/Events/Weapon_Upgrade_Sounds/lmg_upgrade.lmg_upgrade")))
    (Utilities|Array|SetArrayElem (Variables|Member|Public|GetUpgradedWeaponIndex) WeaponIndex true)
    (Weapon|SwitchWeaponto WeaponIndex)
    (return true)
    (else
      (return false))))

(fn HasAmountOfArgent
  (params (NeededAmount :type Integer))
  (return (<= NeededAmount (Variables|Member|Private|GetArgentAmount))))

(fn GetAmountOfArgent
  (return (Variables|Member|Private|GetArgentAmount)))

(fn AddArgent
  (params (Amount :type Integer))
  (Variables|Member|Private|SetArgentAmount (+ Amount (Variables|Member|Private|GetArgentAmount))))

(fn RemoveArgent
  (params (Amount :type Integer))
  (if (ArgentManagment|HasAmountOfArgent Amount)
    (Variables|Member|Private|SetArgentAmount (- (Variables|Member|Private|GetArgentAmount) Amount))
    (return true)
    (else
      (return false))))

(fn PauseGame
  (bind _returnvalue (Game|GetPlayerController 0))
  (Game|SetGamePaused true)
  (Utilities|IsValid (Variables|References|UI|GetOpenedMenu)
    (:Is%20Valid
      _)
    (:Is%20Not%20Valid
      (bind _returnvalue_2 (UserInterface|CreateWidget "/Game/UI/UI_Blueprints/PauseBlueprint.PauseBlueprint_C" _returnvalue))
      (bind _output_get (Variables|References|UI|SetOpenedMenu _returnvalue_2))))
  (UserInterface|Viewport|AddtoViewport _output_get 0)
  (Input|SetInputModeUIOnly _returnvalue _output_get "DoNotLock")
  (Variables|/Script/Engine.PlayerController|SetbShowMouseCursor _returnvalue true))

(fn ResumeGame
  (bind _returnvalue (Game|GetPlayerController 0))
  (Game|SetGamePaused false)
  (Viewport|RemoveAllWidgets)
  ;[1 1 1] Main Ui Blueprint
  (bind _returnvalue_2 (UserInterface|CreateWidget "/Game/UI/UI_Blueprints/MainGameBlueprint.MainGameBlueprint_C" _returnvalue))
  (UserInterface|Viewport|AddtoViewport _returnvalue_2 0)
  (Variables|/Script/Engine.PlayerController|SetbShowMouseCursor _returnvalue false)
  (Input|SetInputModeGameOnly _returnvalue))

(fn ProcessJumping
  (if (Variables|Member|Private|Controller|GetJumping)
    (Character|Jump)))

(fn GetLMGTransform
  (bind _returnvalue (Transformation|GetActorForwardVector))
  (bind _returnvalue_2 (Transformation|GetActorLocation))
  (bind _returnvalue_3 (* _returnvalue 2.6e+02))
  (bind (_outhit _returnvalue_4) (Collision|LineTraceByChannel (+ _returnvalue_3 (+ _returnvalue_2 "0, 0,-60.000000")) (+ _returnvalue_3 (+ _returnvalue_2 (Math|Vector|MakeVector 0.0 0.0 -1.2e+02))) "TraceTypeQuery1" false 0 "None"))
  (if _returnvalue_4
    (return (Math|Transform|MakeTransform (.ImpactPoint (Collision|BreakHitResult _outhit)) (Math|Rotator|MakeRotator (.pitch (Math|Rotator|MakeRotfromZ (.ImpactNormal (Collision|BreakHitResult _outhit)))) (.roll (Math|Rotator|MakeRotfromZ (.ImpactNormal (Collision|BreakHitResult _outhit)))) (.yaw (Math|Rotator|MakeRotfromX (Transformation|GetActorForwardVector)))) "1,1,1"))))

(fn IsLMGSelected
  (return (Math|Boolean|ANDBoolean (== (Variables|Member|Public|GetCurrendWeaponIndex) 1) (Utilities|Array|Get(acopy) (Variables|Member|Public|GetUpgradedWeaponIndex) 1) (Utilities|IsValid (Variables|Member|Public|GetCurrendWeapon)))))

(fn SpawnLMG
  (bind _returnvalue (Game|SpawnActorfromClass "/Game/Gameplay/Weapon/Blueprints/Weapons/BP_LMG.BP_LMG_C" (Math|Transform|MakeTransform "0, 0, 0" "0, 0, 0" "1,1,1") "AdjustIfPossibleButAlwaysSpawn" 0 0))
  (Utilities|Array|SetArrayElem (Variables|References|GetWeapons) 1 _returnvalue)
  (Variables|Member|Public|SetCurrendWeapon _returnvalue)
  (return _returnvalue))

(fn ShootRayinFrontOfPlayer
  (bind _camera (Variables|Default|GetCamera))
  (bind _returnvalue (Transformation|GetWorldLocation _camera))
  ;[1 1 1] Shoot a Ray from Camera to forward direction
  (bind _outhit (Collision|LineTraceByChannel _returnvalue (+ _returnvalue (* (Math|Vector|GetForwardVector _camera) 1.5e+03)) "TraceTypeQuery1" false 0 "None"))
  (bind _asbp_base_upgrader (Utilities|Casting|CastToBP_BaseUpgrader (.hitactor _outhit))
    (:then
      (return true _asbp_base_upgrader))
    (:CastFailed
      (return false 0))))

(fn ChangeWepaonEnuminAnim
  (bind _currendweaponindex (Variables|Member|Public|GetCurrendWeaponIndex))
  (bind _animationinstanceref (Variables|References|GetAnimationInstanceRef))
  (if (Utilities|Array|Get(acopy) (Variables|Member|Public|GetUpgradedWeaponIndex) _currendweaponindex)
    (switch int _currendweaponindex
      (:0
        (Variables|/Game/Characters/PC/Anim/Blueprints/BP_PlayerAnim.BP_PlayerAnim_C|SetCurrendWeapon _animationinstanceref "NewEnumerator3"))
      (:1
        (Variables|/Game/Characters/PC/Anim/Blueprints/BP_PlayerAnim.BP_PlayerAnim_C|SetCurrendWeapon _animationinstanceref "NewEnumerator4"))
      (:2
        (Variables|/Game/Characters/PC/Anim/Blueprints/BP_PlayerAnim.BP_PlayerAnim_C|SetCurrendWeapon _animationinstanceref "NewEnumerator5")))
    (else
      (switch int _currendweaponindex
        (:0
          (Variables|/Game/Characters/PC/Anim/Blueprints/BP_PlayerAnim.BP_PlayerAnim_C|SetCurrendWeapon _animationinstanceref "NewEnumerator0"))
        (:1
          (Variables|/Game/Characters/PC/Anim/Blueprints/BP_PlayerAnim.BP_PlayerAnim_C|SetCurrendWeapon _animationinstanceref "NewEnumerator1"))
        (:2
          (Variables|/Game/Characters/PC/Anim/Blueprints/BP_PlayerAnim.BP_PlayerAnim_C|SetCurrendWeapon _animationinstanceref "NewEnumerator2"))))))