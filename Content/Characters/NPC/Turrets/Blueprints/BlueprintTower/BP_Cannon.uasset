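; Cannon turret, a child tower Blueprint that fires BP_CannonProjectile and defines its own cost and per-level damage, attack speed and range increments.
; After each shot it cycles round-robin through its muzzle arrows, which grow to two at level 30 and four at level 90.
; Override functions supply milestone mesh swaps for the parent and report cannon shots and upgrades to the data collector.
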(event EventBeginPlay
  (|CallParentFunction)
  (bind _output_get (Variables|Default|SetMainArrowComponent (Variables|Default|GetArrow)))
  (Variables|Default|SetProjectile "/Game/Characters/NPC/Turrets/Blueprints/BlueprintProjectile/BP_CannonProjectile.BP_CannonProjectile_C")
  (Utilities|Array|Add (Variables|Default|GetArrowArray) _output_get)
  (CallFunction|AddMeshes (Utilities|Array|MakeArray (Variables|Default|GetBarrel_B) (Variables|Default|GetScope_M) (Variables|Default|GetAmmo_M))))

(event Collision|EventActorBeginOverlap
  (params (OtherActor :type Actor%20Object%20Reference)))

(event EventTick
  (params (DeltaSeconds :type Float%20%28single-precision%29))
  (|CallParentFunction DeltaSeconds) ; This node is disabled and will not be called.\nDrag off pins to build functionality.
)

(event EventEvery10thLevel
  (bind _arrowarray (Variables|Default|GetArrowArray))
  (bind _arrowarray_2 (Variables|Default|GetArrowArray))
  (|CallParentFunction)
  (switch int (/ (CallFunction|GetCurrentLevel) 10)
    (:3
      ;[1 1 1] Cange Arrows so is looks more fancy
      (Utilities|Array|Clear (Variables|Default|GetArrowArray))
      (Utilities|Array|Add _arrowarray_2 (Variables|Default|Get2_Arrow_1))
      (Utilities|Array|Add _arrowarray_2 (Variables|Default|Get2_Arrow_2)))
    (:9
      (Utilities|Array|Clear (Variables|Default|GetArrowArray))
      (Utilities|Array|Add _arrowarray (Variables|Default|Get3_Arrow_TL))
      (Utilities|Array|Add _arrowarray (Variables|Default|Get3_Arrow_DL))
      (Utilities|Array|Add _arrowarray (Variables|Default|Get3_Arrow_TR))
      (Utilities|Array|Add _arrowarray (Variables|Default|Get3_Arrow_DR)))))

(event EventOnDeleteTower
  (CallFunction|AddMeshes (Utilities|Array|MakeArray (Variables|Default|GetBarrel_B) (Variables|Default|GetScope_M) (Variables|Default|GetAmmo_M)))
  (|CallParentFunction))

(fn ConstructionScript
  (|CallParentFunction))

(fn ShootProjectile
  (params (ArrowComponent :type Arrow%20Component%20Object%20Reference))
  (|CallParentFunction ArrowComponent)
  (CallFunction|SetNewArrow))

(fn SetNewArrow
  (bind _arrowarray (Variables|Default|GetArrowArray))
  (bind _returnvalue (Utilities|Array|Length _arrowarray))
  ;[1 1 1] If projectile was show change the arrow component and increase the index
  (if (== _returnvalue 0)
    _
    (else
      (Variables|Default|SetMainArrowComponent (Utilities|Array|Get(acopy) (Variables|Default|GetArrowArray) (Math|Integer|%(Integer) (Variables|NewArrow|GetArrowIndex) _returnvalue)))))
  (Math|Integer|IncrementInt (Variables|NewArrow|GetArrowIndex)))

(fn AttackspeedPerXLevel
  (return 0.07))

(fn DamagePerLevel
  (return 0.5))

(fn RangePerXLevel
  (return 2e+02))

(fn GetTurretCosts
  (return 1e+02))

(fn Lvl10MeshChange
  (return (Utilities|Array|MakeArray (Variables|Default|GetBase_B)) (Utilities|Array|MakeArray "/Game/Characters/NPC/Turrets/Meshes/SM_Turrets_Cannon_Cannon_2_Base.SM_Turrets_Cannon_Cannon_2_Base")))

(fn Lvl20MeshChange
  (return (Utilities|Array|MakeArray (Variables|Default|GetYaw_B)) (Utilities|Array|MakeArray "/Game/Characters/NPC/Turrets/Meshes/SM_Turrets_Cannon_Cannon_2_Yaw.SM_Turrets_Cannon_Cannon_2_Yaw")))

(fn Lvl30MeshChange
  (return (Utilities|Array|MakeArray (Variables|Default|GetBarrel_B) (Variables|Default|GetPitch_B)) (Utilities|Array|MakeArray "/Game/Characters/NPC/Turrets/Meshes/SM_Turrets_Cannon_Cannon_2_Barrel.SM_Turrets_Cannon_Cannon_2_Barrel" "/Game/Characters/NPC/Turrets/Meshes/SM_Turrets_Cannon_Cannon_2_Pitch.SM_Turrets_Cannon_Cannon_2_Pitch")))

(fn Lvl40MeshChange
  (return (Utilities|Array|MakeArray (Variables|Default|GetAmmo_M)) (Utilities|Array|MakeArray "/Game/Characters/NPC/Turrets/Meshes/SM_Turrets_Cannon_Cannon_2_Ammo.SM_Turrets_Cannon_Cannon_2_Ammo")))

(fn Lvl60MeshChange
  (return (Utilities|Array|MakeArray (Variables|Default|GetScope_M)) (Utilities|Array|MakeArray "/Game/Characters/NPC/Turrets/Meshes/SM_Turrets_Cannon_Cannon_2_Scope.SM_Turrets_Cannon_Cannon_2_Scope")))

(fn Lvl70MeshChange
  (return (Utilities|Array|MakeArray (Variables|Default|GetBase_B)) (Utilities|Array|MakeArray "/Game/Characters/NPC/Turrets/Meshes/SM_Turrets_Cannon_Cannon_3_Base.SM_Turrets_Cannon_Cannon_3_Base")))

(fn Lvl80MeshChange
  (return (Utilities|Array|MakeArray (Variables|Default|GetYaw_B)) (Utilities|Array|MakeArray "/Game/Characters/NPC/Turrets/Meshes/SM_Turrets_Cannon_Cannon_3_Yaw.SM_Turrets_Cannon_Cannon_3_Yaw")))

(fn Lvl90MeshChange
  (return (Utilities|Array|MakeArray (Variables|Default|GetBarrel_B) (Variables|Default|GetPitch_B)) (Utilities|Array|MakeArray "/Game/Characters/NPC/Turrets/Meshes/SM_Turrets_Cannon_Cannon_3_Barrel.SM_Turrets_Cannon_Cannon_3_Barrel" "/Game/Characters/NPC/Turrets/Meshes/SM_Turrets_Cannon_Cannon_3_Pitch.SM_Turrets_Cannon_Cannon_3_Pitch")))

(fn Lvl100MeshChange
  (return (Utilities|Array|MakeArray (Variables|Default|GetAmmo_M)) (Utilities|Array|MakeArray "/Game/Characters/NPC/Turrets/Meshes/SM_Turrets_Cannon_Cannon_3_Ammo.SM_Turrets_Cannon_Cannon_3_Ammo")))

(fn Lvl120MeshChange
  (return (Utilities|Array|MakeArray (Variables|Default|GetScope_M)) (Utilities|Array|MakeArray "/Game/Characters/NPC/Turrets/Meshes/SM_Turrets_Cannon_Cannon_3_Scope.SM_Turrets_Cannon_Cannon_3_Scope")))

(fn AddShootstoDataCollector
  (params (TowerShots :type Integer))
  (bind _datacollector (CallFunction|GetDataCollector))
  (bind _totalcannonshots (Default|AddCannonShots _datacollector TowerShots))
  (return _totalcannonshots _datacollector))

(fn AddTimesUpgradestoDataCollector
  (params (AmountUpgraded :type Integer))
  (bind _datacollector (CallFunction|GetDataCollector))
  (bind _totalcannonupgrades (Default|AddCannonUpgrade _datacollector AmountUpgraded))
  (return _totalcannonupgrades _datacollector))