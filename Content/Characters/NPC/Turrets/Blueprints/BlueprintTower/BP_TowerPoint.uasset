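; BP_TowerPoint is a turret build slot that spawns, tracks and removes a single turret at its spawn position.
; On BeginPlay it creates placement and upgrade widgets that reference it as owner.
; OpenUI shows the upgrade widget and current range if a valid turret exists, otherwise the placement widget; CloseUI removes the widget and hides the range.
; Range display scales an indicator component from the turret's radius or a supplied value.
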(event EventBeginPlay
  ;[1 1 1] Create and save UI to show when Player interacts with it
  (bind _returnvalue (UserInterface|CreateWidget "/Game/UI/UI_Blueprints/TurretPlacementOptionsBlueprint.TurretPlacementOptionsBlueprint_C"))
  (bind _output_get (Variables|Default|SetNewTowerWidget _returnvalue))
  (Variables|/Game/UI/UI_Blueprints/TurretPlacementOptionsBlueprint.TurretPlacementOptionsBlueprint_C|SetTowerPointOwner _output_get self)
  (bind _returnvalue_2 (UserInterface|CreateWidget "/Game/UI/UI_Blueprints/TurretUIBlueprint.TurretUIBlueprint_C"))
  (bind _output_get_2 (Variables|Default|SetUpgradeTowerWidget _returnvalue_2))
  (Variables|/Game/UI/UI_Blueprints/TurretUIBlueprint.TurretUIBlueprint_C|SetTowerPointOwner _output_get_2 self))

(event Collision|EventActorBeginOverlap
  (params (OtherActor :type Actor%20Object%20Reference)))

(event EventTick
  (params (DeltaSeconds :type Float%20%28single-precision%29)))

(fn ConstructionScript)

(fn SpawnTower
  (params (Tower :type BP%20Base%20Tower%20Class%20Reference))
  ;[1 1 1] Turret has no AI Class so we can simply spawn the actor itself
  (bind _returnvalue (Game|SpawnActorfromClass Tower (Math|Transform|MakeTransform (Transformation|GetWorldLocation (Variables|Default|GetSpawnPosition)) "0, 0, 0" "1,1,1") "Undefined" self 0))
  (Variables|Default|SetTurret _returnvalue))

(fn InUse
  (return (Utilities|IsValid (Variables|Default|GetTurret))))

(fn RemoveTower
  (Actor|DestroyActor (Variables|Default|GetTurret))
  (return))

(fn OpenUI
  (bind _newtowerwidget (Variables|Default|GetNewTowerWidget))
  (bind _upgradetowerwidget (Variables|Default|GetUpgradeTowerWidget))
  (if (CallFunction|InUse)
    (UserInterface|Viewport|AddtoViewport _upgradetowerwidget 0)
    (RangeIndicator|ShowCurrentTowerRange)
    (Variables|Default|SetCurrentUI _upgradetowerwidget)
    (else
      (UserInterface|Viewport|AddtoViewport _newtowerwidget 0)
      (Variables|Default|SetCurrentUI _newtowerwidget))))

(fn CloseUI
  (RangeIndicator|HideTowerRange)
  (Widget|RemovefromParent (Variables|Default|GetCurrentUI)))

(fn ShowTowerRange
  (params (Tower :type BP%20Base%20Tower%20Object%20Reference))
  (bind _radius (Variables|/Game/Characters/NPC/Turrets/Blueprints/BlueprintTower/BP_BaseTower.BP_BaseTower_C|GetRadius Tower))
  (bind _returnvalue (/ _radius 1e+02))
  (Utilities|IsValid Tower
    (:Is%20Valid
      (Transformation|SetWorldScale3D (Variables|Default|GetRangeIndicator) (Math|Vector|MakeVector _returnvalue _returnvalue _returnvalue))
      (Variables|Default|SetRangeVisible true)
      (return true))
    (:Is%20Not%20Valid
      (return false))))

(fn ShowCurrentTowerRange
  (bind _showrangesuccessful (RangeIndicator|ShowTowerRange (Variables|Default|GetTurret)))
  (return _showrangesuccessful))

(fn HideTowerRange
  (Transformation|SetWorldScale3D (Variables|Default|GetRangeIndicator) "0, 0, 0")
  (Variables|Default|SetRangeVisible false))

(fn IsRangeVisible
  (return (Variables|Default|GetRangeVisible)))

(fn ShowRange
  (params (Range :type Float%20%28single-precision%29))
  (bind _returnvalue (/ Range 1e+02))
  (Transformation|SetWorldScale3D (Variables|Default|GetRangeIndicator) (Math|Vector|MakeVector _returnvalue _returnvalue _returnvalue))
  (Variables|Default|SetRangeVisible true))