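; Base tower-defense turret that targets enemies inside its range sphere, fires projectiles at them and can be upgraded.
; Each Tick it favors the enemy farthest along the spline, line-tracing only while no candidate is set.
; Timelines lerp yaw and pitch toward the target and gate firing by reload time.
; Upgrades adjust damage, range and reload through stub functions for child towers, with mesh-swap hooks every tenth level.
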(event OnComponentBeginOverlap(RangeCollider)
  (params (OverlappedComponent :type Primitive%20Component%20Object%20Reference) (OtherActor :type Actor%20Object%20Reference) (OtherComp :type Primitive%20Component%20Object%20Reference) (OtherBodyIndex :type Integer) (bFromSweep :type Boolean) (SweepResult :type Hit%20Result%20Structure%20%28by%20ref%29))
  ;[1 1 1] If enemy steps in the sphere collider, put it in a list
  (bind _asbp_base_enemy (Utilities|Casting|CastToBP_BaseEnemy OtherActor))
  (Utilities|Array|AddUnique (Variables|EnemyList|GetEnemiesInRange) _asbp_base_enemy))

(event OnComponentEndOverlap(RangeCollider)
  (params (OverlappedComponent :type Primitive%20Component%20Object%20Reference) (OtherActor :type Actor%20Object%20Reference) (OtherComp :type Primitive%20Component%20Object%20Reference) (OtherBodyIndex :type Integer))
  ;[1 1 1] If enemy steps out of the sphere collider, remove it from the list
  (bind _asbp_base_enemy (Utilities|Casting|CastToBP_BaseEnemy OtherActor))
  (Utilities|Array|RemoveItem (Variables|EnemyList|GetEnemiesInRange) _asbp_base_enemy))

(event Custom|Shoot
  (params (Arrow :type Arrow%20Component%20Object%20Reference))
  ;[1 1 1] Shoot will be called every frame when an enemy is in range, "Do Once" reduces this. If the shoot timer is finished reset it so the Tower can shoot again.
  (Utilities|FlowControl|DoOnce false :!label _label
    (:Completed
      (Utilities|IsValid (Variables|Default|GetFocusedEnemy)
        (:Is%20Valid
          (CallFunction|ShootProjectile Arrow)
          (Timeline|ShootTimer PlayFromStart
            (:Finished
              (goto _label Reset))))
        (:Is%20Not%20Valid
          (goto _label Reset))))))

(event Custom|FocusedEnemyChanged)

(event Custom|Every10thLevel
  (bind _currentlevel (Variables|Default|GetCurrentLevel))
  (bind (_meshtochange _changeto _canchange) (MeshChange|Level|GetMeshestoChange _currentlevel))
  ;[1 1 1] This function will be called at the END of "Upgrade" Method
  (if _canchange
    (for _index (range 0 (Utilities|Array|Length _meshtochange))
      (MeshChange|ChangeMesh (Utilities|Array|Get(acopy) _meshtochange _index) (Utilities|Array|Get(acopy) _changeto _index)))))

(event Custom|LevelUp
  ;[1 1 1] Called every Upgrade. Calls bevore "Every10thLevel
)

(event EventTick
  (params (DeltaSeconds :type Float%20%28single-precision%29))
  (bind _yaw (Variables|Default|GetYaw))
  (bind _returnvalue (Transformation|GetWorldRotation _yaw))
  ;[1 1 1] Update List of enemies in range. if enemy is not valid skip this frame
  (bind (_newfocusedenemy _focuschanged_) (CallFunction|UpdateFocusedEnemy))
  (Utilities|IsValid _newfocusedenemy
    (:Is%20Valid
      (bind (_rotation _reachable) (CallFunction|GetRotationtoFocusedEnemy))
      (if _reachable
        (if _focuschanged_
          (Variables|Default|SetTmpRotation (Math|Rotator|MakeRotator (.roll _returnvalue) (.pitch (Transformation|GetWorldRotation (Variables|Default|GetPitch))) (.yaw _returnvalue)))
          ;[1 1 1] Rotate to Enemy. When rotation is finished shoot
          (bind _rotationtime (Timeline|RotationTimer PlayFromStart)
            (:Update
              (Transformation|SetWorldRotation (Variables|Default|GetYaw) (Math|Rotator|MakeRotator (.roll (Math|Rotator|Lerp(Rotator) (Variables|Default|GetTmpRotation) _rotation _rotationtime)) 0.0 (.yaw (Math|Rotator|Lerp(Rotator) (Variables|Default|GetTmpRotation) _rotation _rotationtime))) false false)
              (Transformation|SetWorldRotation (Variables|Default|GetPitch) (Math|Rotator|MakeRotator (.roll (Math|Rotator|Lerp(Rotator) (Variables|Default|GetTmpRotation) _rotation _rotationtime)) (.pitch (Math|Rotator|Lerp(Rotator) (Variables|Default|GetTmpRotation) _rotation _rotationtime)) (.yaw (Math|Rotator|Lerp(Rotator) (Variables|Default|GetTmpRotation) _rotation _rotationtime))) false false))
            (:Finished
              (CallFunction|Shoot (Variables|Default|GetMainArrowComponent))))
          (else
            (Timeline|RotationTimer Play)))))))

(event EventBeginPlay
  ;[1 1 1] Set play rate of shoot timer.
  (Upgrade|SetShotTimer (Variables|Default|GetReloadTime))
  ;[1 1 1] Set play rate of rotarion speed.
  (Components|Timeline|SetPlayRate (Variables|Default|GetRotationTimer) (/ 1.0 (Variables|Default|GetRotateSpeed))))

(fn ConstructionScript
  (Components|Sphere|SetSphereRadius (Variables|Default|GetRangeCollider) (Variables|Default|GetRadius) true))

(fn UpdateFocusedEnemy
  (Utilities|Array|Clear (Variables|EnemyList|GetEnemiesInSight))
  (for _array_element (Variables|EnemyList|GetEnemiesInRange)
    ;[1 1 1] Check if temp enemy is set.
    (Utilities|IsValid (LocalVariables|GetTmpEnemy)
      (:Is%20Valid
        ;[1 1 1] If the Enemy is nearer at Goal then the saved enemy overwrite variable
        (if (> (Default|GetDistanceOverSpline _array_element) (Default|GetDistanceOverSpline (LocalVariables|GetTmpEnemy)))
          (LocalVariables|SetTmpEnemy _array_element)))
      (:Is%20Not%20Valid
        ;[1 1 1] If Enemy is in sight, add to list
        (if (.InSight (CallFunction|IsEnemyinSight (Variables|Default|GetArrow) _array_element))
          (Utilities|Array|Add (Variables|EnemyList|GetEnemiesInSight) (.EnemyChecked (CallFunction|IsEnemyinSight (Variables|Default|GetArrow) _array_element)))
          (LocalVariables|SetTmpEnemy (.EnemyChecked (CallFunction|IsEnemyinSight (Variables|Default|GetArrow) _array_element)))))))
  ;[1 1 1] Check if a new enemy got focused
  (if (== (LocalVariables|GetTmpEnemy) (Variables|Default|GetFocusedEnemy))
    (bind _output_get (Variables|Default|SetFocusedEnemy (LocalVariables|GetTmpEnemy)))
    (return _output_get false)
    (else
      (bind _output_get_2 (Variables|Default|SetFocusedEnemy (LocalVariables|GetTmpEnemy)))
      (CallFunction|FocusedEnemyChanged)
      (return _output_get_2 true))))

(fn GetRotationtoFocusedEnemy
  (bind _focusedenemy (Variables|Default|GetFocusedEnemy))
  (bind _arrowcomponent (Variables|Default|GetArrowComponent))
  (bind _returnvalue (Transformation|GetActorLocation _focusedenemy))
  (bind _returnvalue_2 (Transformation|GetWorldLocation _arrowcomponent))
  (bind _returnvalue_3 (Math|Rotator|FindLookatRotation _returnvalue_2 _returnvalue))
  (return (Math|Rotator|MakeRotator (.roll (Transformation|GetWorldRotation (Variables|Default|GetYaw))) (.pitch _returnvalue_3) (.yaw _returnvalue_3)) true))

(fn ShootProjectile
  (params (ArrowComponent :type Arrow%20Component%20Object%20Reference))
  (bind _returnvalue (Transformation|GetWorldTransform ArrowComponent))
  (bind _focusedenemy (Variables|Default|GetFocusedEnemy))
  ;[1 1 1] Spawn Projectile at Location from Arrow (which should be in front of the cannon
  (bind _returnvalue_2 (Game|SpawnActorfromClass (Variables|Default|GetProjectile) (Math|Transform|MakeTransform (.location _returnvalue) (.rotation _returnvalue) "0.500000,0.500000,0.500000") "AlwaysSpawn" 0 0))
  ;[1 1 1] Set Damage and Speed of Projectile
  (Utilities|IsValid _returnvalue_2
    (:Is%20Valid
      (Variables|/Game/Characters/NPC/Turrets/Blueprints/BlueprintProjectile/BP_BaseProjectile.BP_BaseProjectile_C|SetDamage _returnvalue_2 (Variables|Default|GetDamage))
      (Class|FMODBlueprintStatics|PlayEventatLocation (Variables|Default|GetShootSound) (Math|Conversions|ToTransform(Vector) (.location _returnvalue)))
      (Utilities|IsValid _focusedenemy
        (:Is%20Valid
          (Variables|/Game/Characters/NPC/Turrets/Blueprints/BlueprintProjectile/BP_BaseProjectile.BP_BaseProjectile_C|SetTargetedEnemy _returnvalue_2 _focusedenemy)
          (return _returnvalue_2))))))

(fn Upgrade
  ;[1 1 1] Set Damage
  (bind _output_get (Variables|Default|SetCurrentLevel (+ (Variables|Default|GetCurrentLevel) 1)))
  (Variables|Default|SetDamage (/ (Math|Conversions|ToFloat(Integer) (Math|Float|Floor (* (+ (LevelandDamage|CalculateDeltaDamage _output_get) (Variables|Default|GetDamage)) 1e+02))) 1e+02))
  ;[1 1 1] Set Range
  (Upgrade|SetRange (+ (Variables|Default|GetRadius) (LevelandRange|CalculateDeltaRange (Variables|Default|GetCurrentLevel))))
  (Upgrade|SetAttackspeed (- (Variables|Default|GetReloadTime) (LevelandAttackspeed|CalculateDeltaAttackspeed (Variables|Default|GetCurrentLevel))))
  (Development|PrintString (Utilities|String|Append "New Level: " (Utilities|String|ToString(Integer) (Variables|Default|GetCurrentLevel))))
  ;[1 1 1] Every 10th level Event is called
  (CallFunction|LevelUp)
  (if (== (Math|Integer|%(Integer) (Variables|Default|GetCurrentLevel) 10) 0)
    (CallFunction|Every10thLevel))
  (return))

(fn SetShotTimer
  (params (Reload%20Time :type Float%20%28single-precision%29))
  (bind _output_get (Variables|Default|SetReloadTime Reload%20Time))
  (Components|Timeline|SetPlayRate (Variables|Default|GetShootTimer) (/ 1.0 _output_get))
  (return (/ 1.0 _output_get)))

(fn CalculateDeltaCost
  (params (NextLevel :type Integer))
  (return (Math|Float|Truncate (* (* (+ (/ (* (Variables|Default|GetDamage) (LocalVariables|Getb)) (* (Variables|Default|GetReloadTime) (LocalVariables|Getc))) (* (LocalVariables|Getd) (/ (Variables|Default|GetRadius) 1e+02))) (* (Math|Float|Power (LocalVariables|Gete) (Math|Conversions|ToFloat(Integer) NextLevel)) (LocalVariables|Getf))) (LocalVariables|Geta)))))

(fn CalculateDeltaDamage
  (params (NextLevel :type Integer))
  (return (LevelandDamage|DamagePerLevel)))

(fn CalculateDamage
  (params (Level :type Integer))
  (return (+ (* Level (LevelandDamage|DamagePerLevel)) (Variables|Default|GetBaseDamage))))

(fn CalculateNextLevelDamage
  (return (/ (Math|Conversions|ToFloat(Integer) (Math|Float|Floor (* (+ (+ (LevelandDamage|CalculateDeltaDamage (LevelandDamage|GetNextLevel)) (Variables|Default|GetDamage)) (Variables|Default|GetDamage)) 1e+02))) 1e+02)))

(fn GetCurrentLevel
  (return (Variables|Default|GetCurrentLevel)))

(fn GetNextLevel
  (return (+ (LevelandDamage|GetCurrentLevel) 1)))

(fn ShowRange
  (Development|SetHiddeninGame (Variables|Default|GetRangeCollider) false false)
  (return))

(fn HideRange
  (Development|SetHiddeninGame (Variables|Default|GetRangeCollider) true false)
  (return))

(fn SetRange
  (params (NewRange :type Float%20%28single-precision%29))
  (bind _output_get (Variables|Default|SetRadius NewRange))
  (Components|Sphere|SetSphereRadius (Variables|Default|GetRangeCollider) _output_get true)
  (return NewRange))

(fn DamagePerLevel
  (return 0.0))

(fn RangePerXLevel
  (return 0.0))

(fn CanIncreaseRange
  (params (Level :type Integer))
  (return (== (Math|Integer|%(Integer) Level (LocalVariables|GetEveryXLevel)) 0)))

(fn CalculateDeltaRange
  (params (NextLevel :type Integer))
  ;[1 1 1] Checks if Range can be upgraded next level
  (if (LevelandRange|CanIncreaseRange NextLevel)
    (return (LevelandRange|RangePerXLevel))
    (else
      (return 0.0))))

(fn AttackspeedPerXLevel
  (return 0.0))

(fn CanIncreaseAttackspeed
  (params (Level :type Integer))
  (return (== (Math|Integer|%(Integer) Level (LocalVariables|GetEveryXLevel)) 0)))

(fn CalculateDeltaAttackspeed
  (params (NextLevel :type Integer))
  (if (LevelandAttackspeed|CanIncreaseAttackspeed NextLevel)
    (return (LevelandAttackspeed|AttackspeedPerXLevel))
    (else
      (return 0.0))))

(fn SetAttackspeed
  (params (NewAttackspeed :type Float%20%28single-precision%29))
  (bind _output_get (Variables|Default|SetReloadTime NewAttackspeed))
  (Upgrade|SetShotTimer _output_get)
  (return NewAttackspeed))

(fn ChangeMesh
  (params (MeshToChange :type Static%20Mesh%20Component%20Object%20Reference) (NewMesh :type Static%20Mesh%20Object%20Reference))
  (bind _returnvalue (Components|StaticMesh|SetStaticMesh MeshToChange NewMesh))
  (return _returnvalue))

(fn GetTurretCosts
  (return 0.0))

(fn Lvl10MeshChange
  (return 0 0))

(fn Lvl20MeshChange
  (return 0 0))

(fn Lvl30MeshChange
  (return 0 0))

(fn Lvl40MeshChange
  (return 0 0))

(fn Lvl50MeshChange
  (return 0 0))

(fn Lvl60MeshChange
  (return 0 0))

(fn Lvl70MeshChange
  (return 0 0))

(fn Lvl80MeshChange
  (return 0 0))

(fn Lvl90MeshChange
  (return 0 0))

(fn Lvl100MeshChange
  (return 0 0))

(fn Lvl110MeshChange
  (return 0 0))

(fn Lvl120MeshChange
  (return 0 0))

(fn Lvl130MeshChange
  (return 0 0))

(fn Lvl140MeshChange
  (return 0 0))

(fn Lvl150MeshChange
  (return 0 0))

(fn GetMeshestoChange
  (params (Level :type Integer))
  (bind (_meshtochange _changeto) (MeshChange|Level|Lvl90MeshChange))
  (bind (_meshtochange_2 _changeto_2) (MeshChange|Level|Lvl100MeshChange))
  (bind (_meshtochange_3 _changeto_3) (MeshChange|Level|Lvl110MeshChange))
  (bind (_meshtochange_4 _changeto_4) (MeshChange|Level|Lvl120MeshChange))
  (bind (_meshtochange_5 _changeto_5) (MeshChange|Level|Lvl130MeshChange))
  (bind (_meshtochange_6 _changeto_6) (MeshChange|Level|Lvl140MeshChange))
  (bind (_meshtochange_7 _changeto_7) (MeshChange|Level|Lvl150MeshChange))
  (bind (_meshtochange_8 _changeto_8) (MeshChange|Level|Lvl10MeshChange))
  (bind (_meshtochange_9 _changeto_9) (MeshChange|Level|Lvl20MeshChange))
  (bind (_meshtochange_10 _changeto_10) (MeshChange|Level|Lvl30MeshChange))
  (bind (_meshtochange_11 _changeto_11) (MeshChange|Level|Lvl40MeshChange))
  (bind (_meshtochange_12 _changeto_12) (MeshChange|Level|Lvl50MeshChange))
  (bind (_meshtochange_13 _changeto_13) (MeshChange|Level|Lvl60MeshChange))
  (bind (_meshtochange_14 _changeto_14) (MeshChange|Level|Lvl70MeshChange))
  (bind (_meshtochange_15 _changeto_15) (MeshChange|Level|Lvl80MeshChange))
  ;[1 1 1] Do and return nothing if level is not 10th step
  (if (== (Math|Integer|%(Integer) Level 10) 0)
    (switch int (/ Level 10)
      (:Default
        (return 0 0 false))
      (:0
        (return 0 0 false))
      (:1
        (return _meshtochange_8 _changeto_8 true))
      (:2
        (return _meshtochange_9 _changeto_9 true))
      (:3
        (return _meshtochange_10 _changeto_10 true))
      (:4
        (return _meshtochange_11 _changeto_11 true))
      (:5
        (return _meshtochange_12 _changeto_12 true))
      (:6
        (return _meshtochange_13 _changeto_13 true))
      (:7
        (return _meshtochange_14 _changeto_14 true))
      (:8
        (return _meshtochange_15 _changeto_15 true))
      (:9
        (return _meshtochange _changeto true))
      (:10
        (return _meshtochange_2 _changeto_2 true))
      (:11
        (return _meshtochange_3 _changeto_3 true))
      (:12
        (return _meshtochange_4 _changeto_4 true))
      (:13
        (return _meshtochange_5 _changeto_5 true))
      (:14
        (return _meshtochange_6 _changeto_6 true))
      (:15
        (return _meshtochange_7 _changeto_7 true)))
    (else
      (return 0 0 false))))

(fn IsEnemyinSight
  (params (Start :type Arrow%20Component%20Object%20Reference) (Enemy :type BP%20Base%20Enemy%20Object%20Reference))
  ;[1 1 1] Line Trace from Arrow to Enemy and ignore all enemies. If nothing got hit enemy is in sight
  (bind _returnvalue (Collision|LineTraceByChannel (Transformation|GetWorldLocation Start) (Transformation|GetActorLocation Enemy) "TraceTypeQuery3" false 0 "ForOneFrame" true "(R=0.000000,G=1.000000,B=0.000000,A=1.000000)" "(R=1.000000,G=0.000000,B=0.000000,A=1.000000)" 0.1))
  (return (not _returnvalue) Enemy))

(fn GetTowerPoint
  (bind _asbp_tower_point (Utilities|Casting|CastToBP_TowerPoint (Components|GetOwner))
    (:then
      (return _asbp_tower_point true))
    (:CastFailed
      (return 0 false))))