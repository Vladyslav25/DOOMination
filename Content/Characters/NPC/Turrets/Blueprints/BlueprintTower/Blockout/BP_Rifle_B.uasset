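; Rifle turret child Blueprint that sets its stats, cost, per-level gains and projectile for the parent tower class.
; ShootProjectile calls the parent, then plays a barrel recoil timeline that adds per-frame offset deltas rather than setting position.
; The timeline's play rate follows ReloadTime, refreshed on attack speed changes.
; Every10thLevel swaps one part mesh per milestone, progressing through Rifle_2 and then Rifle_3 models.
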(event Custom|ShotAnimation
  ;[1 1 1] Reset Last Value
  (Variables|Components|SetAnimationLastValue 0.0)
  (bind _barrel_b_local_x_coordinate (Timeline|Shoot%20Animation PlayFromStart)
    (:Update
      ;[1 1 1] Subtract the Value last frame from the current value to get the difference, because we ADD local and not SET
      (Transformation|AddLocalOffset (Variables|Default|GetBarrel_B) (Math|Vector|MakeVector (- _barrel_b_local_x_coordinate (Variables|Components|GetAnimationLastValue)) 0.0 0.0) false false)
      (Variables|Components|SetAnimationLastValue _barrel_b_local_x_coordinate))))

(event EventBeginPlay
  (|CallParentFunction)
  (Variables|Default|SetMainArrowComponent (Variables|Default|GetArrow))
  (Variables|Default|SetProjectile "/Game/Characters/NPC/Turrets/Blueprints/BlueprintProjectile/BP_RifleProjectile.BP_RifleProjectile_C")
  ;[1 1 1] Set play rate of shoot Animation.
  (Components|Timeline|SetPlayRate (Variables|Default|GetShoot%20Animation) (/ 1.0 (Variables|Default|GetReloadTime))))

(event Collision|EventActorBeginOverlap
  (params (OtherActor :type Actor%20Object%20Reference)))

(event EventTick
  (params (DeltaSeconds :type Float%20%28single-precision%29))
  (|CallParentFunction DeltaSeconds) ; This node is disabled and will not be called.\nDrag off pins to build functionality.
)

(event EventEvery10thLevel
  (switch int (/ (CallFunction|GetCurrentLevel) 10)
    (:1
      (Components|StaticMesh|SetStaticMesh (Variables|Default|GetBase_B) "/Game/Characters/NPC/Turrets/Meshes/SM_Turrets_Rifle_Rifle_2_Base.SM_Turrets_Rifle_Rifle_2_Base"))
    (:2
      (Components|StaticMesh|SetStaticMesh (Variables|Default|GetYaw_B) "/Game/Characters/NPC/Turrets/Meshes/SM_Turrets_Rifle_Rifle_2_Yaw.SM_Turrets_Rifle_Rifle_2_Yaw"))
    (:3
      (Components|StaticMesh|SetStaticMesh (Variables|Default|GetSpring_M) "/Game/Characters/NPC/Turrets/Meshes/SM_Turrets_Rifle_Rifle_2_Spring.SM_Turrets_Rifle_Rifle_2_Spring"))
    (:4
      (Components|StaticMesh|SetStaticMesh (Variables|Default|GetBack_M) "/Game/Characters/NPC/Turrets/Meshes/SM_Turrets_Rifle_Rifle_2_Back.SM_Turrets_Rifle_Rifle_2_Back"))
    (:5
      (Components|StaticMesh|SetStaticMesh (Variables|Default|GetScope_M) "/Game/Characters/NPC/Turrets/Meshes/SM_Turrets_Rifle_Rifle_2_Scope.SM_Turrets_Rifle_Rifle_2_Scope"))
    (:6
      (Components|StaticMesh|SetStaticMesh (Variables|Default|GetBarrel_B) "/Game/Characters/NPC/Turrets/Meshes/SM_Turrets_Rifle_Rifle_2_Barrel.SM_Turrets_Rifle_Rifle_2_Barrel"))
    (:7
      (Components|StaticMesh|SetStaticMesh (Variables|Default|GetPitch_B) "/Game/Characters/NPC/Turrets/Meshes/SM_Turrets_Rifle_Rifle_2_Pitch.SM_Turrets_Rifle_Rifle_2_Pitch"))
    (:8
      (Components|StaticMesh|SetStaticMesh (Variables|Default|GetBase_B) "/Game/Characters/NPC/Turrets/Meshes/SM_Turrets_Rifle_Rifle_3_Base.SM_Turrets_Rifle_Rifle_3_Base"))
    (:9
      (Components|StaticMesh|SetStaticMesh (Variables|Default|GetYaw_B) "/Game/Characters/NPC/Turrets/Meshes/SM_Turrets_Rifle_Rifle_3_Yaw.SM_Turrets_Rifle_Rifle_3_Yaw"))
    (:10
      (Components|StaticMesh|SetStaticMesh (Variables|Default|GetSpring_M) "/Game/Characters/NPC/Turrets/Meshes/SM_Turrets_Rifle_Rifle_3_Spring.SM_Turrets_Rifle_Rifle_3_Spring"))
    (:11
      (Components|StaticMesh|SetStaticMesh (Variables|Default|GetBack_M) "/Game/Characters/NPC/Turrets/Meshes/SM_Turrets_Rifle_Rifle_3_Back.SM_Turrets_Rifle_Rifle_3_Back"))
    (:12
      (Components|StaticMesh|SetStaticMesh (Variables|Default|GetScope_M) "/Game/Characters/NPC/Turrets/Meshes/SM_Turrets_Rifle_Rifle_3_Scope.SM_Turrets_Rifle_Rifle_3_Scope"))
    (:13
      (Components|StaticMesh|SetStaticMesh (Variables|Default|GetBarrel_B) "/Game/Characters/NPC/Turrets/Meshes/SM_Turrets_Rifle_Rifle_3_Barrel.SM_Turrets_Rifle_Rifle_3_Barrel"))
    (:14
      (Components|StaticMesh|SetStaticMesh (Variables|Default|GetPitch_B) "/Game/Characters/NPC/Turrets/Meshes/SM_Turrets_Rifle_Rifle_3_Pitch.SM_Turrets_Rifle_Rifle_3_Pitch"))))

(fn ConstructionScript
  (Variables|Default|SetRadius 2.5e+03)
  (|CallParentFunction)
  (Variables|Default|SetRotateSpeed 0.5)
  (Variables|Default|SetReloadTime 0.9)
  (Variables|Default|SetDamage 18.0)
  (Variables|Default|SetBaseDamage 18.0))

(fn ShootProjectile
  (params (ArrowComponent :type Arrow%20Component%20Object%20Reference))
  ;[1 1 1] Shoot Projectile and play Animation
  (bind _shotprojectile (|CallParentFunction ArrowComponent))
  (CallFunction|ShotAnimation)
  (return _shotprojectile))

(fn DamagePerLevel
  (return 1.0))

(fn RangePerXLevel
  (return 4e+02))

(fn AttackspeedPerXLevel
  (return 0.11))

(fn GetTurretCosts
  (return 114.0))

(fn SetAttackspeed
  (params (NewAttackspeed :type Float%20%28single-precision%29))
  (bind _attackspeed (|CallParentFunction NewAttackspeed))
  (Components|Timeline|SetPlayRate (Variables|Default|GetShoot%20Animation) (/ 1.0 (Variables|Default|GetReloadTime)))
  (return _attackspeed))