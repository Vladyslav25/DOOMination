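; Laser turret tower, a child of a shared turret base, that deals rapid instant damage to its focused enemy.
; ShootProjectile skips spawning a projectile and calls DoDamage, drawing the beam as a debug line and applying damage directly.
; A damage multiplier grows over time on Tick and resets when the target changes.
; It also overrides base stats, upgrade scaling and cost, and swaps base meshes at level milestones.
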(event EventBeginPlay
  (|CallParentFunction)
  (Variables|Default|SetMainArrowComponent (Variables|Default|GetArrow))
  (Variables|Default|SetProjectile "/Game/Characters/NPC/Turrets/Blueprints/BlueprintProjectile/BP_LaserProjectile.BP_LaserProjectile_C"))

(event Collision|EventActorBeginOverlap
  (params (OtherActor :type Actor%20Object%20Reference)))

(event EventTick
  (params (DeltaSeconds :type Float%20%28single-precision%29))
  (|CallParentFunction DeltaSeconds)
  (Variables|Default|SetCurrentDamageMultiplier (+ (Variables|Default|GetCurrentDamageMultiplier) (* DeltaSeconds (Variables|Default|GetDamageMultiplyPerSecond)))))

(event EventFocusedEnemyChanged
  ;[1 1 1] Reset Damage Multiplier when Enemy is changed
  (Variables|Default|SetCurrentDamageMultiplier 1.0))

(event EventEvery10thLevel
  (switch int (Math|Integer|%(Integer) (CallFunction|GetCurrentLevel) 10)
    (:1
      (Components|StaticMesh|SetStaticMesh (Variables|Default|GetBase_B) "/Game/Characters/NPC/Turrets/Meshes/SM_Turrets_Laser_Laser_2_Base.SM_Turrets_Laser_Laser_2_Base"))
    (:4
      (Components|StaticMesh|SetStaticMesh (Variables|Default|GetBase_B) "/Game/Characters/NPC/Turrets/Meshes/SM_Turrets_Laser_Laser_3_Base.SM_Turrets_Laser_Laser_3_Base"))))

(fn ConstructionScript
  (Variables|Default|SetRadius 2.5e+03)
  (|CallParentFunction)
  (Variables|Default|SetDamageMultiplyPerSecond 0.3)
  (Variables|Default|SetRotateSpeed 0.5)
  (Variables|Default|SetReloadTime 0.1)
  (Variables|Default|SetDamage 2.0))

(fn ShootProjectile
  (params (ArrowComponent :type Arrow%20Component%20Object%20Reference))
  (CallFunction|DoDamage)
  (return 0))

(fn DoDamage
  (bind _focusedenemy (Variables|Default|GetFocusedEnemy))
  (bind _focusedenemy_2 (Variables|Default|GetFocusedEnemy))
  (bind _rootcomponent (Variables|/Script/Engine.Actor|GetRootComponent _focusedenemy))
  (bind _returnvalue (Transformation|GetWorldLocation _rootcomponent))
  (Rendering|Debug|DrawDebugLine (Transformation|GetWorldLocation (Variables|Default|GetArrow)) (Math|Vector|MakeVector (.x _returnvalue) (.y _returnvalue) (+ (.z _returnvalue) (/ (.z (.BoxExtent (Collision|GetComponentBounds (Variables|/Script/Engine.Character|GetMesh _focusedenemy)))) 2.0))) "(R=0.000000,G=0.761148,B=1.000000,A=1.000000)" (Variables|Default|GetReloadTime) 5e+01)
  (Utilities|IsValid _focusedenemy_2
    (:Is%20Valid
      (Game|Damage|ApplyDamage _focusedenemy_2 (* (Variables|Default|GetDamage) (Variables|Default|GetCurrentDamageMultiplier)) 0 self "/Game/Characters/NPC/Turrets/Blueprints/BP_TowerDamagaType.BP_TowerDamagaType_C"))))

(fn DamagePerLevel
  (return 0.25))

(fn RangePerXLevel
  (return 4e+02))

(fn AttackspeedPerXLevel
  (return 0.0))

(fn GetTurretCosts
  (return 1.4e+02))