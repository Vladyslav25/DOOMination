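; Rocket launcher turret, a child tower that sets its own stats, cost and per-level scaling and fires BP_RocketLauncherProjectile with an area-of-effect radius.
; It overrides aiming with a ballistic solve for the lower-arc pitch toward the focused enemy, reporting the target unreachable when no solution exists.
; Every tenth level swaps one mesh part, progressing through the second and third visual tiers.
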(event EventBeginPlay
  (|CallParentFunction)
  (Variables|Default|SetMainArrowComponent (Variables|Default|GetArrow))
  (Variables|Default|SetProjectile "/Game/Characters/NPC/Turrets/Blueprints/BlueprintProjectile/BP_RocketLauncherProjectile.BP_RocketLauncherProjectile_C"))

(event Collision|EventActorBeginOverlap
  (params (OtherActor :type Actor%20Object%20Reference)))

(event EventTick
  (params (DeltaSeconds :type Float%20%28single-precision%29))
  (|CallParentFunction DeltaSeconds) ; This node is disabled and will not be called.\nDrag off pins to build functionality.
)

(event EventEvery10thLevel
  (switch int (/ (CallFunction|GetCurrentLevel) 10)
    (:1
      (Components|StaticMesh|SetStaticMesh (Variables|Default|GetBase_B) "/Game/Characters/NPC/Turrets/Meshes/SM_Turrets_RocketLauncher_RocketLauncher_2_Base.SM_Turrets_RocketLauncher_RocketLauncher_2_Base"))
    (:2
      (Components|StaticMesh|SetStaticMesh (Variables|Default|GetYaw_B) "/Game/Characters/NPC/Turrets/Meshes/SM_Turrets_RocketLauncher_RocketLauncher_2_Yaw.SM_Turrets_RocketLauncher_RocketLauncher_2_Yaw"))
    (:3
      (Components|StaticMesh|SetStaticMesh (Variables|Default|GetBack) "/Game/Characters/NPC/Turrets/Meshes/SM_Turrets_RocketLauncher_RocketLauncher_2_Back.SM_Turrets_RocketLauncher_RocketLauncher_2_Back"))
    (:4
      (Components|StaticMesh|SetStaticMesh (Variables|Default|GetPitch_B) "/Game/Characters/NPC/Turrets/Meshes/SM_Turrets_RocketLauncher_RocketLauncher_2_Pitch.SM_Turrets_RocketLauncher_RocketLauncher_2_Pitch"))
    (:5
      (Components|StaticMesh|SetStaticMesh (Variables|Default|GetScope) "/Game/Characters/NPC/Turrets/Meshes/SM_Turrets_RocketLauncher_RocketLauncher_2_Scope.SM_Turrets_RocketLauncher_RocketLauncher_2_Scope"))
    (:6
      (Components|StaticMesh|SetStaticMesh (Variables|Default|GetBase_B) "/Game/Characters/NPC/Turrets/Meshes/SM_Turrets_RocketLauncher_RocketLauncher_3_Base.SM_Turrets_RocketLauncher_RocketLauncher_3_Base"))
    (:7
      (Components|StaticMesh|SetStaticMesh (Variables|Default|GetYaw_B) "/Game/Characters/NPC/Turrets/Meshes/SM_Turrets_RocketLauncher_RocketLauncher_3_Yaw.SM_Turrets_RocketLauncher_RocketLauncher_3_Yaw"))
    (:8
      (Components|StaticMesh|SetStaticMesh (Variables|Default|GetBack) "/Game/Characters/NPC/Turrets/Meshes/SM_Turrets_RocketLauncher_RocketLauncher_3_Back.SM_Turrets_RocketLauncher_RocketLauncher_3_Back"))
    (:9
      (Components|StaticMesh|SetStaticMesh (Variables|Default|GetPitch_B) "/Game/Characters/NPC/Turrets/Meshes/SM_Turrets_RocketLauncher_RocketLauncher_3_Pitch.SM_Turrets_RocketLauncher_RocketLauncher_3_Pitch"))
    (:10
      (Components|StaticMesh|SetStaticMesh (Variables|Default|GetScope) "/Game/Characters/NPC/Turrets/Meshes/SM_Turrets_RocketLauncher_RocketLauncher_3_Scope.SM_Turrets_RocketLauncher_RocketLauncher_3_Scope"))))

(fn ConstructionScript
  (Variables|Default|SetRadius 3.5e+03)
  (|CallParentFunction)
  (Variables|Default|SetProjectileRadius 7.5e+02)
  (Variables|Default|SetReloadTime 1.0)
  (Variables|Default|SetRotateSpeed 0.5)
  (bind _output_get (Variables|Default|SetDamage 4.0))
  (Variables|Default|SetBaseDamage _output_get))

(fn ShootProjectile
  (params (ArrowComponent :type Arrow%20Component%20Object%20Reference))
  (bind _shotprojectile (|CallParentFunction ArrowComponent))
  (bind _asbp_rocket_launcher_projectile (Utilities|Casting|CastToBP_RocketLauncherProjectile _shotprojectile))
  (Variables|/Game/Characters/NPC/Turrets/Blueprints/BlueprintProjectile/BP_RocketLauncherProjectile.BP_RocketLauncherProjectile_C|SetAOERadius _asbp_rocket_launcher_projectile (Variables|Default|GetProjectileRadius))
  (return _asbp_rocket_launcher_projectile))

(fn GetShootAngle
  (bind _arrow (Variables|Default|GetArrow))
  (bind _focusedenemy (Variables|Default|GetFocusedEnemy))
  (bind _arrow_2 (Variables|Default|GetArrow))
  (bind _focusedenemy_2 (Variables|Default|GetFocusedEnemy))
  (bind _zoffset (LocalVariables|GetZOffset))
  (bind _velocity (LocalVariables|GetVelocity))
  (bind _gravity (LocalVariables|GetGravity))
  (bind _zoffset_2 (LocalVariables|GetZOffset))
  (bind _returnvalue (Math|Float|Square _velocity))
  (bind _returnvalue_2 (Transformation|GetWorldLocation _arrow_2))
  (bind _returnvalue_3 (Transformation|GetActorLocation _focusedenemy_2))
  (bind _returnvalue_4 (Transformation|GetWorldLocation _arrow))
  (bind _returnvalue_5 (Transformation|GetActorLocation _focusedenemy))
  (bind _returnvalue_6 (Math|Float|Square _returnvalue))
  (bind _returnvalue_7 (- (.z _returnvalue_3) _zoffset_2))
  (bind _returnvalue_8 (- (.z _returnvalue_5) _zoffset))
  (bind _returnvalue_9 (- (.x _returnvalue_5) (.x _returnvalue_4)))
  (bind _returnvalue_10 (- (.y _returnvalue_5) (.y _returnvalue_4)))
  (bind _returnvalue_11 (Math|Rotator|FindLookatRotation _returnvalue_2 (Math|Vector|MakeVector (.x _returnvalue_3) (.y _returnvalue_3) _returnvalue_7)))
  (bind _returnvalue_12 (Math|Vector2D|Vector2DLength (Math|Vector2D|MakeVector2D _returnvalue_9 _returnvalue_10)))
  (bind _returnvalue_13 (- _returnvalue_8 (.z _returnvalue_4)))
  (bind _returnvalue_14 (Math|Float|Square _returnvalue_12))
  (bind _returnvalue_15 (* _returnvalue_13 _returnvalue))
  (bind _returnvalue_16 (* _returnvalue_12 _gravity))
  (bind _returnvalue_17 (* _returnvalue_14 _gravity))
  (bind _returnvalue_18 (* _returnvalue_15 2.0))
  (bind _returnvalue_19 (+ _returnvalue_17 _returnvalue_18))
  (bind _returnvalue_20 (* _gravity _returnvalue_19))
  (bind _returnvalue_21 (- _returnvalue_6 _returnvalue_20))
  (bind _returnvalue_22 (Math|Float|Sqrt _returnvalue_21))
  (if (>= _returnvalue_21 0.0)
    (return (Math|Rotator|MakeRotator (.roll _returnvalue_11) (Math|Float|Min(Float) (Class|KismetMathLibrary|DegAtan (/ (- _returnvalue _returnvalue_22) _returnvalue_16)) (Class|KismetMathLibrary|DegAtan (/ (+ _returnvalue_22 _returnvalue) _returnvalue_16))) (.yaw _returnvalue_11)) true)
    (else
      (return "0, 0, 0" false))))

(fn GetRotationtoFocusedEnemy
  (bind (_outputrotation _reachable) (CallFunction|GetShootAngle))
  (return _outputrotation _reachable))

(fn AttackspeedPerXLevel
  (return 0.05))

(fn DamagePerLevel
  (return 0.4))

(fn RangePerXLevel
  (return 5e+02))

(fn GetTurretCosts
  (return 124.0))