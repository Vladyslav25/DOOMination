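; Rocket launcher turret, a child tower Blueprint that fires BP_RocketLauncherProjectile and passes its ProjectileRadius to each rocket as the AOE radius.
; GetShootAngle aims with the ballistic trajectory equation, taking the lower pitch solution toward the focused enemy, or zero rotation if unreachable.
; Overrides supply cost and upgrade scaling, and swap part meshes every ten levels up to 100.
; Shot and upgrade counts go to the data collector.
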(event EventBeginPlay
  (|CallParentFunction)
  (Variables|Default|SetMainArrowComponent (Variables|Default|GetArrow))
  (Variables|Default|SetProjectile "/Game/Characters/NPC/Turrets/Blueprints/BlueprintProjectile/BP_RocketLauncherProjectile.BP_RocketLauncherProjectile_C")
  (CallFunction|AddMeshes (Utilities|Array|MakeArray (Variables|Default|GetBack_M) (Variables|Default|GetScope_M))))

(event Collision|EventActorBeginOverlap
  (params (OtherActor :type Actor%20Object%20Reference)))

(event EventTick
  (params (DeltaSeconds :type Float%20%28single-precision%29))
  (|CallParentFunction DeltaSeconds) ; This node is disabled and will not be called.\nDrag off pins to build functionality.
)

(event EventOnDeleteTower
  (CallFunction|AddMeshes (Utilities|Array|MakeArray (Variables|Default|GetBack_M) (Variables|Default|GetScope_M)))
  (|CallParentFunction))

(fn ConstructionScript
  (|CallParentFunction))

(fn ShootProjectile
  (params (ArrowComponent :type Arrow%20Component%20Object%20Reference))
  (bind _shotprojectile (|CallParentFunction ArrowComponent))
  (bind _asbp_rocket_launcher_projectile (Utilities|Casting|CastToBP_RocketLauncherProjectile _shotprojectile))
  (Variables|/Game/Characters/NPC/Turrets/Blueprints/BlueprintProjectile/BP_RocketLauncherProjectile.BP_RocketLauncherProjectile_C|SetAOERadius _asbp_rocket_launcher_projectile (Variables|Default|GetProjectileRadius))
  (return _asbp_rocket_launcher_projectile))

(fn GetShootAngle
  (bind _focusedenemy (Variables|Default|GetFocusedEnemy))
  (bind _mainarrowcomponent (Variables|Default|GetMainArrowComponent))
  (bind _mainarrowcomponent_2 (Variables|Default|GetMainArrowComponent))
  (bind _focusedenemy_2 (Variables|Default|GetFocusedEnemy))
  (bind _zoffset (LocalVariables|GetZOffset))
  (bind _velocity (LocalVariables|GetVelocity))
  (bind _gravity (LocalVariables|GetGravity))
  (bind _zoffset_2 (LocalVariables|GetZOffset))
  (bind _returnvalue (Math|Float|Square _velocity))
  (bind _returnvalue_2 (Transformation|GetWorldLocation _mainarrowcomponent))
  (bind _returnvalue_3 (Transformation|GetActorLocation _focusedenemy_2))
  (bind _returnvalue_4 (Transformation|GetWorldLocation _mainarrowcomponent_2))
  (bind _returnvalue_5 (Transformation|GetActorLocation _focusedenemy))
  (bind _returnvalue_6 (Math|Float|Square _returnvalue))
  (bind _returnvalue_7 (- (.z _returnvalue_3) _zoffset_2))
  (bind _returnvalue_8 (- (.z _returnvalue_5) _zoffset))
  (bind _returnvalue_9 (- (.x _returnvalue_5) (.x _returnvalue_4)))
  (bind _returnvalue_10 (- (.y _returnvalue_5) (.y _returnvalue_4)))
  (bind _returnvalue_11 (Math|Rotator|FindLookatRotation _returnvalue_2 (Math|Vector|MakeVector (.x _returnvalue_3) (.y _returnvalue_3) _returnvalue_7)))
  (bind _returnvalue_12 (Math|Vector2D|Vector2DLength (Math|Vector2D|MakeVector2D _returnvalue_9 _returnvalue_10)))
  (bind _returnvalue_13 (- _returnvalue_8 (.z _returnvalue_4)))
  (bind _returnvalue_14 (Math|Float|Square _returnvalue_12))
  (bind _returnvalue_15 (* _returnvalue_13 _returnvalue))
  (bind _returnvalue_16 (* _returnvalue_12 _gravity))
  (bind _returnvalue_17 (* _returnvalue_14 _gravity))
  (bind _returnvalue_18 (* _returnvalue_15 2.0))
  (bind _returnvalue_19 (+ _returnvalue_17 _returnvalue_18))
  (bind _returnvalue_20 (* _gravity _returnvalue_19))
  (bind _returnvalue_21 (- _returnvalue_6 _returnvalue_20))
  (bind _returnvalue_22 (Math|Float|Sqrt _returnvalue_21))
  (if (>= _returnvalue_21 0.0)
    (return (Math|Rotator|MakeRotator (.roll _returnvalue_11) (Math|Float|Min(Float) (Class|KismetMathLibrary|DegAtan (/ (- _returnvalue _returnvalue_22) _returnvalue_16)) (Class|KismetMathLibrary|DegAtan (/ (+ _returnvalue_22 _returnvalue) _returnvalue_16))) (.yaw _returnvalue_11)))
    (else
      (return "0, 0, 0"))))

(fn GetRotationtoFocusedEnemy
  (return (CallFunction|GetShootAngle)))

(fn AttackspeedPerXLevel
  (return 0.05))

(fn DamagePerLevel
  (return 0.4))

(fn RangePerXLevel
  (return 5e+02))

(fn GetTurretCosts
  (return 124.0))

(fn Lvl10MeshChange
  (return (Utilities|Array|MakeArray (Variables|Default|GetBase_B)) (Utilities|Array|MakeArray "/Game/Characters/NPC/Turrets/Meshes/SM_Turrets_RocketLauncher_RocketLauncher_2_Base.SM_Turrets_RocketLauncher_RocketLauncher_2_Base")))

(fn Lvl20MeshChange
  (return (Utilities|Array|MakeArray (Variables|Default|GetYaw_B)) (Utilities|Array|MakeArray "/Game/Characters/NPC/Turrets/Meshes/SM_Turrets_RocketLauncher_RocketLauncher_2_Yaw.SM_Turrets_RocketLauncher_RocketLauncher_2_Yaw")))

(fn Lvl30MeshChange
  (return (Utilities|Array|MakeArray (Variables|Default|GetBack_M)) (Utilities|Array|MakeArray "/Game/Characters/NPC/Turrets/Meshes/SM_Turrets_RocketLauncher_RocketLauncher_2_Back.SM_Turrets_RocketLauncher_RocketLauncher_2_Back")))

(fn Lvl40MeshChange
  (return (Utilities|Array|MakeArray (Variables|Default|GetPitch_B)) (Utilities|Array|MakeArray "/Game/Characters/NPC/Turrets/Meshes/SM_Turrets_RocketLauncher_RocketLauncher_2_Pitch.SM_Turrets_RocketLauncher_RocketLauncher_2_Pitch")))

(fn Lvl50MeshChange
  (return (Utilities|Array|MakeArray (Variables|Default|GetScope_M)) (Utilities|Array|MakeArray "/Game/Characters/NPC/Turrets/Meshes/SM_Turrets_RocketLauncher_RocketLauncher_2_Scope.SM_Turrets_RocketLauncher_RocketLauncher_2_Scope")))

(fn Lvl60MeshChange
  (return (Utilities|Array|MakeArray (Variables|Default|GetBase_B)) (Utilities|Array|MakeArray "/Game/Characters/NPC/Turrets/Meshes/SM_Turrets_RocketLauncher_RocketLauncher_3_Base.SM_Turrets_RocketLauncher_RocketLauncher_3_Base")))

(fn Lvl70MeshChange
  (return (Utilities|Array|MakeArray (Variables|Default|GetYaw_B)) (Utilities|Array|MakeArray "/Game/Characters/NPC/Turrets/Meshes/SM_Turrets_RocketLauncher_RocketLauncher_3_Yaw.SM_Turrets_RocketLauncher_RocketLauncher_3_Yaw")))

(fn Lvl80MeshChange
  (return (Utilities|Array|MakeArray (Variables|Default|GetBack_M)) (Utilities|Array|MakeArray "/Game/Characters/NPC/Turrets/Meshes/SM_Turrets_RocketLauncher_RocketLauncher_3_Back.SM_Turrets_RocketLauncher_RocketLauncher_3_Back")))

(fn Lvl90MeshChange
  (return (Utilities|Array|MakeArray (Variables|Default|GetPitch_B)) (Utilities|Array|MakeArray "/Game/Characters/NPC/Turrets/Meshes/SM_Turrets_RocketLauncher_RocketLauncher_3_Pitch.SM_Turrets_RocketLauncher_RocketLauncher_3_Pitch")))

(fn Lvl100MeshChange
  (return (Utilities|Array|MakeArray (Variables|Default|GetScope_M)) (Utilities|Array|MakeArray "/Game/Characters/NPC/Turrets/Meshes/SM_Turrets_RocketLauncher_RocketLauncher_3_Scope.SM_Turrets_RocketLauncher_RocketLauncher_3_Scope")))

(fn AddShootstoDataCollector
  (params (TowerShots :type Integer))
  (bind _datacollector (CallFunction|GetDataCollector))
  (bind _rocketlaunchershotstotal (Default|AddRocketLauncherShots _datacollector TowerShots))
  (return _rocketlaunchershotstotal _datacollector))

(fn AddTimesUpgradestoDataCollector
  (params (AmountUpgraded :type Integer))
  (bind _datacollector (CallFunction|GetDataCollector))
  (bind _totalrocketlauncherupgrades (Default|AddRocketLauncherUpgrade _datacollector AmountUpgraded))
  (return _totalrocketlauncherupgrades _datacollector))