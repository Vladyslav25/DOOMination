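; Laser turret child Blueprint that damages its focused enemy directly, with a damage multiplier that climbs every Tick and resets on target change.
; ShootProjectile calls DoDamage, which aims the beam FX and applies damage.
; The LaserWidth timeline drives beam width and particles, reversing at high speed on shutoff, while DoOnce gates the attached sound.
; Overrides supply per-level stats, cost, mesh swaps every ten levels and data-collector reporting.
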(event Custom|TurnLaserOn
  (params (Target%20Location :type Vector))
  (bind _fx_system (Variables|Default|GetFX%20System))
  (Utilities|FlowControl|Sequence
    (:then_0
      (Utilities|FlowControl|DoOnce false
        (:Completed
          (bind _returnvalue (Class|FMODBlueprintStatics|PlayEventAttached "/Game/FMOD/Events/Turret/laser_shoot.laser_shoot" (Variables|Default|GetArrowComponent) "None" "0, 0, 0" "KeepRelativeOffset")))))
    (:then_1
      (Effects|Components|ParticleSystem|SetVectorParameter _fx_system "EndPos" Target%20Location)
      (Class|NiagaraComponent|SetVariableInt _fx_system "ParticelSpawnCount" 1)
      (bind _output (Timeline|LaserWidth Play)
        (:Update
          (Effects|Components|ParticleSystem|SetFloatParameter _fx_system "BeamWidth" _output)
          (Effects|Components|ParticleSystem|SetFloatParameter _fx_system "DragParticelsSpawnRate" _output))
        (:Finished
          (Utilities|FlowControl|DoOnce false
            (:Completed
              (Components|Timeline|SetPlayRate (Variables|Default|GetLaserWidth) 1.0))))))))

(event Custom|TurnLaserOff
  (bind _fx_system (Variables|Default|GetFX%20System))
  (Utilities|IsValid (stale Custom|TurnLaserOn _returnvalue)
    (:Is%20Valid
      (Class|FMODAudioComponent|Stop (stale Custom|TurnLaserOn _returnvalue)))
    (:Is%20Not%20Valid
      _))
  (Utilities|FlowControl|Sequence
    (:then_0
      (Utilities|FlowControl|DoOnce false) ; enters at Reset
    )
    (:then_1
      (Class|NiagaraComponent|SetVariableInt _fx_system "ParticelSpawnCount")
      (Components|Timeline|SetPlayRate (Variables|Default|GetLaserWidth) 5e+02)
      (Utilities|FlowControl|Sequence
        (:then_0
          (goto _label Reset))
        (:then_1
          (bind _output (Timeline|LaserWidth Reverse)
            (:Update
              (Effects|Components|ParticleSystem|SetFloatParameter _fx_system "BeamWidth" _output)
              (Effects|Components|ParticleSystem|SetFloatParameter _fx_system "DragParticelsSpawnRate" _output))
            (:Finished
              (Utilities|FlowControl|DoOnce false :!label _label
                (:Completed
                  (Components|Timeline|SetPlayRate (Variables|Default|GetLaserWidth) 1.0))))))))))

(event EventBeginPlay
  (|CallParentFunction)
  (Variables|Default|SetMainArrowComponent (Variables|Default|GetArrow_0))
  (Variables|Default|SetProjectile "/Game/Characters/NPC/Turrets/Blueprints/BlueprintProjectile/BP_LaserProjectile.BP_LaserProjectile_C")
  (CallFunction|TurnLaserOff)
  (CallFunction|AddMeshes (Utilities|Array|MakeArray (Variables|Default|GetBatteries_M) (Variables|Default|GetBarrel_M) (Variables|Default|GetScope_M))))

(event Collision|EventActorBeginOverlap
  (params (OtherActor :type Actor%20Object%20Reference)))

(event EventTick
  (params (DeltaSeconds :type Float%20%28single-precision%29))
  (|CallParentFunction DeltaSeconds)
  (Variables|Default|SetCurrentDamageMultiplier (+ (Variables|Default|GetCurrentDamageMultiplier) (* DeltaSeconds (Variables|Default|GetDamageMultiplyPerSecond)))))

(event EventFocusedEnemyChanged
  (CallFunction|TurnLaserOff)
  ;[1 1 1] Reset Damage Multiplier when Enemy is changed
  (Variables|Default|SetCurrentDamageMultiplier 1.0))

(event EventOnDeleteTower
  (CallFunction|AddMeshes (Utilities|Array|MakeArray (Variables|Default|GetBatteries_M) (Variables|Default|GetBarrel_M) (Variables|Default|GetScope_M)))
  (|CallParentFunction))

(fn ConstructionScript
  (bind _fx_system (Variables|Default|GetFX%20System))
  (|CallParentFunction)
  (Effects|Components|ParticleSystem|SetFloatParameter _fx_system "BeamWidth" 0.0)
  (Class|NiagaraComponent|SetVariableInt _fx_system "ParticelSpawnCount")
  (Effects|Components|ParticleSystem|SetFloatParameter _fx_system "DragParticelsSpawnRate" 0.0))

(fn ShootProjectile
  (params (ArrowComponent :type Arrow%20Component%20Object%20Reference))
  (CallFunction|DoDamage)
  (Math|Integer|IncrementInt (Variables|Default|GetShots)
    (:%20%20
      (return 0))))

(fn DoDamage
  (bind _focusedenemy (Variables|Default|GetFocusedEnemy))
  (CallFunction|TurnLaseron (Transformation|GetActorLocation (Variables|Default|GetFocusedEnemy)))
  (Utilities|IsValid _focusedenemy
    (:Is%20Valid
      (Game|Damage|ApplyDamage _focusedenemy (* (Variables|Default|GetDamage) (Variables|Default|GetCurrentDamageMultiplier)) 0 self "/Game/Characters/NPC/Turrets/Blueprints/BP_TowerDamagaType.BP_TowerDamagaType_C"))))

(fn DamagePerLevel
  (return 0.25))

(fn RangePerXLevel
  (return 4e+02))

(fn AttackspeedPerXLevel
  (return 0.0))

(fn GetTurretCosts
  (return 1.4e+02))

(fn Lvl10MeshChange
  (return (Utilities|Array|MakeArray (Variables|Default|GetBase_B)) (Utilities|Array|MakeArray "/Game/Characters/NPC/Turrets/Meshes/SM_Turrets_Laser_Laser_2_Base.SM_Turrets_Laser_Laser_2_Base")))

(fn Lvl20MeshChange
  (return (Utilities|Array|MakeArray (Variables|Default|GetYaw_B)) (Utilities|Array|MakeArray "/Game/Characters/NPC/Turrets/Meshes/SM_Turrets_Laser_Laser_2_Yaw.SM_Turrets_Laser_Laser_2_Yaw")))

(fn Lvl30MeshChange
  (return (Utilities|Array|MakeArray (Variables|Default|GetBarrel_M)) (Utilities|Array|MakeArray "/Game/Characters/NPC/Turrets/Meshes/SM_Turrets_Laser_Laser_2_Barrel.SM_Turrets_Laser_Laser_2_Barrel")))

(fn Lvl40MeshChange
  (return (Utilities|Array|MakeArray (Variables|Default|GetBatteries_M)) (Utilities|Array|MakeArray "/Game/Characters/NPC/Turrets/Meshes/SM_Turrets_Laser_Laser_2_Batteries.SM_Turrets_Laser_Laser_2_Batteries")))

(fn Lvl50MeshChange
  (return (Utilities|Array|MakeArray (Variables|Default|GetPitch_B)) (Utilities|Array|MakeArray "/Game/Characters/NPC/Turrets/Meshes/SM_Turrets_Laser_Laser_2_Pitch.SM_Turrets_Laser_Laser_2_Pitch")))

(fn Lvl60MeshChange
  (return (Utilities|Array|MakeArray (Variables|Default|GetScope_M)) (Utilities|Array|MakeArray "/Game/Characters/NPC/Turrets/Meshes/SM_Turrets_Laser_Laser_2_Scope.SM_Turrets_Laser_Laser_2_Scope")))

(fn Lvl70MeshChange
  (return (Utilities|Array|MakeArray (Variables|Default|GetBase_B)) (Utilities|Array|MakeArray "/Game/Characters/NPC/Turrets/Meshes/SM_Turrets_Laser_Laser_3_Base.SM_Turrets_Laser_Laser_3_Base")))

(fn Lvl80MeshChange
  (return (Utilities|Array|MakeArray (Variables|Default|GetYaw_B)) (Utilities|Array|MakeArray "/Game/Characters/NPC/Turrets/Meshes/SM_Turrets_Laser_Laser_3_Yaw.SM_Turrets_Laser_Laser_3_Yaw")))

(fn Lvl90MeshChange
  (return (Utilities|Array|MakeArray (Variables|Default|GetBarrel_M)) (Utilities|Array|MakeArray "/Game/Characters/NPC/Turrets/Meshes/SM_Turrets_Laser_Laser_3_Barrel.SM_Turrets_Laser_Laser_3_Barrel")))

(fn Lvl100MeshChange
  (return (Utilities|Array|MakeArray (Variables|Default|GetBatteries_M)) (Utilities|Array|MakeArray "/Game/Characters/NPC/Turrets/Meshes/SM_Turrets_Laser_Laser_3_Batteries.SM_Turrets_Laser_Laser_3_Batteries")))

(fn Lvl110MeshChange
  (return (Utilities|Array|MakeArray (Variables|Default|GetPitch_B)) (Utilities|Array|MakeArray "/Game/Characters/NPC/Turrets/Meshes/SM_Turrets_Laser_Laser_3_Pitch.SM_Turrets_Laser_Laser_3_Pitch")))

(fn Lvl120MeshChange
  (return (Utilities|Array|MakeArray (Variables|Default|GetScope_M)) (Utilities|Array|MakeArray "/Game/Characters/NPC/Turrets/Meshes/SM_Turrets_Laser_Laser_3_Scope.SM_Turrets_Laser_Laser_3_Scope")))

(fn AddShootstoDataCollector
  (params (TowerShots :type Integer))
  (bind _datacollector (CallFunction|GetDataCollector))
  (bind _totallasershots (Default|AddLaserShots _datacollector TowerShots))
  (return _totallasershots _datacollector))

(fn AddTimesUpgradestoDataCollector
  (params (AmountUpgraded :type Integer))
  (bind _datacollector (CallFunction|GetDataCollector))
  (bind _totallaserupgrades (Default|AddLaserUpgrade _datacollector AmountUpgraded))
  (return _totallaserupgrades _datacollector))