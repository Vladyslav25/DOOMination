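; Rifle turret, a child tower Blueprint that fires rifle projectiles and supplies its own cost and per-level damage, range and attack speed values.
; Each shot plays a barrel recoil timeline, applied as per-frame local offset deltas, with play rate tied to reload time.
; Level milestone overrides swap individual meshes through upgraded visual tiers every ten levels.
; It also counts rifle shots in the tower point's data collector.
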(event Custom|ShotAnimation
  ;[1 1 1] Reset Last Value
  (Variables|Components|SetAnimationLastValue 0.0)
  (bind _barrel_b_local_x_coordinate (Timeline|Shoot%20Animation PlayFromStart)
    (:Update
      ;[1 1 1] Subtract the Value last frame from the current value to get the difference, because we ADD local and not SET
      (Transformation|AddLocalOffset (Variables|Default|GetBarrel_B) (Math|Vector|MakeVector (- _barrel_b_local_x_coordinate (Variables|Components|GetAnimationLastValue)) 0.0 0.0) false false)
      (Variables|Components|SetAnimationLastValue _barrel_b_local_x_coordinate))))

(event EventBeginPlay
  (|CallParentFunction)
  (Variables|Default|SetMainArrowComponent (Variables|Default|GetArrow))
  (Variables|Default|SetProjectile "/Game/Characters/NPC/Turrets/Blueprints/BlueprintProjectile/BP_RifleProjectile.BP_RifleProjectile_C")
  ;[1 1 1] Set play rate of shoot Animation.
  (Components|Timeline|SetPlayRate (Variables|Default|GetShoot%20Animation) (/ 1.0 (Variables|Default|GetReloadTime)))
  (CallFunction|AddMeshes (Utilities|Array|MakeArray (Variables|Default|GetBack_M) (Variables|Default|GetBarrel_B) (Variables|Default|GetScope_M) (Variables|Default|GetSpring_M))))

(event Collision|EventActorBeginOverlap
  (params (OtherActor :type Actor%20Object%20Reference)))

(event EventTick
  (params (DeltaSeconds :type Float%20%28single-precision%29))
  (|CallParentFunction DeltaSeconds) ; This node is disabled and will not be called.\nDrag off pins to build functionality.
)

(event EventOnDeleteTower
  (CallFunction|AddMeshes (Utilities|Array|MakeArray (Variables|Default|GetBack_M) (Variables|Default|GetBarrel_B) (Variables|Default|GetScope_M) (Variables|Default|GetSpring_M)))
  (|CallParentFunction))

(fn ConstructionScript
  (|CallParentFunction))

(fn ShootProjectile
  (params (ArrowComponent :type Arrow%20Component%20Object%20Reference))
  ;[1 1 1] Shoot Projectile and play Animation
  (bind _shotprojectile (|CallParentFunction ArrowComponent))
  (CallFunction|ShotAnimation)
  (return _shotprojectile))

(fn DamagePerLevel
  (return 1.0))

(fn RangePerXLevel
  (return 4e+02))

(fn AttackspeedPerXLevel
  (return 0.11))

(fn GetTurretCosts
  (return 114.0))

(fn SetAttackspeed
  (params (NewAttackspeed :type Float%20%28single-precision%29))
  (bind _attackspeed (|CallParentFunction NewAttackspeed))
  (Components|Timeline|SetPlayRate (Variables|Default|GetShoot%20Animation) (/ 1.0 (Variables|Default|GetReloadTime)))
  (return _attackspeed))

(fn Lvl10MeshChange
  (return (Utilities|Array|MakeArray (Variables|Default|GetBase_B)) (Utilities|Array|MakeArray "/Game/Characters/NPC/Turrets/Meshes/SM_Turrets_Rifle_Rifle_2_Base.SM_Turrets_Rifle_Rifle_2_Base")))

(fn Lvl20MeshChange
  (return (Utilities|Array|MakeArray (Variables|Default|GetYaw_B)) (Utilities|Array|MakeArray "/Game/Characters/NPC/Turrets/Meshes/SM_Turrets_Rifle_Rifle_2_Yaw.SM_Turrets_Rifle_Rifle_2_Yaw")))

(fn Lvl30MeshChange
  (bind _spring_m (Variables|Default|GetSpring_M))
  ;[1 1 1] Spring lvl 1 has another material than lvl 2 and lvl 3, so we need to change the material here
  (Rendering|Material|SetMaterial _spring_m 0 "/Game/Characters/NPC/Turrets/Materials/M_Spring_2Surface.M_Spring_2Surface")
  (return (Utilities|Array|MakeArray _spring_m) (Utilities|Array|MakeArray "/Game/Characters/NPC/Turrets/Meshes/SM_Turrets_Rifle_Rifle_2_Spring.SM_Turrets_Rifle_Rifle_2_Spring")))

(fn Lvl40MeshChange
  (return (Utilities|Array|MakeArray (Variables|Default|GetBack_M)) (Utilities|Array|MakeArray "/Game/Characters/NPC/Turrets/Meshes/SM_Turrets_Rifle_Rifle_2_Back.SM_Turrets_Rifle_Rifle_2_Back")))

(fn Lvl50MeshChange
  (return (Utilities|Array|MakeArray (Variables|Default|GetScope_M)) (Utilities|Array|MakeArray "/Game/Characters/NPC/Turrets/Meshes/SM_Turrets_Rifle_Rifle_2_Scope.SM_Turrets_Rifle_Rifle_2_Scope")))

(fn Lvl60MeshChange
  (return (Utilities|Array|MakeArray (Variables|Default|GetBarrel_B)) (Utilities|Array|MakeArray "/Game/Characters/NPC/Turrets/Meshes/SM_Turrets_Rifle_Rifle_2_Barrel.SM_Turrets_Rifle_Rifle_2_Barrel")))

(fn Lvl70MeshChange
  (return (Utilities|Array|MakeArray (Variables|Default|GetPitch_B)) (Utilities|Array|MakeArray "/Game/Characters/NPC/Turrets/Meshes/SM_Turrets_Rifle_Rifle_2_Pitch.SM_Turrets_Rifle_Rifle_2_Pitch")))

(fn Lvl80MeshChange
  (return (Utilities|Array|MakeArray (Variables|Default|GetBase_B)) (Utilities|Array|MakeArray "/Game/Characters/NPC/Turrets/Meshes/SM_Turrets_Rifle_Rifle_3_Base.SM_Turrets_Rifle_Rifle_3_Base")))

(fn Lvl90MeshChange
  (return (Utilities|Array|MakeArray (Variables|Default|GetYaw_B)) (Utilities|Array|MakeArray "/Game/Characters/NPC/Turrets/Meshes/SM_Turrets_Rifle_Rifle_3_Yaw.SM_Turrets_Rifle_Rifle_3_Yaw")))

(fn Lvl100MeshChange
  (return (Utilities|Array|MakeArray (Variables|Default|GetSpring_M)) (Utilities|Array|MakeArray "/Game/Characters/NPC/Turrets/Meshes/SM_Turrets_Rifle_Rifle_3_Spring.SM_Turrets_Rifle_Rifle_3_Spring")))

(fn Lvl110MeshChange
  (return (Utilities|Array|MakeArray (Variables|Default|GetBack_M)) (Utilities|Array|MakeArray "/Game/Characters/NPC/Turrets/Meshes/SM_Turrets_Rifle_Rifle_3_Back.SM_Turrets_Rifle_Rifle_3_Back")))

(fn Lvl120MeshChange
  (return (Utilities|Array|MakeArray (Variables|Default|GetScope_M)) (Utilities|Array|MakeArray "/Game/Characters/NPC/Turrets/Meshes/SM_Turrets_Rifle_Rifle_3_Scope.SM_Turrets_Rifle_Rifle_3_Scope")))

(fn Lvl130MeshChange
  (return (Utilities|Array|MakeArray (Variables|Default|GetBarrel_B)) (Utilities|Array|MakeArray "/Game/Characters/NPC/Turrets/Meshes/SM_Turrets_Rifle_Rifle_3_Barrel.SM_Turrets_Rifle_Rifle_3_Barrel")))

(fn Lvl140MeshChange
  (return (Utilities|Array|MakeArray (Variables|Default|GetPitch_B)) (Utilities|Array|MakeArray "/Game/Characters/NPC/Turrets/Meshes/SM_Turrets_Rifle_Rifle_3_Pitch.SM_Turrets_Rifle_Rifle_3_Pitch")))

(fn AddShoottoDataCollector
  (bind _result (Math|Integer|IncrementInt (Variables|/Game/DataCollector/BP_DataCollector.BP_DataCollector_C|GetShotRifleShots (Default|GetDataCollector (.TowerPoint (CallFunction|GetTowerPoint)))))
    (:%20%20
      (return _result))))