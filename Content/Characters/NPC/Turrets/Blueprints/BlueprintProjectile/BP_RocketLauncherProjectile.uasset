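; Rocket launcher turret projectile that deals area damage to enemies and destroys itself when either of its colliders begins an overlap.
; Both the Collider and Box overlap events pass their component location to AOEDamage.
; AOEDamage runs a sphere overlap for BP_BaseEnemy pawns within AOERadius and applies Damage to each with the tower damage type.
; It also draws a debug sphere showing the blast radius.
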(event OnComponentBeginOverlap(Collider)
  (params (OverlappedComponent :type Primitive%20Component%20Object%20Reference) (OtherActor :type Actor%20Object%20Reference) (OtherComp :type Primitive%20Component%20Object%20Reference) (OtherBodyIndex :type Integer) (bFromSweep :type Boolean) (SweepResult :type Hit%20Result%20Structure%20%28by%20ref%29))
  (CallFunction|AOEDamage (Transformation|GetWorldLocation (Variables|Default|GetCollider)))
  (Actor|DestroyActor))

(event OnComponentBeginOverlap(Box)
  (params (OverlappedComponent :type Primitive%20Component%20Object%20Reference) (OtherActor :type Actor%20Object%20Reference) (OtherComp :type Primitive%20Component%20Object%20Reference) (OtherBodyIndex :type Integer) (bFromSweep :type Boolean) (SweepResult :type Hit%20Result%20Structure%20%28by%20ref%29))
  (CallFunction|AOEDamage (Transformation|GetWorldLocation (Variables|Default|GetBox)))
  (Actor|DestroyActor))

(event EventBeginPlay)

(event Collision|EventActorBeginOverlap
  (params (OtherActor :type Actor%20Object%20Reference)))

(fn ConstructionScript
  (|CallParentFunction))

(fn AOEDamage
  (params (OverlappedObjectPosition :type Vector))
  ;[1 1 1] DEBUG__Draw AOE
  (Rendering|Debug|DrawDebugSphere OverlappedObjectPosition (Variables|Default|GetAOERadius) 12 "(R=1.000000,G=0.000000,B=0.902083,A=1.000000)" 1.0)
  ;[1 1 1] Create Sphere Collider arount the Projectile to check if enemies are in range.
  (bind _outactors (Collision|SphereOverlapActors OverlappedObjectPosition (Variables|Default|GetAOERadius) (Utilities|Array|MakeArray "ObjectTypeQuery3") "/Game/Characters/NPC/Enemies/Blueprints/BP_BaseEnemy.BP_BaseEnemy_C"))
  ;[1 1 1] check if hit enemies or max hit count is higher. decrease it by 1 to contert it to index
  (bind _result (Math|Integer|DecrementInt (Utilities|Array|Length _outactors))
    (:%20%20
      ;[1 1 1] Apply Damage to every Enemy in Range
      (for _index (range 0 _result)
        (Game|Damage|ApplyDamage (Utilities|Array|Get(acopy) _outactors _index) (Variables|Default|GetDamage) 0 self "/Game/Characters/NPC/Turrets/Blueprints/BP_TowerDamagaType.BP_TowerDamagaType_C"))
      (return _outactors))))