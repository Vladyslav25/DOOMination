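; Base projectile for NPC turrets that homes in on a targeted enemy and damages the enemies it hits.
; Each Tick re-aims ProjectileMovement velocity at the target's location at initial speed, curving the flight to prevent misses.
; Collider and Box overlaps apply tower damage to any BP_BaseEnemy, targeted or not.
; DestroyProjectile spawns an effect and destroys the actor on impact or despawner contact; a five-second lifespan also limits it.
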(event OnComponentBeginOverlap(Collider)
  (params (OverlappedComponent :type Primitive%20Component%20Object%20Reference) (OtherActor :type Actor%20Object%20Reference) (OtherComp :type Primitive%20Component%20Object%20Reference) (OtherBodyIndex :type Integer) (bFromSweep :type Boolean) (SweepResult :type Hit%20Result%20Structure%20%28by%20ref%29))
  ;[1 1 1] Hit an enemy. Does not check for target. If projectile hit an enemy it applies damage to it
  (bind _asbp_base_enemy (Utilities|Casting|CastToBP_BaseEnemy OtherActor)
    (:then
      (Game|Damage|ApplyDamage _asbp_base_enemy (Variables|Default|GetDamage) 0 self "/Game/Characters/NPC/Turrets/Blueprints/BP_TowerDamagaType.BP_TowerDamagaType_C"))
    (:CastFailed
      _))
  (CallFunction|DestroyProjectile))

(event OnComponentBeginOverlap(Box)
  (params (OverlappedComponent :type Primitive%20Component%20Object%20Reference) (OtherActor :type Actor%20Object%20Reference) (OtherComp :type Primitive%20Component%20Object%20Reference) (OtherBodyIndex :type Integer) (bFromSweep :type Boolean) (SweepResult :type Hit%20Result%20Structure%20%28by%20ref%29))
  ;[1 1 1] Hit an enemy. Does not check for target. If projectile hit an enemy it applies damage to it
  (bind _asbp_base_enemy (Utilities|Casting|CastToBP_BaseEnemy OtherActor)
    (:then
      (Game|Damage|ApplyDamage _asbp_base_enemy (Variables|Default|GetDamage) 0 self "/Game/Characters/NPC/Turrets/Blueprints/BP_TowerDamagaType.BP_TowerDamagaType_C"))
    (:CastFailed
      (Utilities|Casting|CastToBP_ProjectileDespawner OtherActor)))
  (CallFunction|DestroyProjectile))

(event EventBeginPlay
  (Actor|SetLifeSpan 5.0))

(event EventTick
  (params (DeltaSeconds :type Float%20%28single-precision%29))
  (bind _targetedenemy (Variables|Default|GetTargetedEnemy))
  ;[1 1 1] Projectile look to enemy and fly in this direction (curves) so the projectile can not miss
  (Utilities|IsValid _targetedenemy
    (:Is%20Valid
      (Variables|/Script/Engine.MovementComponent|SetVelocity (Variables|Default|GetProjectileMovement) (* (Math|Rotator|GetRotationXVector (Math|Rotator|FindLookatRotation (Transformation|GetActorLocation) (Transformation|GetActorLocation _targetedenemy))) (Variables|/Script/Engine.ProjectileMovementComponent|GetInitialSpeed (Variables|Default|GetProjectileMovement)))))))

(fn ConstructionScript)

(fn DestroyProjectile
  (Niagara|SpawnSystematLocation 0 (Transformation|GetActorLocation))
  (Actor|DestroyActor))