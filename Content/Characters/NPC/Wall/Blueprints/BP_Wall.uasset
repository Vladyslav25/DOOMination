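; BP_Wall is a damageable wall, filed with the NPC characters, that tracks its own hitpoints and death state.
; AnyDamage passes damage to GetDamage, which lowers Hitpoints with a floor of zero, sets Dead at zero and returns that flag.
; A true result calls OnDeath, currently an empty event, and repeats on any later hit.
; GetHitpoints and IsDead expose the current state.
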(event Custom|OnDeath)

(event Game|Damage|EventAnyDamage
  (params (Damage :type Float%20%28single-precision%29) (DamageType :type Damage%20Type%20Object%20Reference) (InstigatedBy :type Controller%20Object%20Reference) (DamageCauser :type Actor%20Object%20Reference))
  (bind _lethal (CallFunction|GetDamage Damage))
  (if _lethal
    (CallFunction|OnDeath)))

(fn ConstructionScript)

(fn GetHitpoints
  (return (Variables|Default|GetHitpoints)))

(fn GetDamage
  (params (Damage :type Float%20%28single-precision%29))
  ;[1 1 1] Set new HP. Min value: 0
  (bind _output_get (Variables|Default|SetHitpoints (Math|Float|Max(Float) (- (Variables|Default|GetHitpoints) Damage) 0.0)))
  (if (<= _output_get 0.0)
    ;[1 1 1] Set Dead variable
    (Variables|Default|SetDead true))
  (return (Variables|Default|GetDead)))

(fn IsDead
  (return (Variables|Default|GetDead)))