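; Base tower-defense enemy that advances along a spline, damages the wall, and drops Argent on death.
; Damage is tallied by player or tower type, with overkill trimmed; player final blows, or tower kills without majority tower damage, count as player kills.
; Player kills spawn double Argent that flies to the player.
; Death removes it from its spawner, ragdolls it, then dissolves its material on Tick before destroying it and attached actors.
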(event Custom|OnDeath
  (bind _enemyspawner (Variables|Default|GetEnemySpawner))
  (CallFunction|ActivateRagdoll)
  (if (Variables|Default|GetPlayerKill?)
    (CallFunction|PlayerKill)
    (else
      (CallFunction|TowerKill)))
  ;[1 1 1] Remove from List
  (Utilities|IsValid _enemyspawner
    (:Is%20Valid
      (Default|RemoveEnemy _enemyspawner self))
    (:Is%20Not%20Valid
      ;[1 1 1] If EnemySpawner is null, print string instead
      (Development|PrintString (Utilities|String|Append "Enemy Spawner is null: " (Utilities|GetDisplayName self)) true true "(R=1.000000,G=0.000000,B=0.000000,A=1.000000)" 5.0)))
  ;[1 1 1] Set Delay so enemy does not disappear instantly
  (Utilities|FlowControl|Delay 2.5)
  (Variables|Default|SetIsDisintegrating true))

(event Custom|ReachedEnd
  (AI|Logic|StopLogic (Variables|/Script/AIModule.AIController|GetBrainComponent (AI|GetAIController self)) "Is at Wall"))

(event Custom|DamageToWall
  (Game|Damage|ApplyDamage (Variables|WallValues|GetWall) (Variables|WallValues|GetWallDamage) 0 self))

(event EventBeginPlay
  (bind _returnvalue (Rendering|Material|CreateDynamicMaterialInstance (Variables|Default|GetMesh) 0 (Variables|Default|GetMaterial) "None" :!class /Script/Engine.PrimitiveComponent))
  (Variables|Default|SetMaterialRef _returnvalue))

(event Game|Damage|EventAnyDamage
  (params (Damage :type Float%20%28single-precision%29) (DamageType :type Damage%20Type%20Object%20Reference) (InstigatedBy :type Controller%20Object%20Reference) (DamageCauser :type Actor%20Object%20Reference))
  (CallFunction|GetDamage Damage DamageType DamageCauser))

(event EventTick
  (params (DeltaSeconds :type Float%20%28single-precision%29))
  (bind _materialref (Variables|Default|GetMaterialRef))
  (if (Variables|Default|GetIsDisintegrating)
    (bind _returnvalue (Rendering|Material|GetScalarParameterValue _materialref "Amount" :!class /Script/Engine.MaterialInstanceDynamic))
    (Rendering|Material|SetScalarParameterValue _materialref "Amount" (- _returnvalue (* DeltaSeconds 0.5)) :!class /Script/Engine.MaterialInstanceDynamic)
    (if (<= _returnvalue 0.0)
      (Utilities|FlowControl|DoOnce false
        (:Completed
          ;[1 1 1] If Enemy is dead, destroy it + attachments and do not run alive code
          (if (Variables|Default|GetIsDead)
            ;;[1 0.2656 0.2656 1 12] Need to save the attached compnents, because while destroying the array shift
            (bind _output_get (Variables|Default|SetAttachedComponents (Actor|GetAttachedActors false)))
            (for _array_element _output_get
              (Actor|DestroyActor _array_element))
            (Actor|DestroyActor)))))))

(fn ConstructionScript
  (Variables|/Script/Engine.FloatingPawnMovement|SetMaxSpeed (Variables|Default|GetFloatingPawnMovement) (Variables|Default|GetSpeed))
  (Variables|Default|SetHP (Variables|Default|GetStartHP)))

(fn GetPercentageOverSpline
  (bind _mainspline (Variables|Default|GetMainSpline))
  (bind _spline (Variables|/Game/Characters/NPC/Enemies/Blueprints/BP_Spline.BP_Spline_C|GetSpline _mainspline))
  (return (* (/ (Class|SplineComponent|FindInputKeyClosesttoWorldLocation _spline (Transformation|GetActorLocation)) (Math|Conversions|ToFloat(Integer) (- (Spline|GetNumberOfSplinePoints _spline) 1))) (Spline|GetSplineLength _spline))))

(fn GetDamage
  (params (Damage :type Float%20%28single-precision%29) (DamageType :type Damage%20Type%20Object%20Reference) (DamageCauser :type Actor%20Object%20Reference))
  (bind _output_get (LocalVariables|SetDamageDealt (Math|Float|Max(Float) Damage 0.0)))
  (Utilities|FlowControl|Sequence
    (:then_0
      ;[1 1 1] First reduce HP by amount of Damage
      (bind _output_get_2 (Variables|Default|SetHP (- (Variables|Default|GetHP) _output_get)))
      (if (<= _output_get_2 0.0)
        (Variables|Default|SetIsDead true)
        ;[1 1 1] Damage calculation how much Damage needed to kill so the Player needs to deal 50% of max HP of enemy.
        ; Enemy Max HP = 100, current HP = 1 --> 99 DMG from Player. If Tower deals more than 200 Dmg he would have dealt more damage than the Player. To solve this, Damage dealt can only be max equal to current health
        (Utilities|FlowControl|DoOnce false
          (:Completed
            (LocalVariables|SetDamageDealt (+ (LocalVariables|GetDamageDealt) (Variables|Default|GetHP)))))))
    (:then_1
      ;[1 1 1] Then check the source of the Damage so we know how dealt the damage. This is Tower Damage
      (Utilities|Casting|CastToBP_TowerDamagaType DamageType
        (:then
          (Variables|Default|SetTotalDamageByTower (+ _output_get (Variables|Default|GetTotalDamageByTower)))
          (Variables|Default|SetPlayerKill? false)
          ;[1 1 1] Checks if the Enemy is dead. If so call Function to do something. Set bool to True so the other function can not be called
          (if (Variables|Default|GetIsDead)
            (Utilities|FlowControl|DoOnce (Variables|Default|GetDoOnceClosed)
              (:Completed
                (if (> (Variables|Default|GetTotalDamageByTower) (Variables|Default|GetTotalDamageByPlayer))
                  (Variables|Default|SetDoOnceClosed true)
                  (else
                    (Variables|Default|SetPlayerKill? true :!label _label)
                    (Variables|Default|SetDoOnceClosed true)))))
            (else
              (return))))
        (:CastFailed
          ;[1 1 1] Then check the source of the Damage so we know how dealt the damage. This is Player Damage
          (Utilities|Casting|CastToBT_PlayerDamagaType DamageType)
          (Variables|Default|SetTotalDamageByPlayer (+ _output_get (Variables|Default|GetTotalDamageByPlayer)))
          (Variables|Default|SetPlayerKill? true)
          (if (Variables|Default|GetIsDead)
            (Utilities|FlowControl|DoOnce (Variables|Default|GetDoOnceClosed)
              (:Completed
                (goto _label)))
            (else
              (return)))))
      (CallFunction|OnDeath)
      (return))))

(fn TowerKill
  (Development|PrintString "Killed by Tower")
  (Game|SpawnActorfromClass "/Game/Gameplay/Argent/BP_Argent.BP_Argent_C" (Transformation|GetActorTransform) "Undefined" 0 (.Argent%20%28Rounded%29 (CallFunction|CalculateArgenttoSpawn)) false 0))

(fn PlayerKill
  (Development|PrintString "Killed by Player")
  (Game|SpawnActorfromClass "/Game/Gameplay/Argent/BP_Argent.BP_Argent_C" (Transformation|GetActorTransform) "Undefined" 0 (* (.Argent%20%28Rounded%29 (CallFunction|CalculateArgenttoSpawn)) 2) true 0))

(fn ChangeMaxHP
  (params (NewHP :type Float%20%28single-precision%29))
  (bind _output_get (Variables|Default|SetStartHP NewHP))
  (Variables|Default|SetHP _output_get)
  (return))

(fn SetWall
  (params (Wall :type BP%20Wall%20Object%20Reference))
  (bind _output_get (Variables|WallValues|SetWall Wall))
  (return _output_get))

(fn ActivateRagdoll
  (bind _mesh (Variables|Default|GetMesh))
  ;[1 1 1] Stop Movment
  (Class|NavMovementComponent|StopActiveMovement (Variables|Default|GetFloatingPawnMovement))
  ;[1 1 1] Disable Enemy Collision (Head and Capsule)
  (Collision|SetCollisionEnabled (Variables|Default|GetHeadCollision) "NoCollision")
  (Collision|SetCollisionEnabled (Variables|Default|GetCapsuleComponent) "NoCollision")
  ;[1 1 1] Configure Mesh Collision for Ragdoll
  (Collision|SetCollisionProfileName _mesh "EnemyPreset" false :!class /Script/Engine.PrimitiveComponent)
  (Collision|SetCollisionEnabled _mesh "QueryAndPhysics")
  (Physics|SetSimulatePhysics _mesh true)
  ;[1 1 1] Stop Animation
  (Class|SkeletalMeshComponent|SetAnimClass _mesh)
  ;[1 1 1] Stop Behaviortree so Enemies stop walking
  (AI|Logic|StopLogic (Variables|/Script/AIModule.AIController|GetBrainComponent (AI|GetAIController self)) "You Dead"))

(fn CalculateArgenttoSpawn
  (bind _starthp (Variables|Default|GetStartHP))
  (bind _returnvalue (* _starthp 0.1))
  (return (Math|Float|Truncate _returnvalue) _returnvalue))