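; BP_Tank is the Tank enemy NPC, a child Blueprint that relies on its parent for most behavior.
; Its construction script sets the Speed variable before running the parent construction script.
; On ReachedEnd it calls the parent, then sets CanAttack on its BP_TankAnimation anim instance to enable attacking.
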(event EventBeginPlay
  (|CallParentFunction) ; This node is disabled and will not be called.\nDrag off pins to build functionality.
)

(event Collision|EventActorBeginOverlap
  (params (OtherActor :type Actor%20Object%20Reference)))

(event EventTick
  (params (DeltaSeconds :type Float%20%28single-precision%29))
  (|CallParentFunction DeltaSeconds) ; This node is disabled and will not be called.\nDrag off pins to build functionality.
)

(event EventReachedEnd
  (|CallParentFunction)
  (bind _asbp_tank_animation (Utilities|Casting|CastToBP_TankAnimation (Components|SkeletalMesh|GetAnimInstance (Variables|Character|GetMesh))))
  (Variables|/Game/Characters/NPC/Enemies/Animations/Blueprints/BP_TankAnimation.BP_TankAnimation_C|SetCanAttack _asbp_tank_animation true))

(fn ConstructionScript
  (Variables|Default|SetSpeed 3.5e+02)
  (|CallParentFunction))