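; Base AI controller for enemy NPCs that supplies behavior tree destinations along the pawn's spline.
; On first Tick, it caches the BP_BaseEnemy pawn and its MainSpline, then runs BT_BaseEnemy, because the pawn is not yet set at BeginPlay.
; SplinePointReached advances the index, stores the new location and notifies the enemy.
; SetDestinationInBT writes the current point's world location, clamped to the last point, to the "destination" Blackboard key.
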(event Custom|SplinePointReached
  ;[1 1 1] Increase spline index by 1 and set new location for BT to move
  (bind _output_get (Variables|Default|SetSplineIndex (Math|Integer|Min(Integer) (Spline|GetNumberOfSplinePoints (Variables|/Game/Characters/NPC/Enemies/Blueprints/BP_Spline.BP_Spline_C|GetSpline (Variables|Default|GetSpline))) (+ (Variables|Default|GetSplineIndex) 1))))
  (Variables|Default|SetLocation (CallFunction|GetNewDestination _output_get))
  ;[1 1 1] Call method in BaseEnemy
  (Default|SplinePointReached (Variables|Default|GetMyCharacter) _output_get))

(event EventTick
  (params (DeltaSeconds :type Float%20%28single-precision%29))
  (Utilities|FlowControl|DoOnce false
    (:Completed
      ;[1 1 1] Set character and spline reference. Start behavior tree. This is done in the first "Tick" because in "BeginPlay", the controlled pawn is not set so we can't get the references.
      (bind _asbp_base_enemy (Utilities|Casting|CastToBP_BaseEnemy (Pawn|GetControlledPawn)))
      (Variables|Default|SetMyCharacter _asbp_base_enemy)
      (Variables|Default|SetSpline (Variables|/Game/Characters/NPC/Enemies/Blueprints/BP_BaseEnemy.BP_BaseEnemy_C|GetMainSpline _asbp_base_enemy))
      (AI|RunBehaviorTree "/Game/Characters/NPC/Enemies/Blueprints/AI/BT_BaseEnemy.BT_BaseEnemy"))))

(fn ConstructionScript)

(fn SetDestinationinBT
  (bind _splineindex (Variables|Default|GetSplineIndex))
  (bind _newlocation (CallFunction|GetNewDestination _splineindex))
  ;[1 1 1] Get new Destination and set it to BB variable
  (AI|Components|Blackboard|SetValueasVector (Variables|Default|GetBlackboard) (Utilities|Name|MakeLiteralName "destination") _newlocation)
  (return _newlocation))

(fn GetNewDestination
  (params (Index :type Integer))
  (bind _spline (Variables|Default|GetSpline))
  (bind _spline_2 (Variables|/Game/Characters/NPC/Enemies/Blueprints/BP_Spline.BP_Spline_C|GetSpline _spline))
  (return (Spline|GetLocationatSplinePoint _spline_2 (Math|Integer|Min(Integer) (- (Spline|GetNumberOfSplinePoints _spline_2) 1) Index) "World")))