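; BP_BaseEnemyAIController is the AI controller for base enemy characters.
; On BeginPlay it casts the controlled pawn to BP_BaseEnemy, caches it and runs the BT_BaseEnemy behavior tree.
; SetDestination asks the enemy for a new destination, writes it to the "destination" Blackboard key and returns it.
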(event EventBeginPlay
  (bind _asbp_base_enemy (Utilities|Casting|CastToBP_BaseEnemy (Pawn|GetControlledPawn)))
  (Variables|Default|SetMyCharacter _asbp_base_enemy)
  (AI|RunBehaviorTree "/Game/Test/VladiAi/Enemy/AI/BT_BaseEnemy.BT_BaseEnemy"))

(fn ConstructionScript)

(fn SetDestination
  ;[1 1 1] Get new Destination and set it to BB variable
  (bind _newdestination (Default|GetNewDestination (Variables|Default|GetMyCharacter)))
  (AI|Components|Blackboard|SetValueasVector (Variables|Default|GetBlackboard) (Utilities|Name|MakeLiteralName "destination") _newdestination)
  (return _newdestination))