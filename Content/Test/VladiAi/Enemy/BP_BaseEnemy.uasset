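; Base enemy character for what appears to be a tower defense mode, with spline helpers for its next destination and path progress.
; GetDamage reduces HP, trims overkill from the killing hit, and totals tower and player damage by damage type.
; A player's final hit earns player credit, while a tower's earns it only if tower damage leads; kill hooks are empty stubs.
; Death removes it from EnemySpawner, and Tick destroys it.
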(event Custom|OnDeath
  ;[1 1 1] Remove from List
  (Default|RemoveEnemy (Variables|Default|GetEnemySpawner) self))

(event EventBeginPlay)

(event Game|Damage|EventAnyDamage
  (params (Damage :type Float%20%28single-precision%29) (DamageType :type Damage%20Type%20Object%20Reference) (InstigatedBy :type Controller%20Object%20Reference) (DamageCauser :type Actor%20Object%20Reference))
  (CallFunction|GetDamage Damage DamageType DamageCauser))

(event EventTick
  (params (DeltaSeconds :type Float%20%28single-precision%29))
  (if (Variables|Default|GetIsDead)
    (Actor|DestroyActor)))

(fn ConstructionScript
  (Variables|/Script/Engine.CharacterMovementComponent|SetMaxWalkSpeed (Variables|Character|GetCharacterMovement) (Variables|Default|GetSpeed))
  (Variables|Default|SetHP (Variables|Default|GetStartHP)))

(fn GetNewDestination
  (bind _output_get (Variables|Default|SetDestination (Spline|FindLocationClosesttoWorldLocation (Variables|/Game/Test/VladiAi/BP_Spline.BP_Spline_C|GetSpline (Variables|Default|GetMainSpline)) (Transformation|GetWorldLocation (Variables|Default|GetMoveToGoal)) "World")))
  (return _output_get))

(fn GetPercentageOverSpline
  (bind _mainspline (Variables|Default|GetMainSpline))
  (bind _spline (Variables|/Game/Test/VladiAi/BP_Spline.BP_Spline_C|GetSpline _mainspline))
  (return (* (/ (Class|SplineComponent|FindInputKeyClosesttoWorldLocation _spline (Transformation|GetActorLocation)) (Math|Conversions|ToFloat(Integer) (- (Spline|GetNumberOfSplinePoints _spline) 1))) (Spline|GetSplineLength _spline))))

(fn GetDamage
  (params (Damage :type Float%20%28single-precision%29) (DamageType :type Damage%20Type%20Object%20Reference) (DamageCauser :type Actor%20Object%20Reference))
  (bind _output_get (LocalVariables|SetDamageDealt Damage))
  (Utilities|FlowControl|Sequence
    (:then_0
      ;[1 1 1] First reduce HP by amount of Damage
      (bind _output_get_2 (Variables|Default|SetHP (- (Variables|Default|GetHP) _output_get)))
      (if (<= _output_get_2 0.0)
        (Variables|Default|SetIsDead true)
        ;[1 1 1] Damage calculation how much Damage needed to kill so the Player needs to deal 50% of max HP of enemy.
        ; Enemy Max HP = 100, current HP = 1 --> 99 DMG from Tower. If player deals more than 200 Dmg he would have dealt more damage than the tower. To solve this, Damage dealt can only be max equal to current health
        (Utilities|FlowControl|DoOnce false
          (:Completed
            (LocalVariables|SetDamageDealt (+ (LocalVariables|GetDamageDealt) (Variables|Default|GetHP)))
            (CallFunction|OnDeath)))))
    (:then_1
      ;[1 1 1] Then check the source of the Damage so we know how dealt the damage. This is Tower Damage
      (Utilities|Casting|CastToBP_TowerDamagaType DamageType
        (:then
          (Variables|Default|SetTotalDamageByTower (+ _output_get (Variables|Default|GetTotalDamageByTower)))
          (Variables|Default|SetPlayerKill? false)
          ;[1 1 1] Checks if the Enemy is dead. If so call Function to do something. Set bool to True so the other function can not be called
          (if (Variables|Default|GetIsDead)
            (Utilities|FlowControl|DoOnce (Variables|Default|GetDoOnceClosed)
              (:Completed
                (if (> (Variables|Default|GetTotalDamageByTower) (Variables|Default|GetTotalDamageByPlayer))
                  (Variables|Default|SetDoOnceClosed true)
                  (Development|PrintString "Killed by Tower")
                  (return)
                  (else
                    _))))
            (else
              (return))))
        (:CastFailed
          ;[1 1 1] Then check the source of the Damage so we know how dealt the damage. This is Player Damage
          (Utilities|Casting|CastToBT_PlayerDamagaType DamageType)
          (Variables|Default|SetTotalDamageByPlayer (+ _output_get (Variables|Default|GetTotalDamageByPlayer)))
          (Variables|Default|SetPlayerKill? true)
          (if (Variables|Default|GetIsDead)
            (Utilities|FlowControl|DoOnce (Variables|Default|GetDoOnceClosed)
              (:Completed
                _))
            (else
              (return)))))
      (CallFunction|PlayerKill)
      (Variables|Default|SetDoOnceClosed true)
      (Development|PrintString "Killed by Player")
      (return))))

(fn TowerKill)

(fn PlayerKill)