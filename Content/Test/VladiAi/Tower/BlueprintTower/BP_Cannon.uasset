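; BP_Cannon is a tower Blueprint that fires BP_CannonProjectile from four alternating muzzle arrows.
; On BeginPlay it sets the projectile class and starts at the top-left arrow, leaving the shot itself to the parent class.
; After each parent ShootProjectile call, SetNewArrow picks the main arrow from ArrowIndex modulo four and increments the index.
; Since the index is read before incrementing, the first switch can reselect the starting arrow.
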(event EventBeginPlay
  (|CallParentFunction)
  (Variables|Default|SetMainArrowComponent (Variables|Default|GetArrow_TL))
  (Variables|Default|SetProjectile "/Game/Test/VladiAi/Tower/BlueprintProjectile/BP_CannonProjectile.BP_CannonProjectile_C"))

(event Collision|EventActorBeginOverlap
  (params (OtherActor :type Actor%20Object%20Reference)))

(event EventTick
  (params (DeltaSeconds :type Float%20%28single-precision%29))
  (|CallParentFunction DeltaSeconds) ; This node is disabled and will not be called.\nDrag off pins to build functionality.
)

(fn ConstructionScript
  (|CallParentFunction))

(fn ShootProjectile
  (params (ArrowComponent :type Arrow%20Component%20Object%20Reference))
  (|CallParentFunction ArrowComponent)
  (CallFunction|SetNewArrow))

(fn SetNewArrow
  ;[1 1 1] If projectile was show change the arrow component and increase the index
  (switch int (Math|Integer|%(Integer) (Variables|NewArrow|GetArrowIndex) 4)
    (:0
      (Variables|Default|SetMainArrowComponent (Variables|Default|GetArrow_TL)))
    (:1
      (Variables|Default|SetMainArrowComponent (Variables|Default|GetArrow_DL)))
    (:2
      (Variables|Default|SetMainArrowComponent (Variables|Default|GetArrow_TR)))
    (:3
      (Variables|Default|SetMainArrowComponent (Variables|Default|GetArrow_DR))))
  (Math|Integer|IncrementInt (Variables|NewArrow|GetArrowIndex)))