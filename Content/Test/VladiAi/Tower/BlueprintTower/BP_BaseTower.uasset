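; Base tower Blueprint for a tower defense that aims at and fires projectiles at enemies inside its radius-sized sphere.
; Overlaps maintain the in-range list; each tick focuses the enemy with the greatest Distance value.
; A rotation timeline lerps separate yaw and pitch components toward the target, then calls Shoot, gated by a DoOnce that a reload timeline resets.
; Spawned projectiles receive damage, velocity, target and optional AOE settings.
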(event OnComponentBeginOverlap(Sphere)
  (params (OverlappedComponent :type Primitive%20Component%20Object%20Reference) (OtherActor :type Actor%20Object%20Reference) (OtherComp :type Primitive%20Component%20Object%20Reference) (OtherBodyIndex :type Integer) (bFromSweep :type Boolean) (SweepResult :type Hit%20Result%20Structure%20%28by%20ref%29))
  ;[1 1 1] If enemy steps in the sphere collider, put it in a list
  (bind _asbp_base_enemy (Utilities|Casting|CastToBP_BaseEnemy OtherActor))
  (Utilities|Array|AddUnique (Variables|Default|GetEnemysInRange) _asbp_base_enemy))

(event OnComponentEndOverlap(Sphere)
  (params (OverlappedComponent :type Primitive%20Component%20Object%20Reference) (OtherActor :type Actor%20Object%20Reference) (OtherComp :type Primitive%20Component%20Object%20Reference) (OtherBodyIndex :type Integer))
  ;[1 1 1] If enemy steps out of the sphere collider, remove it from the list
  (bind _asbp_base_enemy (Utilities|Casting|CastToBP_BaseEnemy OtherActor))
  (Utilities|Array|RemoveItem (Variables|Default|GetEnemysInRange) _asbp_base_enemy))

(event Custom|Shoot
  (params (Arrow :type Arrow%20Component%20Object%20Reference))
  ;[1 1 1] Shoot will be called every frame when an enemy is in range, "Do Once" reduces this. If the shoot timer is finished reset it so the Tower can shoot again.
  (Utilities|FlowControl|DoOnce false :!label _label
    (:Completed
      (Utilities|IsValid (Variables|Default|GetFocusedEnemy)
        (:Is%20Valid
          (CallFunction|ShootProjectile Arrow)
          (Timeline|ShootTimer PlayFromStart
            (:Finished
              (goto _label Reset))))))))

(event EventTick
  (params (DeltaSeconds :type Float%20%28single-precision%29))
  (bind _yaw_b (Variables|Default|GetYaw_B))
  (bind _returnvalue (Transformation|GetWorldRotation _yaw_b))
  ;[1 1 1] Update List of enemies in range. if enemy is not valid skip this frame
  (bind (_newfocusedenemy _focuschanged_) (CallFunction|UpdateFocusedEnemy))
  (Utilities|IsValid _newfocusedenemy
    (:Is%20Valid
      (bind _rotation (CallFunction|GetRotationtoFocusedEnemy))
      (if _focuschanged_
        (Variables|Default|SetTmpRotation (Math|Rotator|MakeRotator (.roll _returnvalue) (.pitch (Transformation|GetWorldRotation (Variables|Default|GetPitch_B))) (.yaw _returnvalue)))
        ;[1 1 1] Rotate to Enemy. When rotation is finished shoot
        (bind _rotationtime (Timeline|RotationTimer PlayFromStart)
          (:Update
            (Transformation|SetWorldRotation (Variables|Default|GetYaw_B) (Math|Rotator|MakeRotator (.roll (Math|Rotator|Lerp(Rotator) (Variables|Default|GetTmpRotation) _rotation _rotationtime)) 0.0 (.yaw (Math|Rotator|Lerp(Rotator) (Variables|Default|GetTmpRotation) _rotation _rotationtime))) false false)
            (Transformation|SetWorldRotation (Variables|Default|GetPitch_B) (Math|Rotator|MakeRotator (.roll (Math|Rotator|Lerp(Rotator) (Variables|Default|GetTmpRotation) _rotation _rotationtime)) (.pitch (Math|Rotator|Lerp(Rotator) (Variables|Default|GetTmpRotation) _rotation _rotationtime)) (.yaw (Math|Rotator|Lerp(Rotator) (Variables|Default|GetTmpRotation) _rotation _rotationtime))) false false))
          (:Finished
            (CallFunction|Shoot (Variables|Default|GetMainArrowComponent))))
        (else
          (Timeline|RotationTimer Play))))))

(event EventBeginPlay
  ;[1 1 1] Set play rate of shoot timer.
  (Components|Timeline|SetPlayRate (Variables|Default|GetShootTimer) (/ 1.0 (Variables|Default|GetReloadTime)))
  ;[1 1 1] Set play rate of rotarion speed.
  (Components|Timeline|SetPlayRate (Variables|Default|GetRotationTimer) (/ 1.0 (Variables|Default|GetRotateSpeed))))

(fn ConstructionScript
  (Components|Sphere|SetSphereRadius (Variables|Default|GetSphere) (Variables|Default|GetRadius) true))

(fn UpdateFocusedEnemy
  (for _array_element (Variables|Default|GetEnemysInRange)
    (Utilities|IsValid (LocalVariables|GetTmpEnemy)
      (:Is%20Valid
        (if (> (Variables|/Game/Test/VladiAi/Enemy/BP_BaseEnemy.BP_BaseEnemy_C|GetDistance _array_element) (Variables|/Game/Test/VladiAi/Enemy/BP_BaseEnemy.BP_BaseEnemy_C|GetDistance (LocalVariables|GetTmpEnemy)))
          (LocalVariables|SetTmpEnemy _array_element)))
      (:Is%20Not%20Valid
        (LocalVariables|SetTmpEnemy _array_element))))
  (if (== (LocalVariables|GetTmpEnemy) (Variables|Default|GetFocusedEnemy))
    (bind _output_get (Variables|Default|SetFocusedEnemy (LocalVariables|GetTmpEnemy)))
    (return _output_get false)
    (else
      (bind _output_get_2 (Variables|Default|SetFocusedEnemy (LocalVariables|GetTmpEnemy)))
      (return _output_get_2 true))))

(fn GetRotationtoFocusedEnemy
  (bind _focusedenemy (Variables|Default|GetFocusedEnemy))
  (bind _yaw_b (Variables|Default|GetYaw_B))
  (bind _returnvalue (Transformation|GetActorLocation _focusedenemy))
  (bind _returnvalue_2 (Transformation|GetWorldLocation _yaw_b))
  (bind _returnvalue_3 (Math|Rotator|FindLookatRotation _returnvalue_2 _returnvalue))
  (return (Math|Rotator|MakeRotator (.roll (Transformation|GetWorldRotation _yaw_b)) (.pitch _returnvalue_3) (.yaw _returnvalue_3))))

(fn ShootProjectile
  (params (ArrowComponent :type Arrow%20Component%20Object%20Reference))
  (bind _returnvalue (Transformation|GetWorldTransform ArrowComponent))
  (bind _aoeinfo (Variables|Default|GetAOEInfo))
  (bind _focusedenemy (Variables|Default|GetFocusedEnemy))
  ;[1 1 1] Spawn Projectile at Location from Arrow (which should be in front of the cannon
  (bind _returnvalue_2 (Game|SpawnActorfromClass (Variables|Default|GetProjectile) (Math|Transform|MakeTransform (.location _returnvalue) (.rotation _returnvalue) "0.500000,0.500000,0.500000") "AlwaysSpawn" 0 0))
  ;[1 1 1] Set Damage and Speed of Projectile
  (Utilities|IsValid _returnvalue_2
    (:Is%20Valid
      (Variables|/Game/Test/VladiAi/Tower/BlueprintProjectile/BP_BaseProjectile.BP_BaseProjectile_C|SetDamage _returnvalue_2 (Variables|Default|GetDamage))
      (Variables|/Script/Engine.MovementComponent|SetVelocity (Variables|/Game/Test/VladiAi/Tower/BlueprintProjectile/BP_BaseProjectile.BP_BaseProjectile_C|GetProjectileMovement _returnvalue_2) (* (Math|Vector|GetForwardVector ArrowComponent) 9999.0))
      ;[1 1 1] Set AOE Info to Projectile
      (if (.canaoe (Variables|Default|GetAOEInfo))
        (Variables|/Game/Test/VladiAi/Tower/BlueprintProjectile/BP_BaseProjectile.BP_BaseProjectile_C|SetCanAOE _returnvalue_2 true)
        (Variables|/Game/Test/VladiAi/Tower/BlueprintProjectile/BP_BaseProjectile.BP_BaseProjectile_C|SetAOE_Radius _returnvalue_2 (.radius _aoeinfo))
        (Variables|/Game/Test/VladiAi/Tower/BlueprintProjectile/BP_BaseProjectile.BP_BaseProjectile_C|SetAOE_MaxHitCount _returnvalue_2 (.maxhitcount _aoeinfo))
        (Variables|/Game/Test/VladiAi/Tower/BlueprintProjectile/BP_BaseProjectile.BP_BaseProjectile_C|SetDamage _returnvalue_2 (* (Variables|Default|GetDamage) (.dmgscalemultiplehit _aoeinfo))))
      (Utilities|IsValid _focusedenemy
        (:Is%20Valid
          (Variables|/Game/Test/VladiAi/Tower/BlueprintProjectile/BP_BaseProjectile.BP_BaseProjectile_C|SetTarget _returnvalue_2 _focusedenemy))))))