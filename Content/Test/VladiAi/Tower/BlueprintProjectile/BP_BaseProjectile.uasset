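; Base tower projectile actor that damages BP_BaseEnemy actors and destroys itself on overlap or after a timed lifetime.
; Every Tick it points its ProjectileMovement velocity straight at Target, so it homes in at high speed.
; Collider and Box overlaps either damage whichever enemy is hit, Target or not, or, with CanAOE, call AOEDamage.
; AOEDamage runs a debug-drawn sphere overlap and damages enemies up to AOEMaxHitCount.
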(event OnComponentBeginOverlap(Collider)
  (params (OverlappedComponent :type Primitive%20Component%20Object%20Reference) (OtherActor :type Actor%20Object%20Reference) (OtherComp :type Primitive%20Component%20Object%20Reference) (OtherBodyIndex :type Integer) (bFromSweep :type Boolean) (SweepResult :type Hit%20Result%20Structure%20%28by%20ref%29))
  (if (Variables|AOEInfo|GetCanAOE)
    (CallFunction|AOEDamage)
    (Actor|DestroyActor)
    (else
      ;[1 1 1] Hit an enemy. Does not check for target. If projectile hit an enemy it applies damage to it
      (bind _asbp_base_enemy (Utilities|Casting|CastToBP_BaseEnemy OtherActor)
        (:then
          (Game|Damage|ApplyDamage _asbp_base_enemy (Variables|Default|GetDamage) 0 self "/Game/Test/VladiAi/Tower/BP_TowerDamagaType.BP_TowerDamagaType_C")
          (Actor|DestroyActor))
        (:CastFailed
          (Actor|DestroyActor))))))

(event OnComponentBeginOverlap(Box)
  (params (OverlappedComponent :type Primitive%20Component%20Object%20Reference) (OtherActor :type Actor%20Object%20Reference) (OtherComp :type Primitive%20Component%20Object%20Reference) (OtherBodyIndex :type Integer) (bFromSweep :type Boolean) (SweepResult :type Hit%20Result%20Structure%20%28by%20ref%29))
  (if (Variables|AOEInfo|GetCanAOE)
    (CallFunction|AOEDamage)
    (Actor|DestroyActor)
    (else
      ;[1 1 1] Hit an enemy. Does not check for target. If projectile hit an enemy it applies damage to it
      (bind _asbp_base_enemy (Utilities|Casting|CastToBP_BaseEnemy OtherActor)
        (:then
          (Game|Damage|ApplyDamage _asbp_base_enemy (Variables|Default|GetDamage) 0 self "/Game/Test/VladiAi/Tower/BP_TowerDamagaType.BP_TowerDamagaType_C")
          (Actor|DestroyActor))
        (:CastFailed
          (Actor|DestroyActor))))))

(event EventBeginPlay
  (Utilities|FlowControl|Delay 5.0)
  (Actor|DestroyActor)
  (Development|PrintString "destroyed by Time [BP_BaseProjectile]" true true "(R=0.021898,G=1.000000,B=0.000000,A=1.000000)" 3.0))

(event EventTick
  (params (DeltaSeconds :type Float%20%28single-precision%29))
  (bind _target (Variables|Default|GetTarget))
  ;[1 1 1] Projectile look to enemy and fly in this direction (curves) so the projectile can not miss
  (Utilities|IsValid _target
    (:Is%20Valid
      (Variables|/Script/Engine.MovementComponent|SetVelocity (Variables|Default|GetProjectileMovement) (* (Math|Rotator|GetRotationXVector (Math|Rotator|FindLookatRotation (Transformation|GetActorLocation) (Transformation|GetActorLocation _target))) 9999.0)))))

(fn ConstructionScript)

(fn AOEDamage
  ;[1 1 1] DEBUG__Draw AOE
  (Rendering|Debug|DrawDebugSphere (Transformation|GetWorldLocation (Variables|Default|GetSphere)) (Variables|AOEInfo|GetAOE_Radius) 12 "(R=1.000000,G=0.000000,B=0.902083,A=1.000000)" 1.0)
  ;[1 1 1] Create Sphere Collider arount the Projectile to check if enemies are in range.
  (bind _outactors (Collision|SphereOverlapActors (Transformation|GetWorldLocation (Variables|Default|GetSphere)) (Variables|AOEInfo|GetAOE_Radius) (Utilities|Array|MakeArray "ObjectTypeQuery3") "/Game/Test/VladiAi/Enemy/BP_BaseEnemy.BP_BaseEnemy_C"))
  ;[1 1 1] check if hit enemies or max hit count is higher. decrease it by 1 to contert it to index
  (bind _result (Math|Integer|DecrementInt (Math|Integer|Min(Integer) (Utilities|Array|Length _outactors) (Variables|AOEInfo|GetAOE_MaxHitCount)))
    (:%20%20
      ;[1 1 1] Apply Damage to every Enemy in Range
      (for _index (range 0 _result)
        (Game|Damage|ApplyDamage (Utilities|Array|Get(acopy) _outactors _index) (Variables|Default|GetDamage) 0 self "/Game/Test/VladiAi/Tower/BP_TowerDamagaType.BP_TowerDamagaType_C"))
      (return _outactors))))