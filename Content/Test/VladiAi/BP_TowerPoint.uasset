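; BP_TowerPoint is a placement spot that holds a single turret and a UI widget for player interaction.
; BeginPlay creates a TurretWikiBlueprint widget once, and OpenUI and CloseUI add it to or remove it from the viewport.
; SpawnTower spawns the given tower class at the point's root location and stores it as Turret.
; InUse reports whether that turret is valid, and RemoveTower destroys it.
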(event EventBeginPlay
  ;[1 1 1] Create and save UI to show when Player interacts with it
  (bind _returnvalue (UserInterface|CreateWidget "/Game/UI/TurretWikiBlueprint.TurretWikiBlueprint_C"))
  (Variables|Default|SetWidget _returnvalue))

(event Collision|EventActorBeginOverlap
  (params (OtherActor :type Actor%20Object%20Reference)))

(event EventTick
  (params (DeltaSeconds :type Float%20%28single-precision%29)))

(fn ConstructionScript)

(fn SpawnTower
  (params (Tower :type BP%20Base%20Tower%20Class%20Reference))
  ;[1 1 1] Turret has no AI Class so we can simply spawn the actor itself
  (bind _returnvalue (Game|SpawnActorfromClass Tower (Math|Transform|MakeTransform (Transformation|GetWorldLocation (Variables|Default|GetDefaultSceneRoot)) "0, 0, 0" "1,1,1") "Undefined" 0 0))
  (Variables|Default|SetTurret _returnvalue))

(fn InUse
  (return (Utilities|IsValid (Variables|Default|GetTurret))))

(fn RemoveTower
  (Actor|DestroyActor (Variables|Default|GetTurret))
  (return))

(fn OpenUI
  (UserInterface|Viewport|AddtoViewport (Variables|Default|GetWidget) 0))

(fn CloseUI
  (Widget|RemovefromParent (Variables|Default|GetWidget)))