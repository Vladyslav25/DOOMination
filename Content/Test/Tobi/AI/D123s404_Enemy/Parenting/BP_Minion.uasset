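; BP_Minion is a child enemy Blueprint, in a test AI folder, for a minion driven by an AI controller.
; It calls parent logic on BeginPlay and Tick, and overrides Health at BeginPlay.
; Tick casts the controller to AI_MainEnemy but only prints a message on failure.
; The controller's spline-percentage query is left unconnected and never runs.
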(event EventBeginPlay
  (|CallParentFunction)
  (Variables|Default|SetHealth 3e+02))

(event Collision|EventActorBeginOverlap
  (params (OtherActor :type Actor%20Object%20Reference))
  (|CallParentFunction OtherActor) ; This node is disabled and will not be called.\nDrag off pins to build functionality.
)

(event EventTick
  (params (DeltaSeconds :type Float%20%28single-precision%29))
  (bind _self self)
  (bind _returnvalue (Pawn|GetController _self))
  (|CallParentFunction DeltaSeconds)
  (Utilities|IsValid _self
    (:Is%20Valid
      (Utilities|IsValid _returnvalue
        (:Is%20Valid
          (bind _asai_main_enemy (Utilities|Casting|CastToAI_MainEnemy _returnvalue)
            (:CastFailed
              (Development|PrintString "Could not cast to AI_Mainenemy"))))))))

(fn ConstructionScript
  (|CallParentFunction))