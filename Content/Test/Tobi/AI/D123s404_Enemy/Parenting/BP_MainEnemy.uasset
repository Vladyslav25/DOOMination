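; BP_MainEnemy is a base enemy actor that tracks health and death, and which turrets have it in range.
; GetDamage subtracts damage from Health and sets Dead at zero or below, while AddTurret and RemoveTurret maintain the turret list.
; Tick polls Dead, then has every listed turret remove this enemy from its list before the actor destroys itself.
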(event EventBeginPlay)

(event Collision|EventActorBeginOverlap
  (params (OtherActor :type Actor%20Object%20Reference)))

(event EventTick
  (params (DeltaSeconds :type Float%20%28single-precision%29))
  (if (Variables|Default|GetDead)
    (CallFunction|SendMessagetoAllTurrets)
    (Actor|DestroyActor)))

(fn ConstructionScript)

(fn GetDamage
  (params (Damage :type Float%20%28single-precision%29))
  ;[1 1 1] Subtract damage from health
  (bind _output_get (Variables|Default|SetHealth (- (Variables|Default|GetHealth) Damage)))
  (bind _output_get_2 (Variables|Default|SetDead (<= _output_get 0.0)))
  ;[1 1 1] Return true if health is 0 or below
  (return _output_get_2))

(fn IsDead
  (return (Variables|Default|GetDead)))

(fn AddTurret
  (params (Turret :type BP%20Main%20Turret%20Object%20Reference))
  (bind _returnvalue (Utilities|Array|Add (Variables|Default|GetTurrents%20in%20Range) Turret))
  (return _returnvalue))

(fn RemoveTurret
  (params (Turret :type BP%20Main%20Turret%20Object%20Reference))
  (bind _returnvalue (Utilities|Array|RemoveItem (Variables|Default|GetTurrents%20in%20Range) Turret))
  (return _returnvalue))

(fn SendMessagetoAllTurrets
  (for _array_element (Variables|Default|GetTurrents%20in%20Range)
    (Default|RemoveEnemyfromList _array_element self)))