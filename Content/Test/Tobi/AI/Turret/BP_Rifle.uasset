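; Test rifle turret Blueprint that turns toward and damages an enemy within range.
; Each tick it gets the enemies in range, aims at the first one, applies its damage value every frame with no fire-rate gate, and prints that enemy's health.
; Aiming rotates only the world yaw of the RifleYawB component, keeping its pitch and roll.
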(event EventBeginPlay
  (|CallParentFunction) ; This node is disabled and will not be called.\nDrag off pins to build functionality.
)

(event Collision|EventActorBeginOverlap
  (params (OtherActor :type Actor%20Object%20Reference))
  (|CallParentFunction OtherActor) ; This node is disabled and will not be called.\nDrag off pins to build functionality.
)

(event EventTick
  (params (DeltaSeconds :type Float%20%28single-precision%29))
  (|CallParentFunction DeltaSeconds)
  (bind _enemy_list (CallFunction|GetEnemiesinRange))
  (if (> (Utilities|Array|Length _enemy_list) 0)
    (CallFunction|LooktoEmeny (Utilities|Array|Get(acopy) _enemy_list))
    (bind _damage (CallFunction|Damage))
    (Default|GetDamage (Utilities|Array|Get(acopy) _enemy_list) _damage)
    (Development|PrintString (Utilities|String|ToString(Float) (Variables|/Game/Test/Tobi/AI/D123s404_Enemy/Parenting/BP_MainEnemy.BP_MainEnemy_C|GetHealth (Utilities|Array|Get(acopy) _enemy_list))))))

(fn ConstructionScript
  (|CallParentFunction))

(fn LooktoEmeny
  (params (Current%20Enemy :type BP%20Main%20Enemy%20Object%20Reference))
  (bind _rifle_yaw_b (Variables|Default|GetRifle_Yaw_B))
  (bind _returnvalue (Transformation|GetWorldRotation _rifle_yaw_b))
  ;[1 1 1] Makes sure only Z axis will rotate
  (Transformation|SetWorldRotation _rifle_yaw_b (Math|Rotator|MakeRotator (.roll _returnvalue) (.pitch _returnvalue) (.yaw (Math|Rotator|FindLookatRotation (Transformation|GetWorldLocation (Variables|Default|GetRifle_Yaw_B)) (Transformation|GetActorLocation Current%20Enemy)))) false false))