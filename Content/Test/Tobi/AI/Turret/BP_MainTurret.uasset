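; Base turret actor that tracks BP_MainEnemy actors inside its collision sphere.
; Sphere overlaps add and remove enemies from EnemiesInRange and register or unregister the turret with each enemy, printing debug strings.
; Each Tick, RefreshList gathers dead or invalid enemies into ToDelete, then subtracts EnemiesInRange from that set, leaving EnemiesInRange itself unpruned.
; Functions expose the list, manual removal and a fixed damage value, while LookToEmeny is an empty stub.
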(event OnComponentBeginOverlap(SphereCollision)
  (params (OverlappedComponent :type Primitive%20Component%20Object%20Reference) (OtherActor :type Actor%20Object%20Reference) (OtherComp :type Primitive%20Component%20Object%20Reference) (OtherBodyIndex :type Integer) (bFromSweep :type Boolean) (SweepResult :type Hit%20Result%20Structure%20%28by%20ref%29))
  (Development|PrintString (Utilities|GetDisplayName OtherActor))
  (bind _asbp_main_enemy (Utilities|Casting|CastToBP_MainEnemy OtherActor)
    (:then
      (Utilities|Array|Add (Variables|Default|GetEnemies%20in%20Range) _asbp_main_enemy)
      (Default|AddTurret _asbp_main_enemy self))
    (:CastFailed
      (Development|PrintString "Object was not an Enemy" true true "(R=1.000000,G=0.000000,B=0.063568,A=1.000000)" 3.0))))

(event OnComponentEndOverlap(SphereCollision)
  (params (OverlappedComponent :type Primitive%20Component%20Object%20Reference) (OtherActor :type Actor%20Object%20Reference) (OtherComp :type Primitive%20Component%20Object%20Reference) (OtherBodyIndex :type Integer))
  (Development|PrintString (Utilities|GetDisplayName OtherActor))
  (bind _asbp_main_enemy (Utilities|Casting|CastToBP_MainEnemy OtherActor)
    (:then
      (Utilities|Array|RemoveItem (Variables|Default|GetEnemies%20in%20Range) _asbp_main_enemy)
      (Default|RemoveTurret _asbp_main_enemy self))
    (:CastFailed
      (Development|PrintString "Object was not an Enemy" true true "(R=1.000000,G=0.000000,B=0.063568,A=1.000000)" 3.0))))

(event EventBeginPlay)

(event Collision|EventActorBeginOverlap
  (params (OtherActor :type Actor%20Object%20Reference)))

(event EventTick
  (params (DeltaSeconds :type Float%20%28single-precision%29))
  (CallFunction|RefreshList))

(fn ConstructionScript)

(fn GetEnemiesinRange
  (return (Variables|Default|GetEnemies%20in%20Range)))

(fn RefreshList
  (for _array_element (Variables|Default|GetEnemies%20in%20Range)
    (Utilities|IsValid _array_element
      (:Is%20Valid
        (bind _enemy_dead (Default|IsDead _array_element))
        (if _enemy_dead
          (Utilities|Set|Add (LocalVariables|GetTo%20Delete) _array_element :!label _label)))
      (:Is%20Not%20Valid
        (goto _label))))
  (Utilities|Set|RemoveItems (LocalVariables|GetTo%20Delete) (Variables|Default|GetEnemies%20in%20Range)))

(fn RemoveEnemyfromList
  (params (Enemy :type BP%20Main%20Enemy%20Object%20Reference))
  (bind _returnvalue (Utilities|Array|RemoveItem (Variables|Default|GetEnemies%20in%20Range) Enemy))
  (return _returnvalue))

(fn Damage
  (return 1.5))

(fn LooktoEmeny
  (params (Current%20Enemy :type BP%20Main%20Enemy%20Object%20Reference)))