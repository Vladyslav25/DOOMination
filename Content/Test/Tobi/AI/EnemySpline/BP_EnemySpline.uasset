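; BP_EnemySpline is a test enemy that follows a spline track under control of its AI_EnemySpline controller.
; On BeginPlay it registers itself with the controller as the controlled actor, then picks a random BP_Track from the level.
; It passes that track to the controller and starts FollowSplineTrail, printing debug messages if no track or controller is found.
; The movement logic itself lives in the controller.
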(event EventBeginPlay
  (CallFunction|SetActorOfAIController)
  (bind _outactors (Actor|GetAllActorsOfClass "/Game/Test/Tobi/AI/EnemySpline/BP_Track.BP_Track_C"))
  ;[1 1 1] DEBUG
  (if (== (Utilities|Array|Length _outactors) 0)
    (Development|PrintString "No Spline Trail found" true true "(R=1.000000,G=0.000000,B=0.000000,A=1.000000)" 5.0)
    (else
      (bind _asbp_track (Utilities|Casting|CastToBP_Track (Utilities|Array|Get(acopy) _outactors (Math|Random|RandomIntegerinRange 0 (- (Utilities|Array|Length _outactors) 1)))))
      (Variables|Default|SetTrack _asbp_track)
      (bind _asai_enemy_spline (Utilities|Casting|CastToAI_EnemySpline (AI|GetAIController self))
        (:then
          (Variables|/Game/Test/Tobi/AI/EnemySpline/AI_EnemySpline.AI_EnemySpline_C|SetSplineToFollow _asai_enemy_spline (Variables|Default|GetTrack))
          (Default|FollowSplineTrail _asai_enemy_spline))
        (:CastFailed
          (Development|PrintString "Cast Failed"))))))

(event Collision|EventActorBeginOverlap
  (params (OtherActor :type Actor%20Object%20Reference)))

(event EventTick
  (params (DeltaSeconds :type Float%20%28single-precision%29)))

(fn ConstructionScript)

(fn SetActorOfAIController
  (bind _asai_enemy_spline (Utilities|Casting|CastToAI_EnemySpline (AI|GetAIController self)))
  (Variables|/Game/Test/Tobi/AI/EnemySpline/AI_EnemySpline.AI_EnemySpline_C|SetActorOfAI _asai_enemy_spline self))