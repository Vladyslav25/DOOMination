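; BP_Track is a test spline track actor that moves a particle system along its spline in a repeating loop.
; A looping timer started on BeginPlay calls MoveAlongSpline, which advances a normalized progress value and places the particles at that distance in world space.
; The step scales inversely with spline length for constant speed, and progress resets to the start upon reaching the end.
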(event EventBeginPlay
  (Utilities|Time|SetTimerbyFunctionName 0 "MoveAlongSpline" 0.1 true))

(event Collision|EventActorBeginOverlap
  (params (OtherActor :type Actor%20Object%20Reference)))

(event EventTick
  (params (DeltaSeconds :type Float%20%28single-precision%29)))

(fn ConstructionScript)

(fn MoveAlongSpline
  (Variables|Default|SetSplinePercent (Math|Float|Clamp(Float) (+ (Variables|Default|GetSplinePercent) (/ 0.01 (/ (Spline|GetSplineLength (Variables|Default|GetSplineTrack)) 2e+03)))))
  (Transformation|SetWorldLocation (Variables|Default|GetParticleSystem) (Spline|GetLocationatDistanceAlongSpline (Variables|Default|GetSplineTrack) (* (Variables|Default|GetSplinePercent) (Spline|GetSplineLength (Variables|Default|GetSplineTrack))) "World") false false)
  ;[1 1 1] Reset Particle System Location
  (if (== (Variables|Default|GetSplinePercent) 1.0)
    (Variables|Default|SetSplinePercent 0.0)))